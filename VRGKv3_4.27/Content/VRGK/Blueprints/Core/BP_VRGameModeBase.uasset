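; VR game mode base that creates the shared helper actors a level needs at startup.
; On BeginPlay it spawns and stores the menu controller, spectator camera, player vignette and camera water overlay, then runs the game instance's level begin-play events.
; A final step spawns the VR subtitle actor.
; Getter functions expose the menu controller, subtitle and vignette actors to other Blueprints.
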(event `self.ReceiveBeginPlay`
  ;[1 1 1] Begin Play
  (`|ExecutionSequence`
    (:`then_0`
      (bind _returnvalue (`|SpawnActorFromClass` "/Game/VRGK/Blueprints/Core/BP_MenuController.BP_MenuController_C" (`KismetMathLibrary.MakeTransform` (0.0 0.0 0.0)) "Undefined" "OverrideRootScale" null null))
      (set `self.MenuController` _returnvalue)
      (bind _returnvalue_2 (`|SpawnActorFromClass` "/Game/VRGK/Blueprints/SpectatorCams/BP_VRSpectator.BP_VRSpectator_C" (`KismetMathLibrary.MakeTransform` (0.0 0.0 0.0)) "Undefined" "OverrideRootScale" null null))
      (set `self.VRSpectatorCamera` _returnvalue_2)
      (bind _returnvalue_3 (`|SpawnActorFromClass` "/Game/VRGK/Blueprints/Player/BP_PlayerVignette.BP_PlayerVignette_C" (`KismetMathLibrary.MakeTransform` (0.0 0.0 0.0)) "Undefined" "OverrideRootScale" null null))
      (set `self.PlayerVignette` _returnvalue_3)
      (bind _returnvalue_4 (`|SpawnActorFromClass` "/Game/VRGK/Blueprints/Player/BP_CameraWaterOverlay.BP_CameraWaterOverlay_C" (`KismetMathLibrary.MakeTransform` (0.0 0.0 0.0)) "Undefined" "OverrideRootScale" null null))
      (set `self.CameraWaterOverlay` _returnvalue_4))
    (:`then_1`
      (bind _bp_game_instance (`/Game/VRGK/Blueprints/BPFL_GlobalFunctions.GetBPGameInstance`))
      (`/Game/VRGK/Blueprints/Core/BP_GameInstance.DoLevelBeginPlayEvents` _bp_game_instance))
    (:`then_2`
      (`self.SetupVRSubtitles`))))

(event `SetupVRSubtitles`
  ;[1 1 1] Setup VR Subtitles
  (bind _returnvalue (`|SpawnActorFromClass` "/Game/VRGK/Blueprints/Subtitles/BP_VRSubtitles.BP_VRSubtitles_C" (`KismetMathLibrary.MakeTransform` (0.0 0.0 0.0)) "Undefined" "OverrideRootScale" null null))
  (set `self.VRSubtitleActor` _returnvalue))

(fn `GetMenuController`
  (returns (MenuController :type "/Game/VRGK/Blueprints/Core/BP_MenuController Object Reference"))
  (return (`self.MenuController`)))

(fn `GetSubtitleActor`
  (returns (Actor :type "/Game/VRGK/Blueprints/Subtitles/BP_VRSubtitles Object Reference"))
  (return (`self.VRSubtitleActor`)))

(fn `GetVignetteActor`
  (returns (Vignette :type "/Game/VRGK/Blueprints/Player/BP_PlayerVignette Object Reference"))
  (return (`self.PlayerVignette`)))

(fn `UserConstructionScript`)