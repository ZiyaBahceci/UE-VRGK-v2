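; BPC_StabPosition is a component in the VRGK stabbing tools that defines where a stab starts and ends relative to its own transform.
; It projects a given point onto a start segment along local X, then offsets the result along local Z to get the matching end point.
; It also exposes a world center halfway along that Z depth, with all extents hardcoded in local space.
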(fn `Get World Center`
  (returns (ReturnValue :type "Vector Structure"))
  (return (`KismetMathLibrary.TransformLocation` (`self.K2_GetComponentToWorld`) (0.0 0.0 50.0))))

(fn `GetClosestEndPoint`
  (params (Point :type "Vector Structure"))
  (returns (ReturnValue :type "Vector Structure"))
  (return (+ (`self.GetClosestPointOnStartLine` Point) (`KismetMathLibrary.TransformDirection` (`self.K2_GetComponentToWorld`) (0.0 0.0 100.0)))))

(fn `GetClosestPointOnStartLine`
  (params (Point :type "Vector Structure"))
  (returns (ReturnValue :type "Vector Structure"))
  (bind _returnvalue (`self.K2_GetComponentToWorld`))
  (return (`KismetMathLibrary.FindClosestPointOnSegment` Point (`KismetMathLibrary.TransformLocation` _returnvalue (50.0 0.0 0.0)) (`KismetMathLibrary.TransformLocation` _returnvalue (-50.0 0.0 0.0)))))