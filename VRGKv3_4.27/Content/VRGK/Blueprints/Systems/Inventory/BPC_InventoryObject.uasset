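; Inventory object component that lets its owning actor be stored in a BPC_InventorySlot, extending a parent's attach and release logic.
; On attach it measures the largest colliding-bounds extent, disables actor collision and, if the slot allows, uniformly scales the actor to the slot radius.
; Release resets scale to one rather than the original, restores collision, then runs parent release.
; Both report through OnInventoryObjectAdjustment; BeginPlay deliberately skips parent logic.
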(event `self.ReceiveBeginPlay`)

(fn `DoAttachmentToSlot`
  (locals (ActorBoundsRadius :type "Float (double-precision)" :default 0.0))
  (bind (_origin _boxextent) (`Actor.GetActorBounds` (`self.GetOwner`) true false))
  (bind _asbpc_inventory_slot (cast `/Game/VRGK/Blueprints/Systems/Inventory/BPC_InventorySlot` (`self.AttachedSlot`) :!pure true))
  (`parent.DoAttachmentToSlot`)
  (`|ExecutionSequence`
    (:`then_0`
      (set `local.ActorBoundsRadius` (`KismetMathLibrary.FMax` (.x _boxextent) (.y _boxextent) (.z _boxextent)))
      (`Actor.SetActorEnableCollision` (`self.GetOwner`) false)
      (if (`/Game/VRGK/Blueprints/Systems/Inventory/BPC_InventorySlot.Scale Attached Actor to Slot Radius` _asbpc_inventory_slot)
        (`Actor.SetActorScale3D` (`self.GetOwner`) (`KismetMathLibrary.Conv_DoubleToVector` (`KismetMathLibrary.FMax` (/ (`/Game/VRGK/Blueprints/Systems/Inventory/BPC_InventorySlot.Slot Radius` _asbpc_inventory_slot) (`local.ActorBoundsRadius`)) 0.01)))))
    (:`then_1`
      (`self.OnInventoryObjectAdjustment` self true))))

(fn `DoReleaseAttachment`
  (bind _returnvalue (`self.GetOwner`))
  (`|ExecutionSequence`
    (:`then_0`
      (`Actor.SetActorScale3D` _returnvalue (`KismetMathLibrary.Conv_DoubleToVector` 1.0))
      (`Actor.SetActorEnableCollision` _returnvalue true))
    (:`then_1`
      (`self.OnInventoryObjectAdjustment` self))
    (:`then_2`
      (`parent.DoReleaseAttachment`))))