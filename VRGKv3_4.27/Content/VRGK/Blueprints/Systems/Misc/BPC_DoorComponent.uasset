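; BPC_DoorComponent is a component that holds a door's locked state and notifies listeners when it changes.
; SetDoorLocked fires OnLockStateChanged only when the new value differs, but records the owner's game time since creation on every call.
; A getter returns the time elapsed since that timestamp, so a redundant set call also restarts that interval.
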(event `SetDoorLocked`
  (params (NewLocked :type Boolean))
  (set `self.LockStateChangeTime` (`Actor.GetGameTimeSinceCreation` (`self.GetOwner`)))
  (if (!= NewLocked (`self.Locked`))
    (set `self.Locked` NewLocked)
    (`self.OnLockStateChanged` (`self.Locked`))))

(fn `Get TIme Since Last Lock Change`
  (returns (ReturnValue :type "Float (double-precision)"))
  (return (- (`Actor.GetGameTimeSinceCreation` (`self.GetOwner`)) (`self.LockStateChangeTime`))))