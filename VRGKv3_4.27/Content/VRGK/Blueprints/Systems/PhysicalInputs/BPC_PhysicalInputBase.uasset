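; Base component for VR physical inputs, with overridable events for child components to update and calculate their values.
; Setup, optionally automatic on BeginPlay by component name, links a child primitive and, in constraint mode, its physics constraint.
; Grabbing hands are tracked for that primitive.
; To limit cost, it ticks only while the simulated body is awake or, in welded mode, while a hand holds it.
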(event `self.ReceiveBeginPlay`
  ;[0.2827 1 0.7412] Begin Play
  (if (`self.SetupOnBeginPlay`)
    ;[1 1 1] Auto Setup
    (bind _component (`/Game/VRGK/Blueprints/BPFL_GlobalFunctions.GetComponentWithName` (`self.GetOwner`) (`self.Primitive Component Name`)))
    (bind _asprimitive_component (cast `PrimitiveComponent` _component)
      (:`then`
        (switch `/Game/VRGK/Blueprints/Systems/PhysicalInputs/Enum_PhysicalInputInteractionmode` (`self.Interaction Mode`)
          (:`NewEnumerator0`
            (bind _component_2 (`/Game/VRGK/Blueprints/BPFL_GlobalFunctions.GetComponentWithName` (`self.GetOwner`) (`self.Physics Constraint Name`)))
            (bind _asphysics_constraint_component (cast `PhysicsConstraintComponent` _component_2)
              (:`then`
                (`self.SetupPhysicalInput` _asphysics_constraint_component _asprimitive_component))
              (:`CastFailed`
                (`self.DoErrorPrint` "Get Parent Physics Constraint"))))
          (:`NewEnumerator1`
            (`self.SetupPhysicalInput` null _asprimitive_component))))
      (:`CastFailed`
        (`self.DoErrorPrint` "Get Child Primitive Component")))))

(event `self.ReceiveTick`
  (params (DeltaSeconds :type "Float (single-precision)"))
  ;[1 0.4637 0.7996] Event Ticks
  (bind _output_get (set `self.CurrentDeltaSeconds` DeltaSeconds))
  (`self.Physical Input Tick` _output_get))

(event `Physical Input Tick`
  (params (`Delta Seconds` :type "Float (double-precision)"))
  ;[1 0.4637 0.7996] Event Ticks
  (set `self.CurrentInputDeltaSeconds` `Delta Seconds`))

(event `CalculateCurrentInputValues`)

(event `PrepareConstruction`)

(event `SetupPhysicalInput`
  (params (ParentPhysicsConstraint :type "PhysicsConstraintComponent Object Reference") (ChildPrimitiveComponent :type "PrimitiveComponent Object Reference"))
  ;[0.2331 1 0.2328] Setup the Physical Input Component.
  (`|ExecutionSequence`
    (:`then_0`
      (set `self.ParentPhysicsConstraint` ParentPhysicsConstraint)
      (set `self.ChildPrimitiveComponent` ChildPrimitiveComponent))
    (:`then_1`
      (switch `/Game/VRGK/Blueprints/Systems/PhysicalInputs/Enum_PhysicalInputInteractionmode` (`self.Interaction Mode`)
        (:`NewEnumerator0`
          (bind _childprimitivecomponent (`self.ChildPrimitiveComponent`)
            (:`then`
              (add `PrimitiveComponent.OnComponentWake` _childprimitivecomponent (delegate `OnChildPrimitiveWake`))
              (add `PrimitiveComponent.OnComponentSleep` (`self.ChildPrimitiveComponent`) (delegate `OnChildPrimitiveSleep`)))
            (:`else`
              (`self.DoErrorPrint` "Invalid Child Primitive on Binding Wake/Sleep"))))))))

(event `TryRegisterHand`
  (params (`This Hand` :type "/Game/VRGK/Blueprints/Player/Hand/BP_VRHand Object Reference") (`Grabbed Component` :type "PrimitiveComponent Object Reference"))
  ;[0.3951 0.7162 1] Register Hands.
  (if (== `Grabbed Component` (`self.ChildPrimitiveComponent`))
    (`KismetArrayLibrary.Array_AddUnique` (`self.TrackedHandArray`) `This Hand`)
    (`self.UpdatePhysicalInputState` :!label _label)))

(event `TryUnregisterHand`
  (params (`This Hand` :type "/Game/VRGK/Blueprints/Player/Hand/BP_VRHand Object Reference") (`Grabbed Component` :type "PrimitiveComponent Object Reference"))
  ;[0.3951 0.7162 1] Register Hands.
  (if (== `Grabbed Component` (`self.ChildPrimitiveComponent`))
    (`KismetArrayLibrary.Array_RemoveItem` (`self.TrackedHandArray`) `This Hand`)
    (goto _label)))

(event `OnChildPrimitiveWake`
  (params (WakingComponent :type "PrimitiveComponent Object Reference") (BoneName :type Name))
  ;[0.2331 1 0.2328] Setup the Physical Input Component.
  (`self.UpdatePhysicalInputState`))

(event `OnChildPrimitiveSleep`
  (params (SleepingComponent :type "PrimitiveComponent Object Reference") (BoneName :type Name))
  ;[0.2331 1 0.2328] Setup the Physical Input Component.
  (`self.UpdatePhysicalInputState`))

(event `UpdatePhysicalInputState`
  ;[1 0.3089 0.513] Update Input State
  (switch `/Game/VRGK/Blueprints/Systems/PhysicalInputs/Enum_PhysicalInputInteractionmode` (`self.Interaction Mode`)
    (:`NewEnumerator0`
      (`self.SetInputUpdateEnabled` (`PrimitiveComponent.IsAnyRigidBodyAwake` (`self.ChildPrimitiveComponent`))))
    (:`NewEnumerator1`
      (`self.SetInputUpdateEnabled` (> (`KismetArrayLibrary.Array_Length` (`self.TrackedHandArray`)) 0)))))

(event `SetInputUpdateEnabled`
  (params (Condition :type Boolean))
  (bind _returnvalue (`self.IsComponentTickEnabled`))
  ;[1 0.3089 0.513] Update Input State
  (if Condition
    (if (not _returnvalue)
      (`self.SetComponentTickEnabled` true)
      (set `self.GameTimeOnUpdateEnabled` (`self.OwnersGameTimeSinceCreation`)))
    (elif _returnvalue
      (`self.SetComponentTickEnabled` false))))

(fn `DoErrorPrint`
  (params (String :type String))
  (`KismetSystemLibrary.PrintString` (`KismetStringLibrary.Concat_StrStr` (`KismetSystemLibrary.GetDisplayName` (`self.GetOwner`)) " - Failed Physical Input Base, " String)))

(fn `OwnersGameTimeSinceCreation`
  (returns (ReturnValue :type "Float (double-precision)"))
  (return (`Actor.GetGameTimeSinceCreation` (`self.GetOwner`))))