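; VR hand for the physics pawn, driven by physics constraints to the rig's hand center.
; ReconstraintHandConstraints binds the hand collision, and optionally a PD sphere, to that center, then refreshes target frames.
; UpdateHandConstraintFrames interpolates the hand socket's rig-relative transform into both constraints, scaling location by pawn world scale, so fast controller motion doesn't jolt the pawn.
; Updates pause when the attach parent's low relative height indicates bad tracking.
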(event `self.ReceiveBeginPlay`
  (`parent.ReceiveBeginPlay`))

(event `self.ReceiveTick`
  (params (DeltaSeconds :type "Float (single-precision)"))
  (`parent.ReceiveTick` DeltaSeconds))

(event `SetConstraintTargetFrames`
  (params (RefFrame :type "Transform Structure (by ref)"))
  (bind _returnvalue (`KismetMathLibrary.MakeTransform` (* (.location RefFrame) (`/Game/VRGK/Blueprints/Player/PlayerCore/BP_VRGamePawn.GetVRPawnWorldScale` (`self.VRPawn`))) (.rotation RefFrame) (.scale RefFrame)))
  ;[1 1 1] Set Constraint Target Frames
  (`PhysicsConstraintComponent.SetConstraintReferenceFrame` (`self.HandBaseConstraint`) "Frame2" _returnvalue)
  (`PhysicsConstraintComponent.SetConstraintReferenceFrame` (`self.PDBaseConstraint`) "Frame2" _returnvalue))

(event `UpdateHandConstraintFrames`
  (bind (_targetreferenceframe_location _targetreferenceframe_rotation) (`KismetMathLibrary.BreakTransform` (`self.TargetReferenceFrame`)))
  (bind _targetreferenceframe_location_2 (`KismetMathLibrary.BreakTransform` (`self.TargetReferenceFrame`)))
  (bind _returnvalue (`SceneComponent.GetAttachParent` (`self.HandSceneRoot`)))
  (bind (_returnvalue_location _returnvalue_rotation) (`KismetMathLibrary.BreakTransform` (`SceneComponent.K2_GetComponentToWorld` (`self.HandSocket`))))
  (bind _returnvalue_2 (`SceneComponent.K2_GetComponentToWorld` (`/Game/VRGK/Blueprints/Player/GamePawns/PhysicsPawn/BP_VRPhysicsPawn_PhysicsRig.GetHandCenter` (`self.PhysicsRig`))))
  (bind (_relativelocation_x _relativelocation_y _relativelocation_z) (`KismetMathLibrary.BreakVector` (`SceneComponent.RelativeLocation` _returnvalue)))
  (bind (_returnvalue_location_2 _returnvalue_rotation_2 _returnvalue_scale) (`KismetMathLibrary.BreakTransform` (`KismetMathLibrary.MakeTransform` (`KismetMathLibrary.InverseTransformLocation` _returnvalue_2 _returnvalue_location) (`KismetMathLibrary.InverseTransformRotation` _returnvalue_2 _returnvalue_rotation))))
  (bind (_returnvalue_roll _returnvalue_pitch _returnvalue_yaw) (`KismetMathLibrary.BreakRotator` (`KismetMathLibrary.NormalizedDeltaRotator` _returnvalue_rotation_2 _targetreferenceframe_rotation)))
  (bind (_returnvalue_x _returnvalue_y _returnvalue_z) (`KismetMathLibrary.BreakVector` (+ (`KismetMathLibrary.MakeVector` (.roll _targetreferenceframe_rotation) (.pitch _targetreferenceframe_rotation) (.yaw _targetreferenceframe_rotation)) (`KismetMathLibrary.VInterpTo` (0.0 0.0 0.0) (`KismetMathLibrary.MakeVector` _returnvalue_roll _returnvalue_pitch _returnvalue_yaw) (`GameplayStatics.GetWorldDeltaSeconds`) 50.0))))
  ;[0.9454 0.498 1] Update this Hands Constraint Frames, Relative to the physics pawn rig.
  ;;[1 1 1] Error Reduction; Hand Constraint should not update when the controllers have bad tracking.
  (`/Engine/EditorBlueprintResources/StandardMacros.IsValid` _returnvalue
    (:`Is Valid`
      (if (> _relativelocation_z 1.0)
        (bind _output_get (set `self.TargetReferenceFrame` (`KismetMathLibrary.MakeTransform` (`KismetMathLibrary.VInterpTo` _targetreferenceframe_location_2 _returnvalue_location_2 (`GameplayStatics.GetWorldDeltaSeconds`) 50.0) (`KismetMathLibrary.MakeRotator` _returnvalue_x _returnvalue_y _returnvalue_z) _returnvalue_scale) :!label _label))
        (`self.SetConstraintTargetFrames` _output_get)))
    (:`Is Not Valid`
      (goto _label))))

(fn `ReconstraintHandConstraints`
  (`|ExecutionSequence`
    (:`then_0`
      (`PhysicsConstraintComponent.SetConstrainedComponents` (`self.HandBaseConstraint`) (`self.HandBaseCollision`) "None" (`/Game/VRGK/Blueprints/Player/GamePawns/PhysicsPawn/BP_VRPhysicsPawn_PhysicsRig.GetHandCenter` (`self.PhysicsRig`)) "None")
      (`PhysicsConstraintComponent.SetConstraintReferenceFrame` (`self.HandBaseConstraint`) "Frame1" (`KismetMathLibrary.MakeTransform` (0.0 0.0 0.0)))
      (if (`self.UseHandConstraintPDSwitch`)
        (`PhysicsConstraintComponent.SetConstrainedComponents` (`self.PDBaseConstraint`) (`self.PDBaseSphere`) "None" (`/Game/VRGK/Blueprints/Player/GamePawns/PhysicsPawn/BP_VRPhysicsPawn_PhysicsRig.GetHandCenter` (`self.PhysicsRig`)) "None")
        (`PhysicsConstraintComponent.SetConstraintReferenceFrame` (`self.PDBaseConstraint`) "Frame1" (`KismetMathLibrary.MakeTransform` (0.0 0.0 0.0)))))
    (:`then_1`
      (`self.UpdateHandConstraintFrames`))))

(fn `UserConstructionScript`
  (`parent.UserConstructionScript`))