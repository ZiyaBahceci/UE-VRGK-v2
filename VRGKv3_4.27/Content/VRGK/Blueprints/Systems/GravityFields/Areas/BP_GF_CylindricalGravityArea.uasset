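; Cylindrical gravity area for the gravity field system, pulling toward its local Z axis, or away from it when inverted.
; GetGravityAreaDirection flattens the location in actor space, builds a radial look-at rotation and returns it in world space with priority and strength.
; IsInRange tests against a fixed-size local-space cylinder, so the actor's transform scale sets the area's real size.
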(event `self.ReceiveBeginPlay`
  (`parent.ReceiveBeginPlay`))

(fn `GetGravityAreaDirection`
  (params (AtLocation :type "Vector Structure"))
  (returns (ToRotation :type "Rotator Structure") (Priority :type Integer) (Strength :type "Float (double-precision)"))
  (bind (_returnvalue_x _returnvalue_y) (`KismetMathLibrary.BreakVector` (`KismetMathLibrary.InverseTransformLocation` (`self.GetTransform`) AtLocation)))
  (bind _returnvalue (`KismetMathLibrary.MakeVector` _returnvalue_x _returnvalue_y))
  (return (`KismetMathLibrary.TransformRotation` (`self.GetTransform`) (`KismetMathLibrary.SelectRotator` (`KismetMathLibrary.FindLookAtRotation` (0.0 0.0 0.0) _returnvalue) (`KismetMathLibrary.FindLookAtRotation` _returnvalue (0.0 0.0 0.0)) (`self.IsInverted`))) (`self.Priority`) (`self.GravityStrength`)))

(fn `IsInRange`
  (params (AtLocation :type "Vector Structure"))
  (returns (InRange :type Boolean))
  (bind (_returnvalue_x _returnvalue_y _returnvalue_z) (`KismetMathLibrary.BreakVector` (`KismetMathLibrary.InverseTransformLocation` (`self.GetTransform`) AtLocation)))
  (return (and (< (`KismetMathLibrary.VSize` (`KismetMathLibrary.MakeVector` _returnvalue_x _returnvalue_y)) 50.0) (`KismetMathLibrary.InRange_FloatFloat` _returnvalue_z -50.0 50.0 false false))))

(fn `UserConstructionScript`
  (`parent.UserConstructionScript`))