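; BP_CameraWaterOverlay is a VR player actor that shows a water effect on the camera when its sphere overlaps tagged components.
; It snaps to the player camera manager on BeginPlay and registers OverlapSphere with a tagged-component overlap tracker.
; Tracker updates play or reverse a timeline that drives the effect mesh's custom primitive data.
; The actor unhides on overlap and hides once the reverse fade finishes.
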(event `self.ReceiveBeginPlay`
  (`self.K2_AttachToComponent` self (`PlayerCameraManager.TransformComponent` (`GameplayStatics.GetPlayerCameraManager` 0)) "None" "SnapToTarget" "SnapToTarget" "KeepWorld" false)
  (`self.ForceHide`)
  (`/Game/VRGK/Blueprints/Components/BPC_TaggedComponentOverlapTracker.Register Primitive Component For Overlaps` (`self.BPC_TaggedComponentOverlapTracker`) (`self.OverlapSphere`)))

(event `self.BPC_TaggedComponentOverlapTracker.OnTrackerStateUpdate`
  (params (`Is Overlapping` :type Boolean))
  (if `Is Overlapping`
    (`self.SetActorHiddenInGame` false)
    (bind (_direction _alpha) (`Timeline|WaterTimeline` :!label _label)
      (:`Update`
        (`PrimitiveComponent.SetCustomPrimitiveDataFloat` (`self.WaterEffectMesh`) 0 _alpha :!label _label_2))
      (:`Finished`
        (`|ExecutionSequence`
          (:`then_0`
            (goto _label_2))
          (:`then_1`
            (switch `ETimelineDirection` _direction
              (:`Backward`
                (`self.SetActorHiddenInGame` true)))))))
    (else
      (goto _label :!via `Reverse`))))

(event `ForceHide`
  (goto _label :!via `Reverse`))

(fn `UserConstructionScript`)