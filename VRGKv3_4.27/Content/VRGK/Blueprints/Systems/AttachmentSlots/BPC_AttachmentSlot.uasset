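; VR attachment slot component that holds one BPC_AttachableObject at a time.
; Overlaps on its child primitives trigger validation by class, tags, grab state and self-attachment, then either attach the object or optionally release the current one.
; The attachable object performs the actual attach and release, while the slot fires callbacks, plays sounds and releases on EndPlay.
; Each change resets hand hit events on involved grab updaters, including those under the parent's physics root.
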(event `self.ReceiveEndPlay`
  (params (EndPlayReason :type "EEndPlayReason Enum" :default "Destroyed"))
  ;[0.3135 0.1115 0.1296] End Play
  (`self.TryReleaseCurrentObject`))

(event `TryGetHandGrabCollisionUpdater`
  (set `self.HandGrabCollisionUpdater` (`Actor.GetComponentByClass` (`self.GetOwner`) "/Game/VRGK/Blueprints/Components/GrabCollisionUpdater/BPC_HandGrabUpdater.BPC_HandGrabUpdater_C")))

(event `self.ReceiveBeginPlay`
  ;[1 1 1] Begin Play
  (`self.SetupChildOverlaps`)
  (`self.TryGetHandGrabCollisionUpdater`))

(event `SetupChildOverlaps`
  ;[0.3834 0.4114 1] Setup Overlap Events of Child Components. Used for Attachment Events.
  (for _array_element (`self.GetChildrenComponents` false)
    (bind _asprimitive_component (cast `PrimitiveComponent` _array_element))
    (if (`PrimitiveComponent.bGenerateOverlapEvents` _asprimitive_component)
      (add `PrimitiveComponent.OnComponentBeginOverlap` _asprimitive_component (delegate `OnChildOverlap`)))))

(event `OnChildOverlap`
  (params (OverlappedComponent :type "PrimitiveComponent Object Reference") (OtherActor :type "Actor Object Reference") (OtherComp :type "PrimitiveComponent Object Reference") (OtherBodyIndex :type Integer) (bFromSweep :type Boolean) (SweepResult :type "HitResult Structure (by ref)"))
  ;[0.8606 0.5288 1] On Overlap Events of this Slot
  (if (`self.ReleaseIfNewObjectIsOverlapping`)
    (`/Engine/EditorBlueprintResources/StandardMacros.IsValid` (`self.AttachedObject`)
      (:`Is Valid`
        (bind _sucess (`self.CheckIfActorCanAttach` OtherActor))
        (if _sucess
          (`self.TryReleaseCurrentObject`)))
      (:`Is Not Valid`
        (`self.TryAttachActor` OtherActor :!label _label)))
    (else
      (goto _label))))

(fn `CheckIfActorCanAttach`
  (params (`Actor to Check` :type "Actor Object Reference"))
  (returns (Sucess :type Boolean) (`Target Object` :type "/Game/VRGK/Blueprints/Systems/AttachmentSlots/BPC_AttachableObject Object Reference"))
  (locals (TempObject :type "/Game/VRGK/Blueprints/Systems/AttachmentSlots/BPC_AttachableObject Object Reference"))
  (for _array_element (`Actor.K2_GetComponentsByClass` `Actor to Check` (`self.GetValidAttachmentObjectClass`))
    (if (== (`GameplayStatics.GetObjectClass` _array_element) (`self.GetValidAttachmentObjectClass`))
      (set `local.TempObject` _array_element)
      (break)))
  (`|ExecutionSequence`
    (:`then_0`
      (`/Engine/EditorBlueprintResources/StandardMacros.IsValid` (`local.TempObject`)
        (:`Is Valid`
          (if (`self.CheckIfAttachedClassIsValid` (`GameplayStatics.GetObjectClass` (`local.TempObject`)))
            (if (`/Game/VRGK/Blueprints/Systems/AttachmentSlots/BPC_AttachableObject.CanAttach` (`local.TempObject`) (`self.OnlyAllowGrabbedObjects`))
              (if (`self.CheckIfAttachedTagsAreValid` (`local.TempObject`))
                (for _array_element_2 (`Actor.K2_GetComponentsByClass` (`self.GetOwner`) (`self.GetValidAttachmentObjectClass`))
                  (if (== (`GameplayStatics.GetObjectClass` _array_element_2) (`self.GetValidAttachmentObjectClass`))
                    (if (== (`/Game/VRGK/Blueprints/Systems/AttachmentSlots/BPC_AttachableObject.AttachedSlot` _array_element_2) self)
                      (return false null))))
                (else
                  (return false null)))
              (else
                (return false null)))
            (else
              (return false null))))
        (:`Is Not Valid`
          (return false null))))
    (:`then_1`
      (return true (`local.TempObject`)))))

(fn `CheckIfAttachedClassIsValid`
  (params (`Class to Check` :type "/Game/VRGK/Blueprints/Systems/AttachmentSlots/BPC_AttachableObject Class Reference"))
  (returns (Valid :type Boolean))
  (return (== `Class to Check` (`self.GetValidAttachmentObjectClass`))))

(fn `CheckIfAttachedTagsAreValid`
  (params (`Attachable Object Ref` :type "/Game/VRGK/Blueprints/Systems/AttachmentSlots/BPC_AttachableObject Object Reference"))
  (returns (Valid :type Boolean))
  (return (`BlueprintGameplayTagLibrary.MatchesAnyTags` (`/Game/VRGK/Blueprints/Systems/AttachmentSlots/BPC_AttachableObject.Attachment Tag` `Attachable Object Ref`) (`self.AllowedTags`) (`self.Exact Matching Tags`))))

(fn `GetAttachedActor`
  (returns (ReturnValue :type "Actor Object Reference"))
  (return (`self.GetOwner` (`self.AttachedObject`))))

(fn `GetParentPhysicsConstraint`
  (returns (`Physics Constraint Comp` :type "PhysicsConstraintComponent Object Reference"))
  (bind _asphysics_constraint_component (cast `PhysicsConstraintComponent` (`self.GetAttachParent`))
    (:`then`
      (return _asphysics_constraint_component))
    (:`CastFailed`
      (`KismetSystemLibrary.PrintString` (`KismetStringLibrary.Concat_StrStr` (`KismetSystemLibrary.GetDisplayName` self) " - Could not find Physics Constraint Component as Parent of this Attachment Slot.") true true (struct :`R` 1.0 :`B` 0.032956 :`A` 1.0))
      (return null))))

(fn `GetParentPrimitiveComponentOfSlot`
  (returns (`AsPrimitive Component` :type "PrimitiveComponent Object Reference") (`Socket Name` :type Name))
  (bind _asprimitive_component (cast `PrimitiveComponent` (`KismetMathLibrary.SelectObject` (`Actor.RootComponent` (`self.GetOwner`)) (`self.GetAttachParent`) (`self.UseRootComponentForParentPrimitive`)))
    (:`then`
      (return _asprimitive_component (select `bool` (`self.UseRootComponentForParentPrimitive`) :`false` (`self.GetAttachSocketName`))))
    (:`CastFailed`
      (return null "None"))))

(fn `GetValidAttachmentObjectClass`
  (returns (`Attachable Object Class` :type "/Game/VRGK/Blueprints/Systems/AttachmentSlots/BPC_AttachableObject Class Reference"))
  (return "/Game/VRGK/Blueprints/Systems/AttachmentSlots/BPC_AttachableObject.BPC_AttachableObject_C"))

(fn `Is Object Attached`
  (returns (True :type Boolean))
  (return (`KismetSystemLibrary.IsValid` (`self.AttachedObject`))))

(fn `Try Reset Attached Hand Hits`
  (params (`Attach Object` :type "/Game/VRGK/Blueprints/Systems/AttachmentSlots/BPC_AttachableObject Object Reference"))
  (locals (CheckedActors :type "Array of Actor Object Reference"))
  (`|ExecutionSequence`
    (:`then_0`
      (bind _handgrabcollisionupdater (`self.HandGrabCollisionUpdater`)
        (:`then`
          (`/Game/VRGK/Blueprints/Components/GrabCollisionUpdater/BPC_HandGrabUpdater.TryResetAllHandsHitEvents` _handgrabcollisionupdater)
          (`KismetArrayLibrary.Array_AddUnique` (`local.CheckedActors`) (`self.GetOwner` _handgrabcollisionupdater)))
        (:`else`)))
    (:`then_1`
      (bind _handgrabcollisionupdater_2 (`/Game/VRGK/Blueprints/Systems/AttachmentSlots/BPC_AttachableObject.HandGrabCollisionUpdater` `Attach Object`)
        (:`then`
          (`/Game/VRGK/Blueprints/Components/GrabCollisionUpdater/BPC_HandGrabUpdater.TryResetAllHandsHitEvents` _handgrabcollisionupdater_2)
          (`KismetArrayLibrary.Array_AddUnique` (`local.CheckedActors`) (`self.GetOwner` _handgrabcollisionupdater_2)))
        (:`else`)))
    (:`then_2`
      (bind (_asprimitive_component _socket_name) (`self.GetParentPrimitiveComponentOfSlot`))
      (`/Engine/EditorBlueprintResources/StandardMacros.IsValid` _asprimitive_component
        (:`Is Valid`
          (bind (_hasphysicsroot _physics_root) (`/Game/VRGK/Blueprints/BPFL_PhysicsObjects.GetPhysicsRoot` _asprimitive_component _socket_name))
          (`/Engine/EditorBlueprintResources/StandardMacros.IsValid` _physics_root
            (:`Is Valid`
              (for _array_element (`self.GetChildrenComponents` _physics_root true)
                (bind _returnvalue (`self.GetOwner` _array_element))
                (if (not (`KismetArrayLibrary.Array_Contains` (`local.CheckedActors`) _returnvalue))
                  (`KismetArrayLibrary.Array_AddUnique` (`local.CheckedActors`) _returnvalue)
                  (bind _returnvalue_2 (`Actor.GetComponentByClass` _returnvalue "/Game/VRGK/Blueprints/Components/GrabCollisionUpdater/BPC_HandGrabUpdater.BPC_HandGrabUpdater_C"))
                  (`/Engine/EditorBlueprintResources/StandardMacros.IsValid` _returnvalue_2
                    (:`Is Valid`
                      (`/Game/VRGK/Blueprints/Components/GrabCollisionUpdater/BPC_HandGrabUpdater.TryResetAllHandsHitEvents` _returnvalue_2))))))))))))

(fn `TryAttachActor`
  (params (`Other Actor` :type "Actor Object Reference"))
  (returns (Sucess :type Boolean))
  (`/Engine/EditorBlueprintResources/StandardMacros.IsValid` (`self.AttachedObject`)
    (:`Is Valid`
      (return false))
    (:`Is Not Valid`
      (bind (_sucess _target_object) (`self.CheckIfActorCanAttach` (`local.Other Actor`)))
      (if _sucess
        ;[1 0.4745 0.07292 1 32] Prepare and Do Attachment Events
        (set `self.AttachedObject` _target_object)
        (`/Game/VRGK/Blueprints/Systems/AttachmentSlots/BPC_AttachableObject.PrepareNewAttachment` (`self.AttachedObject`) self)
        (`/Game/VRGK/Blueprints/Systems/AttachmentSlots/BPC_AttachableObject.DoAttachmentToSlot` (`self.AttachedObject`))
        (`|ExecutionSequence`
          (:`then_0`
            (`self.Try Reset Attached Hand Hits` (`self.AttachedObject`)))
          (:`then_1`
            (`self.OnObjectDidAttach` (`self.AttachedObject`))
            (`|ExecutionSequence`
              (:`then_0`
                (bind _attachment_sound (`self.Attachment Sound`)
                  (:`then`
                    (`GameplayStatics.SpawnSoundAttached` _attachment_sound self "None" (0.0 0.0 0.0) (struct) "KeepRelativeOffset" false 1.0 1.0 0.0 null null))
                  (:`else`)))
              (:`then_1`
                (return true)))))
        (else
          (return false))))))

(fn `TryReleaseCurrentObject`
  (returns (Success :type Boolean) (`Released Object` :type "/Game/VRGK/Blueprints/Systems/AttachmentSlots/BPC_AttachableObject Object Reference"))
  (locals (TempAttachedObject :type "/Game/VRGK/Blueprints/Systems/AttachmentSlots/BPC_AttachableObject Object Reference"))
  (bind _output_get (set `local.TempAttachedObject` (`self.AttachedObject`)))
  (`/Engine/EditorBlueprintResources/StandardMacros.IsValid` _output_get
    (:`Is Valid`
      (if (`/Game/VRGK/Blueprints/Systems/AttachmentSlots/BPC_AttachableObject.CanRelease` _output_get)
        ;[1 0.6769 0.2569 1 32] Prepare and Do Release Events
        (`/Game/VRGK/Blueprints/Systems/AttachmentSlots/BPC_AttachableObject.PrepareRelease` (`self.AttachedObject`))
        (`/Game/VRGK/Blueprints/Systems/AttachmentSlots/BPC_AttachableObject.DoReleaseAttachment` (`self.AttachedObject`))
        (`self.OnObjectWasReleased` (`self.AttachedObject`))
        (set `self.AttachedObject` null)
        (`|ExecutionSequence`
          (:`then_0`
            (`self.Try Reset Attached Hand Hits` (`local.TempAttachedObject`)))
          (:`then_1`
            (`|ExecutionSequence`
              (:`then_0`
                (bind _detach_sound (`self.Detach Sound`)
                  (:`then`
                    (`GameplayStatics.SpawnSoundAttached` _detach_sound self "None" (0.0 0.0 0.0) (struct) "KeepRelativeOffset" false 1.0 1.0 0.0 null null))
                  (:`else`)))
              (:`then_1`
                (return true (`local.TempAttachedObject`))))))
        (else
          (return false null))))
    (:`Is Not Valid`
      (return false null))))