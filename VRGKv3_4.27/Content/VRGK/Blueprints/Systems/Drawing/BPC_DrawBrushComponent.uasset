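; Brush component that paints a textured, coloured brush onto actors carrying a BPC_DrawingComponent, driven by hit results and sizes passed to TryDrawAtHit.
; The first hit caches the target drawing component and stamps a dot, then hits in quick succession draw lines from the last stored hit.
; Movement is measured in the hit component's local space to skip negligible steps, and a short time gap clears the target to end the stroke.
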(event `TryDrawAtHit`
  (params (Hit :type "HitResult Structure") (Size :type "Float (double-precision)"))
  (bind _returnvalue (`Actor.GetComponentByClass` (`.HitActor` (`GameplayStatics.BreakHitResult` (`self.CurHit`))) "/Game/VRGK/Blueprints/Systems/Drawing/BPC_DrawingComponent.BPC_DrawingComponent_C"))
  (set `self.CurHit` Hit)
  (set `self.CurSize` Size)
  (`/Engine/EditorBlueprintResources/StandardMacros.IsValid` _returnvalue
    (:`Is Valid`
      (if (`KismetSystemLibrary.IsValid` (`self.CurTargetDrawing`))
        (if (< (- (`KismetSystemLibrary.GetGameTimeInSeconds`) (`self.LastHitTime`)) 0.2)
          (set `self.LastHitTime` (`KismetSystemLibrary.GetGameTimeInSeconds`))
          (if (> (`KismetMathLibrary.Vector_Distance` (`self.GetHitRelLocation` (`self.CurHit`)) (`self.LastLocation`)) 0.1)
            (`|ExecutionSequence`
              (:`then_0`
                (`self.CurTargetDrawing`
                  (:`then`
                    (`/Game/VRGK/Blueprints/Systems/Drawing/BPC_DrawingComponent.TryDrawTextureBrushLineWithHits` (`self.CurTargetDrawing`) (`self.LastHit`) (`self.CurHit`) (`self.LastSize`) (`self.CurSize`) (`self.Brush Texture`) (`self.Brush Color`)))
                  (:`else`)))
              (:`then_1`
                (`self.SetLastHit`))))
          (else
            (set `self.CurTargetDrawing` null)))
        (else
          (set `self.CurTargetDrawing` _returnvalue)
          (`self.SetLastHit`)
          (bind _curtargetdrawing (`self.CurTargetDrawing`)
            (:`then`
              (`/Game/VRGK/Blueprints/Systems/Drawing/BPC_DrawingComponent.TryDrawTextureBrushWithHit` _curtargetdrawing (`self.CurHit`) (`self.CurSize`) (`self.Brush Texture`) (`self.Brush Color`)))
            (:`else`)))))))

(event `SetLastHit`
  (set `self.LastHitTime` (`KismetSystemLibrary.GetGameTimeInSeconds`))
  (set `self.LastSize` (`self.CurSize`))
  (set `self.LastHit` (`self.CurHit`))
  (set `self.LastLocation` (`self.GetHitRelLocation` (`self.CurHit`))))

(fn `GetHitRelLocation`
  (params (Hit :type "HitResult Structure (by ref)"))
  (returns (ReturnValue :type "Vector Structure"))
  (bind (_bblockinghit _binitialoverlap _time _distance _location _impactpoint _normal _impactnormal _physmat _hitactor _hitcomponent) (`GameplayStatics.BreakHitResult` Hit))
  (bind (_returnvalue_location _returnvalue_rotation) (`KismetMathLibrary.BreakTransform` (`self.K2_GetComponentToWorld` _hitcomponent)))
  (return (`KismetMathLibrary.InverseTransformLocation` (`KismetMathLibrary.MakeTransform` _returnvalue_location _returnvalue_rotation) _impactpoint)))