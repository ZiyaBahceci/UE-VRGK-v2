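; Physical input component for a VR knob that turns the child primitive's rotation into a value and velocity.
; Each tick it accumulates rotation deltas on the chosen axis and broadcasts the result.
; In welded, constraint-free mode it sums tracked hands' angular offsets, interpolates the knob's yaw with optional limits, then updates grab constraints.
; Hand angles come from position when off-axis, or from hand orientation when near the center.
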(event `self.SetupPhysicalInput`
  (params (ParentPhysicsConstraint :type "PhysicsConstraintComponent Object Reference") (ChildPrimitiveComponent :type "PrimitiveComponent Object Reference"))
  (`parent.SetupPhysicalInput` ParentPhysicsConstraint ChildPrimitiveComponent)
  (set `self.LastRawRotation` (`self.GetKnobRotation`)))

(event `self.Physical Input Tick`
  (params (`Delta Seconds` :type "Float (single-precision)"))
  (bind _currentinputdeltaseconds (`self.CurrentInputDeltaSeconds`))
  (bind (_returnvalue_roll _returnvalue_pitch _returnvalue_yaw) (`KismetMathLibrary.BreakRotator` (`KismetMathLibrary.NormalizedDeltaRotator` (`self.TempRotation`) (`self.LastRawRotation`))))
  (bind _returnvalue (select `/Game/VRGK/Blueprints/Systems/PhysicalInputs/Enum_PhysicalInputDirection` (`self.Direction`) :`NewEnumerator0` _returnvalue_roll :`NewEnumerator1` _returnvalue_pitch :`NewEnumerator2` _returnvalue_yaw))
  (`parent.Physical Input Tick` `Delta Seconds`)
  (`|ExecutionSequence`
    (:`then_0`
      ;[1 1 1] Calculate current Knob Values
      (if (> _currentinputdeltaseconds 0.0)
        (set `self.TempRotation` (`self.GetKnobRotation`))
        (set `self.TempValue` (+ (`self.CurrentValue`) _returnvalue))
        (set `self.CurrentVelocity` (`KismetMathLibrary.SelectFloat` 0.0 (* _returnvalue (/ 1.0 _currentinputdeltaseconds)) (== _currentinputdeltaseconds 0.0)))
        (set `self.CurrentValue` (`self.TempValue`))
        (`self.OnKnobValueChange` self (`self.CurrentValue`) (`self.CurrentVelocity`))
        (set `self.LastRawRotation` (`self.TempRotation`))))
    (:`then_1`
      (`self.DoWeldedTick`))))

(event `DoWeldedTick`
  (bind (_rotationlimitrange_min _rotationlimitrange_max) (break `InputRange` (`self.RotationLimitRange`)))
  (bind (_relativerotation_roll _relativerotation_pitch) (`KismetMathLibrary.BreakRotator` (`SceneComponent.RelativeRotation` (`self.ChildPrimitiveComponent`))))
  (bind (_relativerotation_roll_2 _relativerotation_pitch_2 _relativerotation_yaw) (`KismetMathLibrary.BreakRotator` (`SceneComponent.RelativeRotation` (`self.ChildPrimitiveComponent`))))
  (bind _returnvalue (`KismetMathLibrary.FInterpTo` _relativerotation_yaw (+ _relativerotation_yaw (`KismetMathLibrary.FClamp` (`self.TargetRot`) -90.0 90.0)) (`self.CurrentInputDeltaSeconds`) (`self.WeldedInterpSpeed`)))
  (switch `/Game/VRGK/Blueprints/Systems/PhysicalInputs/Enum_PhysicalInputInteractionmode` (`self.Interaction Mode`)
    (:`NewEnumerator1`
      (if (> (- (`self.OwnersGameTimeSinceCreation`) (`self.GameTimeOnUpdateEnabled`)) 0.0)
        (bind _calculated (`self.Calculate Current Hand Target Rotation Offset`))
        (set `self.TargetRot` _calculated)
        (`self.K2_SetRelativeRotation` (`self.ChildPrimitiveComponent`) (`KismetMathLibrary.MakeRotator` _relativerotation_roll _relativerotation_pitch (`KismetMathLibrary.SelectFloat` (`KismetMathLibrary.FClamp` _returnvalue _rotationlimitrange_min _rotationlimitrange_max) _returnvalue (`self.LimitRotation`))) false false)
        (`/Game/VRGK/Blueprints/Player/Hand/BP_VRHand.Update Grab Constraint Frames from Grab` (`self.TrackedHandArray`))))))

(fn `Calculate Current Hand Target Rotation Offset`
  (returns (Calculated :type "Float (double-precision)"))
  (locals (TempRot :type "Float (double-precision)") (TempHand :type "/Game/VRGK/Blueprints/Player/Hand/BP_VRHand Object Reference"))
  (bind _returnvalue (`self.K2_GetComponentToWorld`))
  (bind _temphand (`local.TempHand`))
  (bind _returnvalue_location (`KismetMathLibrary.BreakTransform` (`/Game/VRGK/Blueprints/Player/Hand/BP_VRHand.GetSocketRelativeGrabRootTransform` _temphand)))
  (bind (_returnvalue_location_2 _returnvalue_rotation) (`KismetMathLibrary.BreakTransform` (`/Game/VRGK/Blueprints/Player/Hand/BP_VRHand.GetSocketRelativeGrabRootTransform` (`local.TempHand`))))
  (bind _returnvalue_location_3 (`KismetMathLibrary.BreakTransform` (`self.K2_GetComponentToWorld` (`/Game/VRGK/Blueprints/Player/Hand/BP_VRHand.GrabRoot` (`local.TempHand`)))))
  (bind _returnvalue_2 (`KismetMathLibrary.InverseTransformRotation` (`self.K2_GetComponentToWorld`) _returnvalue_rotation))
  (bind _returnvalue_location_4 (`KismetMathLibrary.BreakTransform` (`self.K2_GetComponentToWorld` (`/Game/VRGK/Blueprints/Player/Hand/BP_VRHand.GrabRoot` _temphand))))
  (bind _returnvalue_3 (`KismetMathLibrary.InverseTransformRotation` (`self.K2_GetComponentToWorld`) (`self.K2_GetComponentRotation` (`/Game/VRGK/Blueprints/Player/Hand/BP_VRHand.GrabRoot` (`local.TempHand`)))))
  (bind (_returnvalue_x _returnvalue_y) (`KismetMathLibrary.BreakVector` (`KismetMathLibrary.InverseTransformLocation` (`self.K2_GetComponentToWorld`) _returnvalue_location_3)))
  (bind _returnvalue_4 (> (`KismetMathLibrary.VSize2D` (`KismetMathLibrary.MakeVector2D` _returnvalue_x _returnvalue_y)) 15.0))
  (bind _returnvalue_5 (`KismetMathLibrary.InRange_FloatFloat` (`KismetMathLibrary.Dot_VectorVector` (`KismetMathLibrary.GetUpVector` _returnvalue_3) (0.0 0.0 1.0)) -0.5 0.5))
  (bind (_returnvalue_roll _returnvalue_pitch _returnvalue_yaw) (`KismetMathLibrary.BreakRotator` (`KismetMathLibrary.NormalizedDeltaRotator` (`KismetMathLibrary.MakeRotator` 0.0 0.0 (`KismetMathLibrary.DegAtan2` (.y (`KismetMathLibrary.SelectVector` (`KismetMathLibrary.InverseTransformLocation` _returnvalue _returnvalue_location) (* (`KismetMathLibrary.SelectVector` (`KismetMathLibrary.GetUpVector` _returnvalue_2) (* (`KismetMathLibrary.GetForwardVector` _returnvalue_2) -1.0) _returnvalue_5) 50.0) _returnvalue_4)) (.x (`KismetMathLibrary.SelectVector` (`KismetMathLibrary.InverseTransformLocation` _returnvalue _returnvalue_location) (* (`KismetMathLibrary.SelectVector` (`KismetMathLibrary.GetUpVector` _returnvalue_2) (* (`KismetMathLibrary.GetForwardVector` _returnvalue_2) -1.0) _returnvalue_5) 50.0) _returnvalue_4)))) (`KismetMathLibrary.MakeRotator` 0.0 0.0 (`KismetMathLibrary.DegAtan2` (.y (`KismetMathLibrary.SelectVector` (`KismetMathLibrary.InverseTransformLocation` _returnvalue _returnvalue_location_4) (* (`KismetMathLibrary.SelectVector` (`KismetMathLibrary.GetUpVector` _returnvalue_3) (* (`KismetMathLibrary.GetForwardVector` _returnvalue_3) -1.0) _returnvalue_5) 50.0) _returnvalue_4)) (.x (`KismetMathLibrary.SelectVector` (`KismetMathLibrary.InverseTransformLocation` _returnvalue _returnvalue_location_4) (* (`KismetMathLibrary.SelectVector` (`KismetMathLibrary.GetUpVector` _returnvalue_3) (* (`KismetMathLibrary.GetForwardVector` _returnvalue_3) -1.0) _returnvalue_5) 50.0) _returnvalue_4)))))))
  (set `local.TempRot` 0.0)
  (for _array_element (`self.TrackedHandArray`)
    (set `local.TempHand` _array_element)
    (set `local.TempRot` (+ (`local.TempRot`) _returnvalue_yaw)))
  (return (`local.TempRot`)))

(fn `GetCurrentKnobValue`
  (returns (CurrentValue :type "Float (double-precision)") (CurrentVelocity :type "Float (double-precision)"))
  (return (`self.CurrentValue`) (`self.CurrentVelocity`)))

(fn `GetKnobRotation`
  (returns (ReturnValue :type "Rotator Structure"))
  (return (`KismetMathLibrary.InverseTransformRotation` (`self.K2_GetComponentToWorld`) (`self.K2_GetComponentRotation` (`self.ChildPrimitiveComponent`)))))