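; VR player vignette actor that attaches to the player camera manager and fades a vignette mesh in and out.
; A timeline, tickable while paused, drives alpha into the mesh's custom primitive data, scaled by the strength setting, and hides the actor after fading out.
; Showing respects the enabled setting and can be instant via a raised play rate.
; Temporary shows use a short retriggerable delay before reversing the fade.
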(event `self.ReceiveBeginPlay`
  (`self.K2_AttachToActor` self (`GameplayStatics.GetPlayerCameraManager` 0) "None" "SnapToTarget" "SnapToTarget" "KeepWorld" false)
  (`self.HideVignette`)
  (`ActorComponent.SetTickableWhenPaused` (`self.VignetteTimeline`) true)
  (bind _settings (`/Game/VRGK/Blueprints/BPFL_GlobalFunctions.Get BPO Game Settings`))
  (bind _output_get (set `self.Settings` _settings))
  (add `/Game/VRGK/Blueprints/Core/BPO_Settings.OnPlayerVignetteChanged` _output_get (delegate `OnVignetteSettingsChanged`)))

(event `OnVignetteSettingsChanged`
  (params (Enabled :type Boolean))
  (`self.SetVignetteAlpha` (`self.CurAlpha`)))

(event `self.ReceiveTick`
  (params (DeltaSeconds :type "Float (single-precision)")))

(event `ShowVignetteTemporary`
  (params (Instant :type Boolean))
  (if (`/Game/VRGK/Blueprints/Core/BPO_Settings.GetPlayerVignetteEnabled` (`self.Settings`))
    (`self.ShowVignette` Instant)
    (`KismetSystemLibrary.RetriggerableDelay` 0.05)
    (`self.HideVignette`)))

(event `SetVignetteAlpha`
  (params (Alpha :type "Float (double-precision)"))
  (bind _output_get (set `self.CurAlpha` Alpha))
  (`PrimitiveComponent.SetCustomPrimitiveDataFloat` (`self.VignetteMesh`) 0 (* _output_get (`/Game/VRGK/Blueprints/Core/BPO_Settings.GetPlayerVignetteStrength` (`self.Settings`)))))

(event `ShowVignette`
  (params (Instant :type Boolean))
  (if (`/Game/VRGK/Blueprints/Core/BPO_Settings.GetPlayerVignetteEnabled` (`self.Settings`))
    (if Instant
      (`TimelineComponent.SetPlayRate` (`self.VignetteTimeline`) (`KismetMathLibrary.SelectFloat` 100.0 1.0 Instant) :!label _label)
      (`|ExecutionSequence`
        (:`then_0`
          (if (`self.bHidden`)
            (`self.SetActorHiddenInGame` false)))
        (:`then_1`
          (bind (_direction _alpha) (`Timeline|VignetteTimeline` :!label _label_2)
            (:`Update`
              (`self.SetVignetteAlpha` _alpha :!label _label_3))
            (:`Finished`
              (`|ExecutionSequence`
                (:`then_0`
                  (goto _label_3))
                (:`then_1`
                  (switch `ETimelineDirection` _direction
                    (:`Backward`
                      (`self.SetActorHiddenInGame` true)))))))))
      (elif (`self.bHidden`)
        (goto _label)))))

(event `HideVignette`
  (`TimelineComponent.SetPlayRate` (`self.VignetteTimeline`) 1.0)
  (goto _label_2 :!via `Reverse`))

(fn `UserConstructionScript`)