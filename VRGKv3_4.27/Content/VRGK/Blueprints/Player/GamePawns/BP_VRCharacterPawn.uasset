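; VR player pawn built on character movement, with sprinting, jumping, climbing, teleport and turning, supplying transforms for the VR avatar.
; Each tick it updates the neck and ground component, then re-centres the VR origin and shifts the capsule toward the head if a trace is clear, during input movement or with avatar enabled.
; Climbing disables movement, moves the actor opposite hand pull, and launches it on release using a constrained tracker sphere's velocity.
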(event `self.ReceiveBeginPlay`
  (bind (_relativelocation_x _relativelocation_y _relativelocation_z) (`KismetMathLibrary.BreakVector` (`SceneComponent.RelativeLocation` (`self.VRFloorRoot`))))
  (`|ExecutionSequence`
    (:`then_0`
      (`self.SetupVelocityTracker`)
      (set `self.VRFloorTargetZ` _relativelocation_z))
    (:`then_1`
      (`parent.ReceiveBeginPlay`))))

(event `self.ReceiveTick`
  (params (DeltaSeconds :type "Float (single-precision)"))
  (`parent.ReceiveTick` DeltaSeconds)
  (`|ExecutionSequence`
    (:`then_0`
      (`self.MovementUpdateTick` DeltaSeconds)
      (set `CharacterMovementComponent.MaxWalkSpeed` (`KismetMathLibrary.SelectFloat` 800.0 400.0 (`self.IsSprinting`)) (`self.CharacterMovement`)))
    (:`then_1`
      (`self.VRAvatar Tick` DeltaSeconds))))

(event `SetupVelocityTracker`
  (bind _velocitytrackerconstraint (`self.VelocityTrackerConstraint`))
  (`PhysicsConstraintComponent.SetConstrainedComponents` (`self.VelocityTrackerConstraint`) (`self.VelocityTrackerSphere`) "None" (`self.CapsuleComponent`) "None")
  (`PhysicsConstraintComponent.SetConstraintReferenceFrame` _velocitytrackerconstraint "Frame1" (`KismetMathLibrary.MakeTransform` (0.0 0.0 0.0)))
  (`PhysicsConstraintComponent.SetConstraintReferenceFrame` _velocitytrackerconstraint "Frame2" (`KismetMathLibrary.MakeTransform` (0.0 0.0 0.0))))

(event `self.OnPlayerCalibrationUpdate`
  (params (Settings :type "/Game/VRGK/Blueprints/Core/BPO_Settings Object Reference"))
  (`parent.OnPlayerCalibrationUpdate` Settings)
  (`SceneComponent.K2_SetRelativeLocation` (`self.VRFloorRoot`) (`KismetMathLibrary.MakeVector` 0.0 0.0 (+ (`self.VRFloorTargetZ`) (`self.Get Current Play Mode Height Difference`))) false false))

(event `MovementUpdateTick`
  (params (DeltaSeconds :type "Float (double-precision)"))
  ;[1 1 1] Movement Tick
  (set `self.WorldInputVector` (`PawnMovementComponent.GetLastInputVector` (`self.CharacterMovement`)))
  (`self.UpdateNeckPosition`)
  (`self.CheckGroundComponent`)
  (`self.UpdateCameraBodyOffset`)
  (`self.UpdateClimbing`))

(event `UpdateClimbing`
  (bind _returnvalue (`self.K2_GetActorLocation`))
  (bind _lefthand (`self.LeftHand`))
  (bind _righthand (`self.RightHand`))
  (bind _returnvalue_2 (or (`/Game/VRGK/Blueprints/Player/Hand/BP_VRHand.GrabHasClimbingTag` (`self.LeftHand`)) (`/Game/VRGK/Blueprints/Player/Hand/BP_VRHand.GrabHasClimbingTag` (`self.RightHand`))))
  (bind _returnvalue_3 (`KismetMathLibrary.VInterpTo` _returnvalue (+ _returnvalue (* (+ (`KismetMathLibrary.SelectVector` (`/Game/VRGK/Blueprints/Player/Hand/BP_VRHand.Get Physics Climb Vector` _lefthand) (0.0 0.0 0.0) (`/Game/VRGK/Blueprints/Player/Hand/BP_VRHand.GrabHasClimbingTag` _lefthand)) (`KismetMathLibrary.SelectVector` (`/Game/VRGK/Blueprints/Player/Hand/BP_VRHand.Get Physics Climb Vector` _righthand) (0.0 0.0 0.0) (`/Game/VRGK/Blueprints/Player/Hand/BP_VRHand.GrabHasClimbingTag` _righthand))) -1.0)) (`GameplayStatics.GetWorldDeltaSeconds`) 20.0))
  ;[1 1 1] Climbing
  (`|ExecutionSequence`
    (:`then_0`
      (if (!= _returnvalue_2 (`self.PlayerIsClimbing`))
        (bind _output_get (set `self.PlayerIsClimbing` _returnvalue_2))
        (if _output_get
          (`CharacterMovementComponent.DisableMovement` (`self.CharacterMovement`))
          (else
            (`CharacterMovementComponent.SetMovementMode` (`self.CharacterMovement`) "MOVE_Walking" 0)
            (`self.LaunchCharacter` (`SceneComponent.GetComponentVelocity` (`self.VelocityTrackerSphere`)) true true)))))
    (:`then_1`
      (if (`self.PlayerIsClimbing`)
        (set `self.LastClimbOffset` (- _returnvalue_3 _returnvalue))
        (`self.K2_SetActorLocation` _returnvalue_3)))))

(event `UpdateCameraBodyOffset`
  (bind _capsulecomponent (`self.CapsuleComponent`))
  (bind _returnvalue (`SceneComponent.K2_GetComponentLocation` (`self.CapsuleComponent`)))
  ;[1 1 1] Update Offset from Camera to Body.
  (if (or (`self.Is VR Player Moving With Input`) (`self.IsVR AvatarEnabled`))
    (`|ExecutionSequence`
      (:`then_0`
        (`self.ResetCameraToCapsule`))
      (:`then_1`
        (set `self.TempCapsuleOffset` (`KismetMathLibrary.TransformDirection` (`self.GetTransform`) (`KismetMathLibrary.MakeVector` (.x (* (`self.TempCameraOffset`) 1.0)) (.y (* (`self.TempCameraOffset`) 1.0)))))
        (bind (_outhit _returnvalue_2) (`KismetSystemLibrary.CapsuleTraceSingleByProfile` :`Start` _returnvalue :`End` (+ _returnvalue (`self.TempCapsuleOffset`)) :`Radius` (* (`CapsuleComponent.CapsuleRadius` _capsulecomponent) 0.9) :`HalfHeight` (* (`CapsuleComponent.CapsuleHalfHeight` _capsulecomponent) 0.9) :`ProfileName` "VRCharacterPawn" :`DrawDebugType` "ForOneFrame"))
        (if (not _returnvalue_2)
          (`SceneComponent.K2_AddWorldOffset` (`self.CapsuleComponent`) (`self.TempCapsuleOffset`) false false))))))

(event `ResetCameraToCapsule`
  (bind (_returnvalue_x _returnvalue_y) (`KismetMathLibrary.BreakVector` (* (`self.TempCameraOffset`) -1.0)))
  ;[1 1 1] Update Offset from Camera to Body.
  (set `self.TempCameraOffset` (`KismetMathLibrary.InverseTransformLocation` (`self.GetTransform`) (`SceneComponent.K2_GetComponentLocation` (`self.NeckRoot`))))
  (`SceneComponent.K2_AddLocalOffset` (`self.VROriginRoot`) (`KismetMathLibrary.MakeVector` _returnvalue_x _returnvalue_y) false false))

(event `UpdateNeckPosition`
  ;[1 1 1] Update Neck Position
  (`SceneComponent.K2_SetRelativeLocation` (`self.NeckRoot`) (`self.CalculateNeckPosition` (`SceneComponent.RelativeLocation` (`self.HeadRoot`))) false true))

(event `CheckGroundComponent`
  (bind (_bblockinghit _binitialoverlap _time _distance _location _impactpoint _normal _impactnormal _physmat _hitactor _hitcomponent) (`GameplayStatics.BreakHitResult` (`.HitResult` (break `FindFloorResult` (`CharacterMovementComponent.CurrentFloor` (`self.CharacterMovement`))))))
  ;[1 1 1] Updated Floor/Ground Component
  (if (!= (`self.CurrentGroundComponent`) _hitcomponent)
    (set `self.CurrentGroundComponent` _hitcomponent)
    (`self.OnGroundChange` false)))

(event `self.DoPlayerJumpPressed`
  (`self.Jump`))

(fn `Calculate Avatar Body World Rotation`
  (returns (ReturnValue :type "Rotator Structure"))
  (return (`parent.Calculate Avatar Body World Rotation`)))

(fn `Get Avatar Movement Status`
  (returns (ShouldWalk :type Boolean))
  (return (`NavMovementComponent.IsMovingOnGround` (`self.CharacterMovement`))))

(fn `Get Ground Transform`
  (returns (`Ground Transform` :type "Transform Structure"))
  (bind (_returnvalue_location _returnvalue_rotation) (`KismetMathLibrary.BreakTransform` (`SceneComponent.K2_GetComponentToWorld` (`self.Mesh`))))
  (bind _currentgroundcomponent (`self.CurrentGroundComponent`)
    (:`then`
      (bind (_returnvalue_location_2 _returnvalue_rotation_2) (`KismetMathLibrary.BreakTransform` (`SceneComponent.K2_GetComponentToWorld` _currentgroundcomponent)))
      (return (`KismetMathLibrary.MakeTransform` _returnvalue_location_2 _returnvalue_rotation_2)))
    (:`else`
      (return (`KismetMathLibrary.MakeTransform` _returnvalue_location _returnvalue_rotation)))))

(fn `GetAvatarFloor`
  (returns (ReturnValue :type "Vector Structure"))
  (return (`KismetMathLibrary.TransformLocation` (`SceneComponent.K2_GetComponentToWorld` (`self.CapsuleComponent`)) (`KismetMathLibrary.MakeVector` 0.0 0.0 (`self.VRFloorTargetZ`)))))

(fn `GetAvatarHeadRotationDelta`
  (returns (Delta :type "Float (double-precision)"))
  (return (`parent.GetAvatarHeadRotationDelta`)))

(fn `GetAvatarRotationSpeed`
  (params (TargetRotation :type "Rotator Structure"))
  (returns (`Alpha Speed` :type "Float (double-precision)"))
  (return (`parent.GetAvatarRotationSpeed` TargetRotation)))

(fn `GetAvatarTransforms`
  (returns (HeadTransform :type "Transform Structure") (NeckLocation :type "Vector Structure") (CurBodyHeight :type "Float (double-precision)") (FullBodyHeight :type "Float (double-precision)"))
  (return (`/Game/VRGK/Blueprints/BPFL_GlobalFunctions.TransformTransform` (`SceneComponent.K2_GetComponentToWorld` (`self.Camera`)) (`KismetMathLibrary.MakeTransform` (-5.0 0.0 0.0))) (`SceneComponent.K2_GetComponentLocation` (`self.CapsuleComponent`)) (`KismetMathLibrary.Vector_Distance` (`SceneComponent.K2_GetComponentLocation` (`self.Mesh`)) (`SceneComponent.K2_GetComponentLocation` (`self.Camera`))) (`self.GetCurrentTotalPlayerHeight`)))

(fn `GetAvatarVelocity`
  (returns (`World Space Velocity` :type "Vector Structure"))
  (return (`self.GetVelocity`)))

(fn `RotateVRPawn`
  (params (TurnDegrees :type "Float (double-precision)"))
  (`self.K2_AddActorLocalRotation` (`KismetMathLibrary.MakeRotator` 0.0 0.0 TurnDegrees)))

(fn `TeleportVRPawn`
  (params (NewLocation :type "Vector Structure") (`With Hands` :type Boolean))
  (`self.K2_SetActorLocation` NewLocation)
  (`self.OnGroundChange` true)
  (`self.ResetCameraToCapsule`)
  (`/Game/VRGK/Blueprints/Player/Hand/BP_VRHand.PhysicsToHandTeleport` (`self.LeftHand`))
  (`/Game/VRGK/Blueprints/Player/Hand/BP_VRHand.PhysicsToHandTeleport` (`self.RightHand`)))

(fn `UserConstructionScript`
  (`parent.UserConstructionScript`))