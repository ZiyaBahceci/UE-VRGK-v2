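; BP_VRMenuPawn is the VR pawn used while a menu is open, letting the player point at and click widgets with both hands.
; On BeginPlay it copies transforms from the VR player pawn, offsets the hand roots for the HMD device and caches both pointer child actors.
; Tick places each pointer at its widget interaction hit, shown only over hit-testable widgets.
; Triggers act as left mouse clicks, and the menu button closes the menu through the game mode's menu controller.
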(event `self.ReceiveBeginPlay`
  (bind (_handpivot_location _handpivot_rotation) (`KismetMathLibrary.BreakTransform` (`/Game/VRGK/Blueprints/BPFL_GlobalFunctions.GetHandDevicePivot` "NewEnumerator0")))
  (bind (_handpivot_location_2 _handpivot_rotation_2) (`KismetMathLibrary.BreakTransform` (`/Game/VRGK/Blueprints/BPFL_GlobalFunctions.GetHandDevicePivot` "NewEnumerator1")))
  (`parent.ReceiveBeginPlay`)
  (`self.CopyVRTransformsForComponents` (`self.VRPlayerPawn`))
  (`|ExecutionSequence`
    (:`then_0`
      ;[1 1 1] Update Hand Pivot Positions based on HMD Device
      (`|ExecutionSequence`
        (:`then_0`
          (`SceneComponent.K2_SetRelativeLocationAndRotation` (`self.HandRootLeft`) _handpivot_location_2 _handpivot_rotation_2 false false))
        (:`then_1`
          (`SceneComponent.K2_SetRelativeLocationAndRotation` (`self.HandRootRight`) _handpivot_location _handpivot_rotation false false))))
    (:`then_1`
      ;[1 1 1] Prepare Pointer Actors
      (`|ExecutionSequence`
        (:`then_0`
          (bind _asbp_menu_pointer (cast `/Game/VRGK/Blueprints/Player/Menu/BP_MenuPointer` (`ChildActorComponent.ChildActor` (`self.PointerRight`))))
          (set `self.MenuPointerRight` _asbp_menu_pointer))
        (:`then_1`
          (bind _asbp_menu_pointer_2 (cast `/Game/VRGK/Blueprints/Player/Menu/BP_MenuPointer` (`ChildActorComponent.ChildActor` (`self.PointerLeft`))))
          (set `self.MenuPointerLeft` _asbp_menu_pointer_2))))))

(event `SetPointerTransform`
  (params (WidgetInteraction :type "WidgetInteractionComponent Object Reference") (Pointer :type "/Game/VRGK/Blueprints/Player/Menu/BP_MenuPointer Object Reference"))
  (bind (_returnvalue_bblockinghit _returnvalue_binitialoverlap _returnvalue_time _returnvalue_distance _returnvalue_location _returnvalue_impactpoint _returnvalue_normal _returnvalue_impactnormal _returnvalue_physmat _returnvalue_hitactor _returnvalue_hitcomponent _returnvalue_hitbonename _returnvalue_hititem _returnvalue_elementindex _returnvalue_faceindex _returnvalue_tracestart _returnvalue_traceend) (`GameplayStatics.BreakHitResult` (`WidgetInteractionComponent.GetLastHitResult` WidgetInteraction)))
  ;[1 1 1] Set Pointer Transform
  (`self.SetActorHiddenInGame` Pointer (not (`WidgetInteractionComponent.IsOverHitTestVisibleWidget` WidgetInteraction)))
  (`self.K2_SetActorLocationAndRotation` Pointer _returnvalue_impactpoint (`KismetMathLibrary.MakeRotFromZ` _returnvalue_impactnormal) false false)
  (`SceneComponent.K2_SetWorldRotation` (`/Game/VRGK/Blueprints/Player/Menu/BP_MenuPointer.PointerRoot` Pointer) (`KismetMathLibrary.ComposeRotators` (struct :`Pitch` 90.0) (`KismetMathLibrary.FindLookAtRotation` _returnvalue_tracestart _returnvalue_traceend)) false false))

(event `self.ReceiveTick`
  (params (DeltaSeconds :type "Float (single-precision)"))
  ;[1 1 1] Event Tick / Update Pointer Transforms
  (`self.SetPointerTransform` (`self.WidgetInteractionLeft`) (`self.MenuPointerLeft`))
  (`self.SetPointerTransform` (`self.WidgetInteractionRight`) (`self.MenuPointerRight`)))

(event `InputAction|PlayerTriggerLeft`
  (params (Key :type "Key Structure"))
  (bind _widgetinteractionleft (`self.WidgetInteractionLeft`))
  ;[1 1 1] Widget Interaction
  (:`Pressed`
    (`WidgetInteractionComponent.PressPointerKey` _widgetinteractionleft "LeftMouseButton"))
  (:`Released`
    (`WidgetInteractionComponent.ReleasePointerKey` _widgetinteractionleft "LeftMouseButton")))

(event `InputAction|PlayerMenu`
  (params (Key :type "Key Structure"))
  ;[1 1 1] Close Menu Action
  (:`Pressed`
    (bind _menucontroller (message `/Game/VRGK/Blueprints/Core/BPI_VRGameMode.GetMenuController` (`GameplayStatics.GetGameMode`)))
    (`/Game/VRGK/Blueprints/Core/BP_MenuController.CloseMenu` _menucontroller)))

(event `InputAction|PlayerTriggerRight`
  (params (Key :type "Key Structure"))
  (bind _widgetinteractionright (`self.WidgetInteractionRight`))
  ;[1 1 1] Widget Interaction
  (:`Pressed`
    (`WidgetInteractionComponent.PressPointerKey` _widgetinteractionright "LeftMouseButton"))
  (:`Released`
    (`WidgetInteractionComponent.ReleasePointerKey` _widgetinteractionright "LeftMouseButton")))

(fn `UserConstructionScript`)