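; BPC_GF_CustomGravity is a gravity field component that replaces engine gravity on its owning actor with a custom directional pull.
; On BeginPlay it disables gravity on the owner's physics-simulating primitive components and caches them.
; Each Tick it applies a mass-independent acceleration to those still simulating, opposite the normalized GravityDirection and scaled by GravityStrength and GravityMultiplier.
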(event `self.ReceiveBeginPlay`
  ;[1 1 1] Begin Play and Setup. Find all Primitive Components of the Owner Actor.
  (for _array_element (`Actor.K2_GetComponentsByClass` (`self.GetOwner`) "/Script/Engine.PrimitiveComponent")
    (if (`SceneComponent.IsSimulatingPhysics` _array_element "None")
      (`PrimitiveComponent.SetEnableGravity` _array_element false)
      (`KismetArrayLibrary.Array_Add` (`self.PrimitiveComponents`) _array_element))))

(event `self.ReceiveTick`
  (params (DeltaSeconds :type "Float (single-precision)"))
  (`self.UpdatePhysics`))

(event `UpdatePhysics`
  ;[1 1 1] Add Physics Force to simulate Gravity.
  (for _array_element (`self.PrimitiveComponents`)
    (if (`SceneComponent.IsSimulatingPhysics` _array_element "None")
      (`PrimitiveComponent.AddForce` _array_element (* (`KismetMathLibrary.Normal` (`self.GravityDirection`)) (* (`self.GravityStrength`) -1.0 (`self.GravityMultiplier`))) "None" true))))