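; A VR player pawn that moves by traces instead of swept collision, with walk and sprint speeds.
; Each tick, capsule traces bend input along walls using a reflection-derived slide direction, stopping it when a second trace is also blocked.
; Moving or rotating re-centres the body capsule under the camera and reverts it to the last valid location on overlap or missing floor.
; A downward sphere trace sets the target height, which the actor smoothly follows.
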(event `self.ReceiveBeginPlay`
  (`parent.ReceiveBeginPlay`)
  (`self.MovementBeginPlay`))

(event `self.ReceiveTick`
  (params (DeltaSeconds :type "Float (single-precision)"))
  (`parent.ReceiveTick` DeltaSeconds)
  (`|ExecutionSequence`
    (:`then_0`
      (`self.MovementTick` DeltaSeconds))))

(event `MovementBeginPlay`
  (bind (_returnvalue_x _returnvalue_y _returnvalue_z) (`KismetMathLibrary.BreakVector` (`SceneComponent.K2_GetComponentLocation` (`self.CapsuleComponent`))))
  ;[1 1 1] Begin Play for Movement Events
  (set `self.LastValidPawnLocation` (`SceneComponent.K2_GetComponentLocation` (`self.CapsuleComponent`)))
  (set `self.TargetZ` _returnvalue_z))

(event `MovementTick`
  (params (`Delta Seconds` :type "Float (double-precision)"))
  (bind (_returnvalue_x _returnvalue_y _returnvalue_z) (`KismetMathLibrary.BreakVector` (`self.K2_GetActorLocation`)))
  (bind _returnvalue (`KismetMathLibrary.Normal` (`self.TempMovementInputVector`)))
  (bind _returnvalue_2 (`KismetMathLibrary.VSize` (`self.TempMovementInputVector`)))
  (bind _returnvalue_3 (* `Delta Seconds` (`self.CurrentMovementInputSpeed`) (`KismetMathLibrary.SelectFloat` (`self.SprintSpeed`) (`self.MovementSpeed`) (`self.IsSprinting`))))
  (`|ExecutionSequence`
    (:`then_0`
      (bind _returnvalue_4 (`self.ConsumeMovementInputVector`))
      (set `self.TempMovementInputVector` _returnvalue_4)
      ;[1 1 1] First Trace.
      (bind (_outhit _returnvalue_5) (`self.DoMovementTrace` (`SceneComponent.K2_GetComponentLocation` (`self.CapsuleComponent`)) (`self.TempMovementInputVector`) (`self.TraceLength`) 8.0 70.0))
      (if _returnvalue_5
        (bind (_bblockinghit _binitialoverlap _time _distance _location _impactpoint _normal) (`GameplayStatics.BreakHitResult` _outhit))
        (set `self.TempDistanceValue` (`KismetMathLibrary.FClamp` (/ (- _distance 15.0) 5.0)))
        (bind _outvector (`self.GetWallDirection` _returnvalue (`KismetMathLibrary.Normal` (`KismetMathLibrary.ProjectVectorOnToPlane` _normal (0.0 0.0 1.0)))))
        (set `self.CurrentMovementVector` (`KismetMathLibrary.VLerp` _outvector _returnvalue (`self.TempDistanceValue`)))
        (set `self.CurrentMovementInputSpeed` (`KismetMathLibrary.Lerp` (* _returnvalue_2 (`KismetMathLibrary.Dot_VectorVector` _returnvalue _outvector)) _returnvalue_2 (`self.TempDistanceValue`)))
        ;[1 1 1] Second Trace, If Blocked
        (bind (_outhit_2 _returnvalue_6) (`self.DoMovementTrace` (`.Location` (`GameplayStatics.BreakHitResult` _outhit)) (`self.CurrentMovementVector`) 30.0 4.0 50.0))
        (if (and _returnvalue_6 (<= (`self.TempDistanceValue`) 0.01))
          (set `self.CurrentMovementVector` (0.0 0.0 0.0))
          (set `self.CurrentMovementInputSpeed` 0.0))
        (else
          ;[1 1 1] Set Movement Data when not blocked
          (set `self.CurrentMovementVector` (`KismetMathLibrary.Normal` (`self.TempMovementInputVector`)))
          (set `self.CurrentMovementInputSpeed` (`KismetMathLibrary.VSize` (`self.TempMovementInputVector`))))))
    (:`then_1`
      ;[1 1 1] Movement Update
      (`self.K2_AddActorWorldOffset` (* (`KismetMathLibrary.Normal` (`self.CurrentMovementVector`)) _returnvalue_3))
      (if (> _returnvalue_3 0.0)
        (`self.UpdateCameraBodyOffset`)
        (`self.CheckValidPawnLocation`)))
    (:`then_2`
      ;[1 1 1] Height Update
      (`self.UpdateFloorPosition`)
      (`self.K2_SetActorLocation` (`KismetMathLibrary.MakeVector` _returnvalue_x _returnvalue_y (`KismetMathLibrary.Lerp` _returnvalue_z (`self.TargetZ`) (`KismetMathLibrary.FClamp` (* `Delta Seconds` 20.0))))))))

(event `CheckValidPawnLocation`
  (bind _returnvalue (`SceneComponent.K2_GetComponentLocation` (`self.CapsuleComponent`)))
  (bind _returnvalue_2 (+ (`SceneComponent.K2_GetComponentLocation` (`self.CapsuleComponent`)) (* (`KismetMathLibrary.Normal` (`self.CurrentMovementVector`)) 15.0)))
  ;[1 1 1] Check For Valid Pawn Body Location. If not valid, then reset the Location to the last valid one.
  (bind (_outhit _returnvalue_3) (`KismetSystemLibrary.CapsuleTraceSingleByProfile` :`Start` _returnvalue :`End` _returnvalue :`Radius` 15.0 :`HalfHeight` 80.0 :`ProfileName` (`self.TraceProfileName`) :`TraceColor` (struct :`G` 0.077964 :`B` 1.0 :`A` 1.0) :`TraceHitColor` (struct :`R` 0.516667 :`G` 0.476878 :`A` 1.0)))
  (if _returnvalue_3
    (`SceneComponent.K2_SetWorldLocation` (`self.CapsuleComponent`) (`self.LastValidPawnLocation`) false false :!label _label)
    (else
      (bind (_outhit_2 _returnvalue_4) (`KismetSystemLibrary.SphereTraceSingleByProfile` :`Start` _returnvalue_2 :`End` (- _returnvalue_2 (0.0 0.0 138.0)) :`Radius` 10.0 :`ProfileName` (`self.TraceProfileName`) :`DrawDebugType` "ForOneFrame" :`TraceColor` (struct :`R` 0.952251 :`B` 1.0 :`A` 1.0) :`TraceHitColor` (struct :`G` 0.728729 :`B` 1.0 :`A` 1.0)))
      (if _returnvalue_4
        (set `self.LastValidPawnLocation` (`SceneComponent.K2_GetComponentLocation` (`self.CapsuleComponent`)))
        (else
          (goto _label))))))

(event `UpdateFloorPosition`
  (bind _capsulecomponent (`self.CapsuleComponent`))
  (bind _returnvalue (`SceneComponent.K2_GetComponentLocation` _capsulecomponent))
  (bind (_relativelocation_x _relativelocation_y _relativelocation_z) (`KismetMathLibrary.BreakVector` (`SceneComponent.RelativeLocation` (`self.VRFloorRoot`))))
  ;[1 1 1] Update Floor Position / Height
  (bind (_outhit _returnvalue_2) (`KismetSystemLibrary.SphereTraceSingleByProfile` _returnvalue (+ _returnvalue (* (`SceneComponent.GetUpVector` _capsulecomponent) -500.0)) 10.0 (`self.TraceProfileName`)))
  (if _returnvalue_2
    (set `self.TargetZ` (- (.z (`.ImpactPoint` (`GameplayStatics.BreakHitResult` _outhit))) _relativelocation_z))))

(event `UpdateCameraBodyOffset`
  (bind (_returnvalue_x _returnvalue_y) (`KismetMathLibrary.BreakVector` (* (`self.TempCameraOffset`) -1.0)))
  ;[1 1 1] Update Camera to Body Offset.
  (set `self.TempCameraOffset` (`KismetMathLibrary.InverseTransformLocation` (`self.GetTransform`) (`SceneComponent.K2_GetComponentLocation` (`self.Camera`))))
  (`SceneComponent.K2_AddLocalOffset` (`self.VROriginRoot`) (`KismetMathLibrary.MakeVector` _returnvalue_x _returnvalue_y) false false)
  (`SceneComponent.K2_AddWorldOffset` (`self.CapsuleComponent`) (`KismetMathLibrary.TransformDirection` (`self.GetTransform`) (`KismetMathLibrary.MakeVector` (.x (* (`self.TempCameraOffset`) 1.0)) (.y (* (`self.TempCameraOffset`) 1.0)))) false false))

(fn `DoMovementTrace`
  (params (StartLocation :type "Vector Structure") (Direction :type "Vector Structure") (Length :type "Float (double-precision)") (Radius :type "Float (double-precision)") (HalfHeight :type "Float (double-precision)"))
  (returns (OutHit :type "HitResult Structure") (ReturnValue :type Boolean))
  (bind (_outhit _returnvalue) (`KismetSystemLibrary.CapsuleTraceSingleByProfile` StartLocation (+ StartLocation (* (`KismetMathLibrary.Normal` Direction) Length)) Radius HalfHeight (`self.TraceProfileName`)))
  (return _outhit _returnvalue))

(fn `DrawHit`
  (params (Hit :type "HitResult Structure"))
  (bind (_bblockinghit _binitialoverlap _time _distance _location _impactpoint _normal) (`GameplayStatics.BreakHitResult` (`local.Hit`)))
  (bind _returnvalue (`KismetMathLibrary.Normal` (`self.TempMovementInputVector`)))
  (bind (_bblockinghit_2 _binitialoverlap_2 _time_2 _distance_2 _location_2 _impactpoint_2 _normal_2) (`GameplayStatics.BreakHitResult` (`local.Hit`)))
  (bind (_outvector _reflectionvector) (`self.GetWallDirection` _returnvalue _normal))
  (bind _returnvalue_2 (`KismetMathLibrary.Dot_VectorVector` _returnvalue _outvector))
  (`|ExecutionSequence`
    (:`then_0`
      (`KismetSystemLibrary.DrawDebugSphere` (`.Location` (`GameplayStatics.BreakHitResult` (`local.Hit`))) 5.0 12 (struct :`R` 1.0 :`G` 1.0 :`B` 1.0 :`A` 1.0) 0.0 0.2))
    (:`then_1`
      (`KismetSystemLibrary.DrawDebugArrow` _location_2 (+ _location_2 (* _normal_2 50.0)) 10.0 (struct :`R` 0.232572 :`B` 0.396875 :`A` 1.0) 0.0 0.5))
    (:`then_2`
      (`|ExecutionSequence`
        (:`then_0`
          (`KismetSystemLibrary.DrawDebugArrow` (- _location (* _returnvalue 50.0)) _location 10.0 (struct :`G` 0.163178 :`B` 0.725 :`A` 1.0) 0.0 0.5))
        (:`then_1`
          (`KismetSystemLibrary.DrawDebugArrow` _location (+ _location (* _reflectionvector 50.0)) 10.0 (struct :`R` 0.725 :`G` 0.421925 :`B` 0.038397 :`A` 1.0) 0.0 0.5)
          (`KismetSystemLibrary.DrawDebugArrow` _location (+ _location (* (* _outvector 50.0) _returnvalue_2)) 10.0 (struct :`R` 0.725 :`B` 0.151795 :`A` 1.0) 0.0 0.5)
          (`KismetSystemLibrary.PrintString` (`KismetStringLibrary.Conv_DoubleToString` _returnvalue_2) true true (struct :`R` 1.0 :`B` 0.030449 :`A` 1.0) 0.0))))))

(fn `GetWallDirection`
  (params (InVector :type "Vector Structure") (Normal :type "Vector Structure"))
  (returns (OutVector :type "Vector Structure") (ReflectionVector :type "Vector Structure"))
  (bind _returnvalue (`KismetMathLibrary.GetReflectionVector` InVector Normal))
  (return (`KismetMathLibrary.Normal` (+ InVector _returnvalue)) _returnvalue))

(fn `RotateVRPawn`
  (params (TurnDegrees :type "Float (double-precision)"))
  (`|ExecutionSequence`
    (:`then_0`
      (`self.UpdateCameraBodyOffset`)
      (`self.CheckValidPawnLocation`))
    (:`then_1`
      (`parent.RotateVRPawn` TurnDegrees))))

(fn `UserConstructionScript`
  (`parent.UserConstructionScript`))