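; Gravity field area shaped as a quarter cylinder around the actor's local Y axis, supplying a curved gravity direction with priority and strength.
; GetGravityAreaDirection derives pitch from the local XZ angle, snaps it to axis-aligned values outside the arc, then rotates it to world space.
; IsInRange accepts points in the positive XZ quadrant within a 100-unit local radius, without checking Y.
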(event `self.ReceiveBeginPlay`
  (`parent.ReceiveBeginPlay`))

(fn `GetGravityAreaDirection`
  (params (AtLocation :type "Vector Structure"))
  (returns (ToRotation :type "Rotator Structure") (Priority :type Integer) (Strength :type "Float (double-precision)"))
  (bind (_returnvalue_location _returnvalue_rotation _returnvalue_scale) (`KismetMathLibrary.BreakTransform` (`self.GetTransform`)))
  (bind (_returnvalue_location_2 _returnvalue_rotation_2 _returnvalue_scale_2) (`KismetMathLibrary.BreakTransform` (`self.GetTransform`)))
  (bind _pitch (.pitch (`KismetMathLibrary.NegateRotator` (`KismetMathLibrary.FindLookAtRotation` (0.0 0.0 0.0) (`KismetMathLibrary.MakeVector` (.x (`KismetMathLibrary.Normal` (`KismetMathLibrary.InverseTransformLocation` (`KismetMathLibrary.MakeTransform` _returnvalue_location_2 _returnvalue_rotation_2 _returnvalue_scale_2) (`local.AtLocation`)))) 0.0 (.z (`KismetMathLibrary.Normal` (`KismetMathLibrary.InverseTransformLocation` (`KismetMathLibrary.MakeTransform` _returnvalue_location_2 _returnvalue_rotation_2 _returnvalue_scale_2) (`local.AtLocation`)))))))))
  (return (`KismetMathLibrary.TransformRotation` (`KismetMathLibrary.MakeTransform` _returnvalue_location _returnvalue_rotation _returnvalue_scale) (`KismetMathLibrary.MakeRotator` 0.0 (`KismetMathLibrary.SelectFloat` (`KismetMathLibrary.SelectFloat` -90.0 0.0 (>= _pitch 45.0)) _pitch (>= _pitch 0.0)) 180.0)) (`self.Priority`) (`self.GravityStrength`)))

(fn `IsInRange`
  (params (AtLocation :type "Vector Structure"))
  (returns (InRange :type Boolean))
  (bind (_returnvalue_x _returnvalue_y _returnvalue_z) (`KismetMathLibrary.BreakVector` (`KismetMathLibrary.InverseTransformLocation` (`self.GetTransform`) AtLocation)))
  (return (and (and (> _returnvalue_x 0.0) (> _returnvalue_z 0.0)) (and (< (`KismetMathLibrary.VSize` (`KismetMathLibrary.MakeVector` _returnvalue_x 0.0 _returnvalue_z)) 100.0) (`KismetMathLibrary.InRange_FloatFloat` _returnvalue_z 0.0 100.0 false false)))))

(fn `UserConstructionScript`
  (`parent.UserConstructionScript`))