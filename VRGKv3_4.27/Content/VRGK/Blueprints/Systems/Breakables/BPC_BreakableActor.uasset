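; Actor component that makes its owner breakable by physical impacts in the VRGK kit.
; Each hit's impulse is compared to a threshold from a data asset, chosen by physical surface type with a default fallback, and stronger hits remove health on a power curve.
; When health runs out, it spawns a parts actor inheriting the owner's velocity, fires OnBroken, plays a sound and optionally destroys the owner.
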(event `self.ReceiveBeginPlay`
  (add `Actor.OnActorHit` (`self.GetOwner`) (delegate `OnActorHit`))
  (`self.SetCurHealth` (`self.Max Health`)))

(event `OnActorHit`
  (params (SelfActor :type "Actor Object Reference") (OtherActor :type "Actor Object Reference") (NormalImpulse :type "Vector Structure") (Hit :type "HitResult Structure (by ref)"))
  (bind _breakable_da (`self.GetBreakableDataAsset`))
  (bind _returnvalue (`KismetMathLibrary.VSize` (`self.CurNormalImpulse`)))
  (bind _returnvalue_2 (* (`self.TargetHitThreshold`) (`self.ThresholdScale`)))
  (bind (_value _returnvalue_3) (`BlueprintMapLibrary.Map_Find` (`/Game/VRGK/Blueprints/Data/BP_BreakablesDataAsset.Surface Hit Thresholds` _breakable_da) (`PhysicalMaterial.SurfaceType` (`.PhysMat` (`GameplayStatics.BreakHitResult` (`self.CurHit`))))))
  (set `self.CurNormalImpulse` NormalImpulse)
  (set `self.CurHit` Hit)
  (`|ExecutionSequence`
    (:`then_0`
      (`/Engine/EditorBlueprintResources/StandardMacros.IsValid` (`.PhysMat` (`GameplayStatics.BreakHitResult` (`self.CurHit`)))
        (:`Is Valid`
          (set `self.TargetHitThreshold` (`KismetMathLibrary.SelectFloat` _value (`/Game/VRGK/Blueprints/Data/BP_BreakablesDataAsset.Default Hit Threshold` _breakable_da) _returnvalue_3)))
        (:`Is Not Valid`
          (set `self.TargetHitThreshold` (`/Game/VRGK/Blueprints/Data/BP_BreakablesDataAsset.Default Hit Threshold` (`self.GetBreakableDataAsset`))))))
    (:`then_1`
      (if (> _returnvalue _returnvalue_2)
        (`self.SetCurHealth` (- (`self.CurHealth`) (`KismetMathLibrary.MultiplyMultiply_FloatFloat` (/ _returnvalue _returnvalue_2) 1.4)))
        (if (< (`self.CurHealth`) 1.0)
          (`self.DoBreakActor`))))))

(event `SetCurHealth`
  (params (CurHealth :type "Float (double-precision)"))
  (bind _output_get (set `self.CurHealth` CurHealth))
  (`self.OnHealthUpdate` self _output_get))

(event `DoBreakActor`
  (bind _returnvalue (`self.GetOwner`))
  (bind (_returnvalue_location _returnvalue_rotation) (`KismetMathLibrary.BreakTransform` (`Actor.GetTransform` (`self.GetOwner`))))
  (bind (_returnvalue_location_2 _returnvalue_rotation_2) (`KismetMathLibrary.BreakTransform` (`Actor.GetTransform` (`self.GetOwner`))))
  (`/Engine/EditorBlueprintResources/StandardMacros.DoOnce` false
    (:`Completed`
      (`|ExecutionSequence`
        (:`then_0`
          (if (`KismetSystemLibrary.IsValidClass` (`self.SpawnPartsActor`))
            (bind _returnvalue_2 (`|SpawnActorFromClass` (`self.SpawnPartsActor`) (`KismetMathLibrary.MakeTransform` _returnvalue_location _returnvalue_rotation) "Undefined" "OverrideRootScale" null null))
            (bind _asprimitive_component (cast `PrimitiveComponent` (`Actor.RootComponent` _returnvalue))
              (:`then`
                (message `/Game/VRGK/Blueprints/Systems/Breakables/BPI_BreakableActor.AddSpawnImpulse` _returnvalue_2 (`SceneComponent.GetComponentVelocity` _asprimitive_component) (`PrimitiveComponent.GetPhysicsAngularVelocityInDegrees` _asprimitive_component "None")))
              (:`CastFailed`
                (message `/Game/VRGK/Blueprints/Systems/Breakables/BPI_BreakableActor.AddSpawnImpulse` _returnvalue_2 (`Actor.GetVelocity` _returnvalue) (0.0 0.0 0.0))))))
        (:`then_1`
          (`self.OnBroken` self)
          (`|ExecutionSequence`
            (:`then_0`
              (bind _destructionsound (`self.DestructionSound`)
                (:`then`
                  (`GameplayStatics.SpawnSoundAtLocation` _destructionsound _returnvalue_location_2 _returnvalue_rotation_2 1.0 1.0 0.0 null null))
                (:`else`)))
            (:`then_1`
              (if (`self.AutoDestroyOwner`)
                (`Actor.K2_DestroyActor` (`self.GetOwner`))))))))))

(fn `GetBreakableDataAsset`
  (returns (`Breakable DA` :type "/Game/VRGK/Blueprints/Data/BP_BreakablesDataAsset Object Reference"))
  (bind _breakable_data (`self.Breakable Data`))
  (return (select `bool` (`KismetSystemLibrary.IsValid` _breakable_data) :`false` (`self.DefaultDataAsset`) :`true` _breakable_data)))