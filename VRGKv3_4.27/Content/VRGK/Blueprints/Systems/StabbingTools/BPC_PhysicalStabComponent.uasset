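; VR stabbing component that pins a physics object into the hit component or bone through a supplied physics constraint.
; SetupStabbingLogic aligns constraint frames to the impact and stab line with soft drives.
; After short delays, SetupStabber locks all but the stab axis, using velocity drive as friction, and arms breaking.
; Pulling past the blade limit or destroying either owner breaks the constraint and fires OnStabberBroken for external cleanup.
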(event `self.ReceiveBeginPlay`
  (`parent.ReceiveBeginPlay`))

(event `SetupStabber`
  (params (ParentPhysicsConstraint :type "PhysicsConstraintComponent Object Reference") (ChildPrimitiveComponent :type "PrimitiveComponent Object Reference") (StabPositionComp :type "/Game/VRGK/Blueprints/Systems/StabbingTools/BPC_StabPosition Object Reference"))
  (bind _parentphysicsconstraint (`self.ParentPhysicsConstraint`))
  (bind _parentphysicsconstraint_2 (`self.ParentPhysicsConstraint`))
  (bind _parentphysicsconstraint_3 (`self.ParentPhysicsConstraint`))
  (bind _parentphysicsconstraint_4 (`self.ParentPhysicsConstraint`))
  ;[1 1 1] Setup Stabbing Logic
  (set `self.StabPositionComp` StabPositionComp)
  (`self.SetupPhysicalInput` ParentPhysicsConstraint ChildPrimitiveComponent)
  (`|ExecutionSequence`
    (:`then_0`
      (`self.K2_AttachToComponent` (`self.ParentPhysicsConstraint`) self "None" "SnapToTarget" "SnapToTarget" "KeepWorld" false)
      (`self.K2_AttachToComponent` (`self.StabPositionComp`) "None" "SnapToTarget" "SnapToTarget" "KeepWorld" false)
      (`self.K2_SetRelativeLocation` (0.0 0.0 100.0)))
    (:`then_1`
      (`KismetSystemLibrary.Delay` 0.2) ; Required to make the initial Stab feel smoother
      (`|ExecutionSequence`
        (:`then_0`
          (`PhysicsConstraintComponent.SetLinearXLimit` _parentphysicsconstraint_4 "LCM_Locked" 0.0)
          (`PhysicsConstraintComponent.SetLinearYLimit` _parentphysicsconstraint_4 "LCM_Locked" 0.0)
          (`PhysicsConstraintComponent.SetLinearZLimit` (`self.ParentPhysicsConstraint`) "LCM_Limited" (+ (`self.Limit`) 1.0))
          (`PhysicsConstraintComponent.SetLinearDriveParams` _parentphysicsconstraint 0.0 (`/Game/VRGK/Blueprints/Systems/StabbingTools/BPC_StabPosition.Friction` (`self.StabPositionComp`)) 0.0)
          (`PhysicsConstraintComponent.SetLinearVelocityDrive` _parentphysicsconstraint false false true)
          (`PhysicsConstraintComponent.SetLinearPositionDrive` _parentphysicsconstraint false false false))
        (:`then_1`
          (`PhysicsConstraintComponent.SetAngularTwistLimit` _parentphysicsconstraint_2 "ACM_Locked" 0.0)
          (`PhysicsConstraintComponent.SetAngularSwing1Limit` _parentphysicsconstraint_2 "ACM_Locked" 0.0)
          (`PhysicsConstraintComponent.SetAngularSwing2Limit` _parentphysicsconstraint_2 "ACM_Locked" 0.0)
          (`PhysicsConstraintComponent.SetAngularVelocityDriveSLERP` _parentphysicsconstraint_3 false)
          (`PhysicsConstraintComponent.SetOrientationDriveSLERP` _parentphysicsconstraint_3 false))))
    (:`then_2`
      (`KismetSystemLibrary.Delay` 0.3) ; Allows the breaking of the stabber after a Delay
      (set `self.ActiveStabber` true))))

(event `self.ReceiveTick`
  (params (DeltaSeconds :type "Float (single-precision)"))
  (`parent.ReceiveTick` DeltaSeconds))

(event `SetupDestroyEvents`
  ;[1 1 1] End Play Events
  (add `Actor.OnDestroyed` (`self.GetOwner` (`self.AttachComponent`)) (delegate `OnCompDestroyed`))
  (add `Actor.OnDestroyed` (`self.GetOwner` (`self.ChildPrimitiveComponent`)) (delegate `OnCompDestroyed`)))

(event `OnCompDestroyed`
  (params (DestroyedActor :type "Actor Object Reference"))
  ;[1 1 1] End Play Events
  (`self.DoBreakStabber`))

(event `DoBreakStabber`
  ;[1 1 1] Break this Stab Component
  (bind _parentphysicsconstraint (`self.ParentPhysicsConstraint`)
    (:`then`
      (`PhysicsConstraintComponent.SetDisableCollision` _parentphysicsconstraint false)
      (`PhysicsConstraintComponent.BreakConstraint` (`self.ParentPhysicsConstraint`))
      (`PrimitiveComponent.AddImpulse` (`self.ChildPrimitiveComponent`) (* (`self.GetUpVector` (`self.StabPositionComp`)) -500.0) "None" true)
      (`/Game/VRGK/Blueprints/BPFL_PhysicsObjects.TryResetPhysicsSimulation` (`self.ChildPrimitiveComponent`))
      (`/Game/VRGK/Blueprints/BPFL_PhysicsObjects.TryResetPhysicsSimulation` (`self.AttachComponent`) (`self.AttachBoneName`))
      ;;[0.5135 0.1368 0.101] Destroy Stabber and Constraint Components directly in the Parent Actor.
      ;; Can't destroy other actor components (Physics Constraints) inside this stabber component.
      (`self.OnStabberBroken` self))
    (:`else`)))

(event `self.Physical Input Tick`
  (params (`Delta Seconds` :type "Float (single-precision)"))
  (bind _relativestabtransform_location (`KismetMathLibrary.BreakTransform` (`self.RelativeStabTransform`)))
  (bind _stabpositioncomp (`self.StabPositionComp`))
  (bind (_returnvalue_location _returnvalue_rotation) (`KismetMathLibrary.BreakTransform` (`self.GetSocketTransform` (`self.AttachComponent`) (`self.AttachBoneName`) "RTS_World")))
  (bind (_returnvalue_x _returnvalue_y _returnvalue_z) (`KismetMathLibrary.BreakVector` (`KismetMathLibrary.InverseTransformLocation` (`KismetMathLibrary.MakeTransform` (`/Game/VRGK/Blueprints/Systems/StabbingTools/BPC_StabPosition.Get World Center` _stabpositioncomp) (`self.K2_GetComponentRotation` _stabpositioncomp)) (`KismetMathLibrary.TransformLocation` (`KismetMathLibrary.MakeTransform` _returnvalue_location _returnvalue_rotation) _relativestabtransform_location))))
  ;[1 1 1] Event Tick Calculation, Checks for the Distance the Stabber is pulled out
  (`parent.Physical Input Tick` `Delta Seconds`)
  (if (`self.ActiveStabber`)
    (if (> _returnvalue_z (`self.Limit`))
      (`self.DoBreakStabber`))))

(fn `SetupStabbingLogic`
  (params (`Hit Result` :type "HitResult Structure"))
  (returns (Success :type Boolean))
  (locals (TempLinearVelocity :type "Vector Structure" :default (0.0 0.0 0.0)))
  (bind _parentphysicsconstraint (`self.ParentPhysicsConstraint`))
  (bind _limit (`self.Limit`))
  (bind _parentphysicsconstraint_2 (`self.ParentPhysicsConstraint`))
  (bind _stabpositioncomp (`self.StabPositionComp`))
  (bind (_relativestabtransform_location _relativestabtransform_rotation) (`KismetMathLibrary.BreakTransform` (`self.RelativeStabTransform`)))
  (bind _parentphysicsconstraint_3 (`self.ParentPhysicsConstraint`))
  (bind _parentphysicsconstraint_4 (`self.ParentPhysicsConstraint`))
  (bind (_returnvalue_x _returnvalue_y _returnvalue_z) (`KismetMathLibrary.BreakVector` (`self.K2_GetComponentScale` (`self.StabPositionComp`))))
  (bind (_bblockinghit _binitialoverlap _time _distance _location _impactpoint _normal _impactnormal _physmat _hitactor _hitcomponent _hitbonename) (`GameplayStatics.BreakHitResult` (`local.Hit Result`)))
  (bind (_returnvalue_location _returnvalue_rotation) (`KismetMathLibrary.BreakTransform` (`self.GetSocketTransform` (`self.AttachComponent`) (`self.AttachBoneName`) "RTS_World")))
  (bind (_returnvalue_location_2 _returnvalue_rotation_2) (`KismetMathLibrary.BreakTransform` (`self.K2_GetComponentToWorld` (`self.ChildPrimitiveComponent`))))
  (bind _returnvalue (`KismetMathLibrary.MakeTransform` _returnvalue_location _returnvalue_rotation))
  (bind _returnvalue_2 (`KismetMathLibrary.MakeTransform` _returnvalue_location_2 _returnvalue_rotation_2))
  (set `self.Limit` (/ (* _returnvalue_z 100.0) 2.0))
  (set `self.AttachComponent` _hitcomponent)
  (set `self.AttachBoneName` _hitbonename)
  (`|ExecutionSequence`
    (:`then_0`
      (`|ExecutionSequence`
        (:`then_0`
          (`PhysicsConstraintComponent.SetAngularTwistLimit` _parentphysicsconstraint "ACM_Limited" 30.0)
          (`PhysicsConstraintComponent.SetAngularSwing1Limit` _parentphysicsconstraint "ACM_Limited" 30.0)
          (`PhysicsConstraintComponent.SetAngularSwing2Limit` _parentphysicsconstraint "ACM_Limited" 30.0)
          (`PhysicsConstraintComponent.SetAngularDriveParams` _parentphysicsconstraint_3 500000.0 500.0 0.0)
          (`PhysicsConstraintComponent.SetAngularDriveMode` _parentphysicsconstraint_3 "SLERP")
          (`PhysicsConstraintComponent.SetAngularVelocityDriveSLERP` _parentphysicsconstraint_3 true)
          (`PhysicsConstraintComponent.SetOrientationDriveSLERP` _parentphysicsconstraint_3 true))
        (:`then_1`
          (`PhysicsConstraintComponent.SetLinearXLimit` _parentphysicsconstraint_2 "LCM_Free" _limit)
          (`PhysicsConstraintComponent.SetLinearYLimit` _parentphysicsconstraint_2 "LCM_Free" _limit)
          (`PhysicsConstraintComponent.SetLinearDriveParams` (`self.ParentPhysicsConstraint`) 500000.0 500.0 0.0))
        (:`then_2`
          (`PhysicsConstraintComponent.SetLinearZLimit` (`self.ParentPhysicsConstraint`) "LCM_Limited" (* (`self.Limit`) 0.9))
          (`PhysicsConstraintComponent.SetDisableCollision` (`self.ParentPhysicsConstraint`) true)
          (`PhysicsConstraintComponent.SetLinearVelocityDrive` _parentphysicsconstraint_4 true true true)
          (`PhysicsConstraintComponent.SetLinearPositionDrive` _parentphysicsconstraint_4 true true false))))
    (:`then_1`
      ;[1 1 1] Setup Physics Constraint Components and Frames
      (`PhysicsConstraintComponent.SetConstrainedComponents` (`self.ParentPhysicsConstraint`) (`self.ChildPrimitiveComponent`) "None" (`self.AttachComponent`) (`self.AttachBoneName`))
      (set `self.RelativeStabTransform` (`KismetMathLibrary.MakeTransform` (`KismetMathLibrary.InverseTransformLocation` _returnvalue (`.ImpactPoint` (`GameplayStatics.BreakHitResult` (`local.Hit Result`)))) (`KismetMathLibrary.InverseTransformRotation` _returnvalue (`self.K2_GetComponentRotation` (`self.StabPositionComp`)))))
      (`PhysicsConstraintComponent.SetConstraintReferenceFrame` (`self.ParentPhysicsConstraint`) "Frame2" (`KismetMathLibrary.MakeTransform` _relativestabtransform_location _relativestabtransform_rotation))
      (`PhysicsConstraintComponent.SetConstraintReferenceFrame` (`self.ParentPhysicsConstraint`) "Frame1" (`KismetMathLibrary.MakeTransform` (`KismetMathLibrary.InverseTransformLocation` _returnvalue_2 (.location (`KismetMathLibrary.MakeTransform` (`KismetMathLibrary.TransformLocation` (`KismetMathLibrary.MakeTransform` (`/Game/VRGK/Blueprints/Systems/StabbingTools/BPC_StabPosition.GetClosestPointOnStartLine` _stabpositioncomp (`.ImpactPoint` (`GameplayStatics.BreakHitResult` (`local.Hit Result`)))) (`self.K2_GetComponentRotation` _stabpositioncomp) (`self.K2_GetComponentScale` _stabpositioncomp)) (0.0 0.0 50.0)) (`self.K2_GetComponentRotation` (`self.StabPositionComp`))))) (`KismetMathLibrary.InverseTransformRotation` _returnvalue_2 (.rotation (`KismetMathLibrary.MakeTransform` (`KismetMathLibrary.TransformLocation` (`KismetMathLibrary.MakeTransform` (`/Game/VRGK/Blueprints/Systems/StabbingTools/BPC_StabPosition.GetClosestPointOnStartLine` _stabpositioncomp (`.ImpactPoint` (`GameplayStatics.BreakHitResult` (`local.Hit Result`)))) (`self.K2_GetComponentRotation` _stabpositioncomp) (`self.K2_GetComponentScale` _stabpositioncomp)) (0.0 0.0 50.0)) (`self.K2_GetComponentRotation` (`self.StabPositionComp`)))))))
      (`/Game/VRGK/Blueprints/BPFL_PhysicsObjects.TryResetPhysicsSimulation` (`self.ChildPrimitiveComponent`)))
    (:`then_2`
      ;[1 1 1] Setup the Physics Tool itself
      (`self.SetupDestroyEvents`)
      (return true))))