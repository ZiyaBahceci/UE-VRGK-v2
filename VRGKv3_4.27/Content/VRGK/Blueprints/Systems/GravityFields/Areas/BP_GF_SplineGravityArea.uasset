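; Gravity field area shaped as a tube along a spline, pulling toward the nearest point on that spline.
; The construction script sizes the collision box, applies the spline's point type and loop setting, and builds spline meshes scaled to the gravity radius.
; Range checks compare distance to the closest spline point against the radius.
; Gravity queries return a look-at rotation to that point with priority and strength, optionally drawing a debug circle.
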(fn `GetGravityAreaDirection`
  (params (AtLocation :type "Vector Structure"))
  (returns (ToRotation :type "Rotator Structure") (Priority :type Integer) (Strength :type "Float (double-precision)"))
  (bind _spline (`self.Spline`))
  (bind _returnvalue (`SplineComponent.FindLocationClosestToWorldLocation` _spline AtLocation "World"))
  (if (`self.DrawDebug`)
    (`KismetSystemLibrary.DrawDebugCircle` _returnvalue (`self.GravityRadius`) 12 (struct :`R` 1.0 :`G` 1.0 :`B` 1.0 :`A` 1.0) 0.0 10.0 (`SplineComponent.FindRightVectorClosestToWorldLocation` _spline AtLocation "Local") (`SplineComponent.FindUpVectorClosestToWorldLocation` _spline AtLocation "World") true))
  (return (`KismetMathLibrary.FindLookAtRotation` AtLocation _returnvalue) (`self.Priority`) (`self.GravityStrength`)))

(fn `IsInRange`
  (params (AtLocation :type "Vector Structure"))
  (returns (InRange :type Boolean))
  (return (< (`KismetMathLibrary.VSize` (- AtLocation (`SplineComponent.FindLocationClosestToWorldLocation` (`self.Spline`) AtLocation "World"))) (`self.GravityRadius`))))

(fn `UserConstructionScript`
  (bind _spline (`self.Spline`))
  (bind _returnvalue (/ (`self.GravityRadius`) 50.0))
  (bind _returnvalue_2 (`KismetMathLibrary.MakeVector2D` _returnvalue _returnvalue))
  (`parent.UserConstructionScript`)
  (`BoxComponent.SetBoxExtent` (`self.BoxCollision`) (`self.BoxExtent`) true)
  (`|ExecutionSequence`
    (:`then_0`
      (`|ExecutionSequence`
        (:`then_0`
          (for _index (range (`SplineComponent.GetNumberOfSplinePoints` (`self.Spline`)))
            (`SplineComponent.SetSplinePointType` (`self.Spline`) _index (`self.SplineType`) true)))
        (:`then_1`
          (`SplineComponent.SetClosedLoop` (`self.Spline`) (`self.ClosedLoop`) true))))
    (:`then_1`
      (for _index_2 (range (+ (- (`SplineComponent.GetNumberOfSplinePoints` (`self.Spline`)) 2) 1))
        (bind _returnvalue_3 (`AddComponent|NODE_AddSplineMeshComponent-2`))
        (bind (_location _tangent) (`SplineComponent.GetLocationAndTangentAtSplinePoint` _spline _index_2 "Local"))
        (bind (_location_2 _tangent_2) (`SplineComponent.GetLocationAndTangentAtSplinePoint` _spline (+ _index_2 1) "Local"))
        (`SplineMeshComponent.SetStartAndEnd` _returnvalue_3 _location _tangent _location_2 _tangent_2 true)
        (`SplineMeshComponent.SetStartScale` _returnvalue_3 _returnvalue_2 true)
        (`SplineMeshComponent.SetEndScale` _returnvalue_3 _returnvalue_2 true)))))