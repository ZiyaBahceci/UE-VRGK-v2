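; Player laser pointer actor that drives a WidgetInteraction component to hover and click widgets, destroying itself with its owner.
; Hover changes fade the laser through a timeline and custom primitive data, while Tick smooths its distance-based scale and moves the target to the hit.
; When hidden, actor tick stops and interaction polling slows.
; Functions forward press/release, switch trace channel, and disable pointing via an empty custom hit.
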(event `self.ReceiveBeginPlay`
  ;[0.1309 1 0.265] Setup
  (set `WidgetInteractionComponent.VirtualUserIndex` (`self.Virtual User Index`) (`self.WidgetInteraction`))
  (set `WidgetInteractionComponent.PointerIndex` (`self.Pointer Index`) (`self.WidgetInteraction`))
  (add `self.OnEndPlay` (`self.GetOwner`) (delegate `OnOwnerEndPlay`))
  (`self.SetInteractionMode` (`self.CurrentLaserMode`))
  (`self.ForceHideLaser`))

(event `OnOwnerEndPlay` :!signature `self.OnEndPlay`
  (params (Actor :type "Actor Object Reference") (EndPlayReason :type "EEndPlayReason Enum" :default "Destroyed"))
  ;[0.1309 1 0.265] Setup
  (`self.K2_DestroyActor`))

(event `self.ReceiveTick`
  (params (DeltaSeconds :type "Float (single-precision)"))
  (bind _laserroot (`self.LaserRoot`))
  (bind (_returnvalue_bblockinghit _returnvalue_binitialoverlap _returnvalue_time _returnvalue_distance _returnvalue_location) (`GameplayStatics.BreakHitResult` (`WidgetInteractionComponent.GetLastHitResult` (`self.WidgetInteraction`))))
  (bind (_returnvalue_bblockinghit_2 _returnvalue_binitialoverlap_2 _returnvalue_time_2 _returnvalue_distance_2) (`GameplayStatics.BreakHitResult` (`WidgetInteractionComponent.GetLastHitResult` (`self.WidgetInteraction`))))
  (bind (_relativescale3d_x _relativescale3d_y _relativescale3d_z) (`KismetMathLibrary.BreakVector` (`SceneComponent.RelativeScale3D` _laserroot)))
  (set `self.CurDeltaSeconds` DeltaSeconds)
  ;[0.4942 0.3602 1] Update Laser Size
  (`SceneComponent.SetRelativeScale3D` _laserroot (`KismetMathLibrary.MakeVector` 1.0 1.0 (`KismetMathLibrary.FInterpTo` _relativescale3d_z (`KismetMathLibrary.MapRangeClamped` (`KismetMathLibrary.SelectFloat` (/ _returnvalue_distance_2 100.0) 0.0 _returnvalue_bblockinghit_2) 0.0 10.0 0.01 8.0) (`self.CurDeltaSeconds`) 10.0)))
  ;[1 0.2662 0.292] Update Target Pointer Location
  (if _returnvalue_bblockinghit
    (`SceneComponent.K2_SetWorldLocation` (`self.TargetRoot`) _returnvalue_location false false)))

(event `self.WidgetInteraction.OnHoveredWidgetChanged`
  (params (WidgetComponent :type "WidgetComponent Object Reference") (PreviousWidgetComponent :type "WidgetComponent Object Reference"))
  ;[0.4878 1 0.6964] Check for Widget Change
  (`/Engine/EditorBlueprintResources/StandardMacros.IsValid` WidgetComponent
    (:`Is Valid`
      (`self.ShowLaser`)
      (`self.OnInteractionChange` true))
    (:`Is Not Valid`
      (`self.HideLaser`)
      (`self.OnInteractionChange` false))))

(event `ShowLaser`
  ;[1 0.8634 0.3468] Fade In and Out the Laser Pointer.
  (`|ExecutionSequence`
    (:`then_0`
      (if (not (`self.IsActorTickEnabled`))
        (`self.SetActorTickEnabled` true)
        (`self.SetActorHiddenInGame` false)
        (`ActorComponent.SetComponentTickIntervalAndCooldown` (`self.WidgetInteraction`) 0.0)))
    (:`then_1`
      (bind (_direction _alpha) (`Timeline|LaserFade` :!label _label)
        (:`Update`
          (`PrimitiveComponent.SetCustomPrimitiveDataFloat` (`self.LaserCylinder`) 0 _alpha :!label _label_2)
          (`PrimitiveComponent.SetCustomPrimitiveDataFloat` (`self.Sphere`) 0 _alpha))
        (:`Finished`
          (`|ExecutionSequence`
            (:`then_0`
              (goto _label_2))
            (:`then_1`
              (switch `ETimelineDirection` _direction
                (:`Backward`
                  (if (`self.IsActorTickEnabled`)
                    (`self.SetActorTickEnabled` false :!label _label_3)
                    (`self.SetActorHiddenInGame` true)
                    (`ActorComponent.SetComponentTickIntervalAndCooldown` (`self.WidgetInteraction`) 0.1)))))))))))

(event `HideLaser`
  ;[1 0.8634 0.3468] Fade In and Out the Laser Pointer.
  (if (`self.IsActorTickEnabled`)
    (goto _label :!via `Reverse`)))

(event `ForceHideLaser`
  ;[1 0.8634 0.3468] Fade In and Out the Laser Pointer.
  (goto _label_3))

(fn `HasValidWidgetToInteract`
  (returns (True :type Boolean))
  (return (`KismetSystemLibrary.IsValid` (`WidgetInteractionComponent.GetHoveredWidgetComponent` (`self.WidgetInteraction`)))))

(fn `IsLaserPointerEnabled`
  (returns (True :type Boolean))
  (return (`|EnumEquality` (`WidgetInteractionComponent.InteractionSource` (`self.WidgetInteraction`)) "World")))

(fn `SetInteractionMode`
  (params (`New Mode` :type "/Game/VRGK/Blueprints/Player/InteractionLaser/Enum_InteractionLaserMode Enum" :default "NewEnumerator0"))
  (set `self.CurrentLaserMode` `New Mode`)
  (set `WidgetInteractionComponent.TraceChannel` (select `/Game/VRGK/Blueprints/Player/InteractionLaser/Enum_InteractionLaserMode` (`self.CurrentLaserMode`) :`NewEnumerator0` "ECC_GameTraceChannel9" :`NewEnumerator1` "ECC_Visibility" :!type "ECollisionChannel Enum") (`self.WidgetInteraction`)))

(fn `SetLaserPointerEnabled`
  (params (Enable :type Boolean))
  (bind _widgetinteraction (`self.WidgetInteraction`))
  (if (!= Enable (`self.IsLaserPointerEnabled`))
    (if Enable
      (set `WidgetInteractionComponent.InteractionSource` "World" _widgetinteraction)
      (else
        (set `WidgetInteractionComponent.InteractionSource` "Custom" _widgetinteraction)
        (`WidgetInteractionComponent.SetCustomHitResult` (`self.WidgetInteraction`) (`GameplayStatics.MakeHitResult` false))
        (`self.HideLaser`)))))

(fn `TryWidgetPress`
  (returns (Valid :type Boolean))
  (if (`self.HasValidWidgetToInteract`)
    (`WidgetInteractionComponent.PressPointerKey` (`self.WidgetInteraction`) "LeftMouseButton")
    (return true)
    (else
      (return true))))

(fn `TryWidgetRelease`
  (returns (Valid :type Boolean))
  (`WidgetInteractionComponent.ReleasePointerKey` (`self.WidgetInteraction`) "LeftMouseButton")
  (if (`self.HasValidWidgetToInteract`)
    (return true)
    (else
      (return true))))

(fn `UserConstructionScript`)