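; BPC_StabHandler is an actor component that lets its owner physically stab tagged actors or components on impact.
; Strong root-primitive hits are tested against oriented boxes at each BPC_StabPosition, plus an impact-normal alignment check.
; A valid hit spawns a physics constraint and BPC_PhysicalStabComponent, tracked to tag the owner while stabbing.
; Broken stabbers are untracked and broadcast via OnChildStabberBroken for external destruction, with a warning if still valid.
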(event `self.ReceiveBeginPlay`
  (bind _asprimitive_component (cast `PrimitiveComponent` (`Actor.RootComponent` (`self.GetOwner`))))
  (set `self.PrimitiveRoot` _asprimitive_component)
  (add `PrimitiveComponent.OnComponentHit` (`self.PrimitiveRoot`) (delegate `OnPrimitiveRootHit`)))

(event `OnPrimitiveRootHit`
  (params (HitComponent :type "PrimitiveComponent Object Reference") (OtherActor :type "Actor Object Reference") (OtherComp :type "PrimitiveComponent Object Reference") (NormalImpulse :type "Vector Structure") (Hit :type "HitResult Structure (by ref)"))
  (bind _tag_name (`/Game/VRGK/Blueprints/Core/BPFL_GlobalVariables.GetTagStab`))
  (bind (_tempboxsize_x _tempboxsize_y _tempboxsize_z) (`KismetMathLibrary.BreakVector` (`self.TempBoxSize`)))
  (bind _tempstabposition (`self.TempStabPosition`))
  (bind _tempclosestpoint (`self.TempClosestPoint`))
  (bind (_returnvalue_location _returnvalue_rotation) (`KismetMathLibrary.BreakTransform` (`SceneComponent.K2_GetComponentToWorld` (`self.TempStabPosition`))))
  (bind (_bblockinghit _binitialoverlap _time _distance _location _impactpoint) (`GameplayStatics.BreakHitResult` (`self.TempHit`)))
  (bind _returnvalue (`KismetMathLibrary.MakeTransform` (`KismetMathLibrary.TransformLocation` (`KismetMathLibrary.MakeTransform` _returnvalue_location _returnvalue_rotation) (`KismetMathLibrary.MakeVector` 0.0 0.0 _tempboxsize_z)) (`SceneComponent.K2_GetComponentRotation` (`self.TempStabPosition`))))
  (if (or (`Actor.ActorHasTag` OtherActor _tag_name) (`self.ComponentHasTag` OtherComp _tag_name))
    (set `self.TempImpulse` NormalImpulse)
    (set `self.TempHit` Hit)
    (if (> (`KismetMathLibrary.VSize` (`self.TempImpulse`)) (`self.ImpulseThreshold`))
      (for _array_element (`Actor.K2_GetComponentsByClass` (`self.GetOwner`) "/Game/VRGK/Blueprints/Systems/StabbingTools/BPC_StabPosition.BPC_StabPosition_C") :!label _label
        (set `self.TempStabPosition` _array_element)
        (set `self.TempBoxSize` (/ (+ (* (`SceneComponent.K2_GetComponentScale` (`self.TempStabPosition`)) 100.0) (`/Game/VRGK/Blueprints/Systems/StabbingTools/BPC_StabPosition.AdditionalOverlapDistance` (`self.TempStabPosition`))) 2.0))
        (`|ExecutionSequence`
          (:`then_0`
            (if (`self.DrawDebug`)
              (`KismetSystemLibrary.DrawDebugBox` (.location _returnvalue) (`self.TempBoxSize`) (struct) (.rotation _returnvalue) 0.0 0.1)))
          (:`then_1`
            (if (`KismetMathLibrary.IsPointInBoxWithTransform` (`.ImpactPoint` (`GameplayStatics.BreakHitResult` (`self.TempHit`))) _returnvalue (`self.TempBoxSize`))
              (set `self.TempClosestPoint` (`KismetMathLibrary.FindClosestPointOnSegment` _impactpoint (`/Game/VRGK/Blueprints/Systems/StabbingTools/BPC_StabPosition.GetClosestPointOnStartLine` _tempstabposition _impactpoint) (`/Game/VRGK/Blueprints/Systems/StabbingTools/BPC_StabPosition.GetClosestEndPoint` _tempstabposition _impactpoint)))
              (`|ExecutionSequence`
                (:`then_0`
                  (if (`self.DrawDebug`)
                    (`KismetSystemLibrary.DrawDebugSphere` (`self.TempClosestPoint`) 2.0 6 (struct :`R` 1.0 :`G` 0.522073 :`A` 1.0) 0.0 0.2)))
                (:`then_1`
                  (`|ExecutionSequence`
                    (:`then_0`
                      (if (`self.DrawDebug`)
                        (`KismetSystemLibrary.DrawDebugArrow` _tempclosestpoint (+ _tempclosestpoint (* (`.ImpactNormal` (`GameplayStatics.BreakHitResult` (`self.TempHit`))) 20.0)) 10.0 (struct :`G` 1.0 :`B` 0.279541 :`A` 1.0) 0.0 0.2)))
                    (:`then_1`
                      (if (> (`KismetMathLibrary.Dot_VectorVector` (`.ImpactNormal` (`GameplayStatics.BreakHitResult` (`self.TempHit`))) (* (`SceneComponent.GetUpVector` (`self.TempStabPosition`)) -1.0)) 0.7)
                        (`self.BreakStabPositionLoop`)
                        (bind _new_stabber (`self.CreateNewStabber` (`self.TempStabPosition`) (`self.TempHit`)))
                        (`KismetArrayLibrary.Array_AddUnique` (`self.StabberArray`) _new_stabber)
                        (add `/Game/VRGK/Blueprints/Systems/StabbingTools/BPC_PhysicalStabComponent.OnStabberBroken` _new_stabber (delegate `OnStabberCompBroken`))
                        (`self.UpdateStabStatus`)))))))))))))

(event `BreakStabPositionLoop`
  (goto _label :!via `Break`))

(event `OnStabberCompBroken`
  (params (`This Comp` :type "/Game/VRGK/Blueprints/Systems/StabbingTools/BPC_PhysicalStabComponent Object Reference"))
  (`KismetArrayLibrary.Array_RemoveItem` (`self.StabberArray`) `This Comp`)
  (`self.OnChildStabberBroken` `This Comp` (`/Game/VRGK/Blueprints/Systems/PhysicalInputs/BPC_PhysicalInputBase.ParentPhysicsConstraint` `This Comp`))
  (`self.UpdateStabStatus`)
  (`/Engine/EditorBlueprintResources/StandardMacros.IsValid` `This Comp`
    (:`Is Valid`
      ;[1 1 1] Do Warning if Components have not been destroyed
      (`KismetSystemLibrary.PrintString` (`KismetStringLibrary.Concat_StrStr` (`KismetSystemLibrary.GetDisplayName` (`self.GetOwner`)) " - Actors StabHandler has not been setup correctly! \nUse the EventDispatcher \"OnChildStabberBroken to Destroy the Stabber and Constraints to avoid gameplay, performance and memory issues! \n \nDue to limitations of UE, it's not possible to destroy those component from within the Stab Handler! \n") true true (struct :`R` 1.0 :`B` 0.21137 :`A` 1.0)))))

(event `UpdateStabStatus`
  (bind _tag_name (`/Game/VRGK/Blueprints/Core/BPFL_GlobalVariables.GetTagStabbingActor`))
  (bind _tags (`Actor.Tags` (`self.GetOwner`)))
  ;[1 1 1] Update Stab Status / Count
  (`|ExecutionSequence`
    (:`then_0`
      (if (`self.IsCurrentlyStabbing`)
        (`KismetArrayLibrary.Array_AddUnique` _tags _tag_name)
        (else
          (`KismetArrayLibrary.Array_RemoveItem` _tags _tag_name))))))

(fn `CreateNewStabber`
  (params (`Stab Position Component` :type "/Game/VRGK/Blueprints/Systems/StabbingTools/BPC_StabPosition Object Reference") (`Hit Result` :type "HitResult Structure"))
  (returns (`New Stabber` :type "/Game/VRGK/Blueprints/Systems/StabbingTools/BPC_PhysicalStabComponent Object Reference"))
  (locals (TempConstraint :type "PhysicsConstraintComponent Object Reference") (TempStabber :type "/Game/VRGK/Blueprints/Systems/StabbingTools/BPC_PhysicalStabComponent Object Reference"))
  (`|ExecutionSequence`
    (:`then_0`
      (bind _returnvalue (`|AddComponentByClass` (`self.GetOwner`) "/Script/Engine.PhysicsConstraintComponent" false (`KismetMathLibrary.MakeTransform` (0.0 0.0 0.0))))
      (set `local.TempConstraint` _returnvalue)
      (bind _returnvalue_2 (`|AddComponentByClass` (`self.GetOwner`) "/Game/VRGK/Blueprints/Systems/StabbingTools/BPC_PhysicalStabComponent.BPC_PhysicalStabComponent_C" false (`KismetMathLibrary.MakeTransform` (0.0 0.0 0.0))))
      (set `local.TempStabber` _returnvalue_2))
    (:`then_1`
      (`/Game/VRGK/Blueprints/Systems/StabbingTools/BPC_PhysicalStabComponent.SetupStabber` (`local.TempStabber`) (`local.TempConstraint`) (`self.PrimitiveRoot`) (`local.Stab Position Component`))
      (`/Game/VRGK/Blueprints/Systems/StabbingTools/BPC_PhysicalStabComponent.SetupStabbingLogic` (`local.TempStabber`) (`local.Hit Result`)))
    (:`then_2`
      (return (`local.TempStabber`)))))

(fn `IsCurrentlyStabbing`
  (returns (ReturnValue :type Boolean))
  (return (> (`KismetArrayLibrary.Array_Length` (`self.StabberArray`)) 0)))