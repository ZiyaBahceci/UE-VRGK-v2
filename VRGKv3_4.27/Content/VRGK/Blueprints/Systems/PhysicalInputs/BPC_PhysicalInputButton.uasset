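; VR physical push button component that reports press and release through event dispatchers and attached sounds.
; It works with a constrained physics body or a welded primitive.
; In welded mode, filtered hit impulses push the primitive along a chosen local axis within a range, then it eases back and stops updating at rest.
; Each tick compares position to separate press and release thresholds, with a time delay to debounce state changes.
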(event `self.SetupPhysicalInput`
  (params (ParentPhysicsConstraint :type "PhysicsConstraintComponent Object Reference") (ChildPrimitiveComponent :type "PrimitiveComponent Object Reference"))
  (`parent.SetupPhysicalInput` ParentPhysicsConstraint ChildPrimitiveComponent)
  (set `self.LastPressChangeTime` (`self.OwnersGameTimeSinceCreation`))
  (switch `/Game/VRGK/Blueprints/Systems/PhysicalInputs/Enum_PhysicalInputInteractionmode` (`self.Interaction Mode`)
    (:`NewEnumerator1`
      (add `PrimitiveComponent.OnComponentHit` (`self.ChildPrimitiveComponent`) (delegate `OnWeldedButtonHit`)))))

(event `OnWeldedButtonHit`
  (params (HitComponent :type "PrimitiveComponent Object Reference") (OtherActor :type "Actor Object Reference") (OtherComp :type "PrimitiveComponent Object Reference") (NormalImpulse :type "Vector Structure") (Hit :type "HitResult Structure (by ref)"))
  (bind (_weldedrange_min _weldedrange_max) (break `InputRange` (`self.WeldedRange`)))
  (bind _temptargetdif (`self.TempTargetDif`))
  (bind _returnvalue (select `/Game/VRGK/Blueprints/Systems/PhysicalInputs/Enum_PhysicalInputDirection` (`self.ButtonDirection`) :`NewEnumerator0` (.x (`KismetMathLibrary.InverseTransformDirection` (`self.K2_GetComponentToWorld`) (* (/ (* NormalImpulse (`|EaseFunction` "EaseIn" (`KismetMathLibrary.FClamp` (/ (`KismetMathLibrary.VSize` NormalImpulse) 100.0)) 0.0 1.0)) 100.0) -1.0))) :`NewEnumerator1` (.y (`KismetMathLibrary.InverseTransformDirection` (`self.K2_GetComponentToWorld`) (* (/ (* NormalImpulse (`|EaseFunction` "EaseIn" (`KismetMathLibrary.FClamp` (/ (`KismetMathLibrary.VSize` NormalImpulse) 100.0)) 0.0 1.0)) 100.0) -1.0))) :`NewEnumerator2` (.z (`KismetMathLibrary.InverseTransformDirection` (`self.K2_GetComponentToWorld`) (* (/ (* NormalImpulse (`|EaseFunction` "EaseIn" (`KismetMathLibrary.FClamp` (/ (`KismetMathLibrary.VSize` NormalImpulse) 100.0)) 0.0 1.0)) 100.0) -1.0)))))
  (if (or (`Actor.ActorHasTag` OtherActor (`self.TagForWeldedHits`)) (`self.ComponentHasTag` OtherComp "None"))
    (set `self.TempTargetDif` (`KismetMathLibrary.SelectFloat` _returnvalue _temptargetdif (< _returnvalue _temptargetdif)))
    (`|ExecutionSequence`
      (:`then_0`
        (set `self.TargetPosition` (`KismetMathLibrary.FClamp` (+ (`self.LastTargetPosition`) (`self.TempTargetDif`)) _weldedrange_min _weldedrange_max)))
      (:`then_1`
        (`self.SetInputUpdateEnabled` true)
        (set `self.IsCurrentlyHit` true)
        (`KismetSystemLibrary.RetriggerableDelay` 0.1)
        (set `self.IsCurrentlyHit` false)))))

(event `self.UpdatePhysicalInputState`
  (switch `/Game/VRGK/Blueprints/Systems/PhysicalInputs/Enum_PhysicalInputInteractionmode` (`self.Interaction Mode`)
    (:`NewEnumerator0`
      (`parent.UpdatePhysicalInputState`))))

(event `self.Physical Input Tick`
  (params (`Delta Seconds` :type "Float (single-precision)"))
  (bind (_weldedrange_min _weldedrange_max) (break `InputRange` (`self.WeldedRange`)))
  (bind (_weldedrange_min_2 _weldedrange_max_2) (break `InputRange` (`self.WeldedRange`)))
  (bind (_weldedrange_min_3 _weldedrange_max_3) (break `InputRange` (`self.WeldedRange`)))
  (bind (_weldedrange_min_4 _weldedrange_max_4) (break `InputRange` (`self.WeldedRange`)))
  (`|ExecutionSequence`
    (:`then_0`
      (switch `/Game/VRGK/Blueprints/Systems/PhysicalInputs/Enum_PhysicalInputInteractionmode` (`self.Interaction Mode`)
        (:`NewEnumerator1`
          (set `self.TargetPosition` (`KismetMathLibrary.FInterpTo` (select `/Game/VRGK/Blueprints/Systems/PhysicalInputs/Enum_PhysicalInputDirection` (`self.ButtonDirection`) :`NewEnumerator0` (.x (`SceneComponent.RelativeLocation` (`self.ChildPrimitiveComponent`))) :`NewEnumerator1` (.y (`SceneComponent.RelativeLocation` (`self.ChildPrimitiveComponent`))) :`NewEnumerator2` (.z (`SceneComponent.RelativeLocation` (`self.ChildPrimitiveComponent`)))) (`KismetMathLibrary.SelectFloat` (`KismetMathLibrary.FClamp` (`self.TargetPosition`) _weldedrange_min_4 _weldedrange_max_4) _weldedrange_max_2 (`self.IsCurrentlyHit`)) (`self.CurrentDeltaSeconds`) (`KismetMathLibrary.SelectFloat` (`self.PushingInSpeed`) (`self.RelaxSpeed`) (`self.IsCurrentlyHit`))))
          (`|ExecutionSequence`
            (:`then_0`
              (if (`self.IsCurrentlyHit`)
                _
                (elif (`KismetMathLibrary.NearlyEqual_FloatFloat` (`self.TargetPosition`) _weldedrange_max_3 0.01)
                  (set `self.TargetPosition` _weldedrange_max)
                  (`self.SetInputUpdateEnabled` false))))
            (:`then_1`
              (`self.K2_SetRelativeLocation` (`self.ChildPrimitiveComponent`) (* (`KismetMathLibrary.Conv_DoubleToVector` (`self.TargetPosition`)) (select `/Game/VRGK/Blueprints/Systems/PhysicalInputs/Enum_PhysicalInputDirection` (`self.ButtonDirection`) :`NewEnumerator0` (1.0 0.0 0.0) :`NewEnumerator1` (0.0 1.0 0.0) :`NewEnumerator2` (0.0 0.0 1.0) :!type "Vector Structure")) false true)
              (set `self.LastTargetPosition` (`self.TargetPosition`))
              (set `self.TempTargetDif` 0.0))))))
    (:`then_1`
      (bind _output_get (set `self.TempPressState` (< (select `/Game/VRGK/Blueprints/Systems/PhysicalInputs/Enum_PhysicalInputDirection` (`self.ButtonDirection`) :`NewEnumerator0` (.x (`KismetMathLibrary.InverseTransformLocation` (`self.K2_GetComponentToWorld`) (`self.K2_GetComponentLocation` (`self.ChildPrimitiveComponent`)))) :`NewEnumerator1` (.y (`KismetMathLibrary.InverseTransformLocation` (`self.K2_GetComponentToWorld`) (`self.K2_GetComponentLocation` (`self.ChildPrimitiveComponent`)))) :`NewEnumerator2` (.z (`KismetMathLibrary.InverseTransformLocation` (`self.K2_GetComponentToWorld`) (`self.K2_GetComponentLocation` (`self.ChildPrimitiveComponent`))))) (`KismetMathLibrary.SelectFloat` (`self.ReleaseDistanceValue`) (`self.PressDistanceValue`) (`self.CurPressed`)))))
      (if (!= _output_get (`self.CurPressed`))
        (if (> (- (`self.OwnersGameTimeSinceCreation`) (`self.LastPressChangeTime`)) (`self.PressChangeTimeDelay`))
          ;[1 1 1] Do Press State Change and Call Event Dispatchers.
          (set `self.LastPressChangeTime` (`self.OwnersGameTimeSinceCreation`))
          (bind _output_get_2 (set `self.CurPressed` (`self.TempPressState`)))
          (`self.OnButtonPressChanged` self _output_get_2)
          (if (`self.CurPressed`)
            (`self.OnButtonPressed` self)
            (`GameplayStatics.SpawnSoundAttached` (`self.SoundOnPress`) self "None" (0.0 0.0 0.0) (struct) "KeepRelativeOffset" false 1.0 1.0 0.0 null null)
            (else
              (`self.OnButtonReleased` self)
              (`GameplayStatics.SpawnSoundAttached` (`self.SoundOnRelease`) self "None" (0.0 0.0 0.0) (struct) "KeepRelativeOffset" false 1.0 1.0 0.0 null null))))
        (else
          (set `self.LastPressChangeTime` (`self.OwnersGameTimeSinceCreation`)))))))

(fn `IsButtonPressed`
  (returns (`Is Pressed` :type Boolean))
  (return (`self.CurPressed`)))