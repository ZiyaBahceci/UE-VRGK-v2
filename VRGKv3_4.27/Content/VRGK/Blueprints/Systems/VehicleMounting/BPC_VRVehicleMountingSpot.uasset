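; BPC_VRVehicleMountingSpot is a VR Game Kit scene component that acts as a mounting slot for a game pawn on a vehicle.
; Attaching registers the slot with the pawn and enables tick, while detaching clears both.
; Each tick passes the slot's world rotation delta to the pawn, so it turns with the vehicle.
; It also exposes its parent primitive and socket, plus target head height from a child BPC_VRVehicleHeadPosition.
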(event `self.ReceiveTick`
  (params (DeltaSeconds :type "Float (single-precision)"))
  (`self.UpdateRotation`))

(event `UpdateRotation`
  (`|ExecutionSequence`
    (:`then_0`
      (`/Game/VRGK/Blueprints/Player/PlayerCore/BP_VRGamePawn.AddRotationFromVehicleMountingSlot` (`self.AttachedGamePawn`) (`KismetMathLibrary.NormalizedDeltaRotator` (`self.K2_GetComponentRotation`) (`self.LastTickRotation`))))
    (:`then_1`
      (`self.SetLastTickRotation`))))

(event `SetLastTickRotation`
  (set `self.LastTickRotation` (`self.K2_GetComponentRotation`)))

(fn `Cast Get Head Positioner`
  (returns (`AsBPC VRVehicle Head Position` :type "/Game/VRGK/Blueprints/Systems/VehicleMounting/BPC_VRVehicleHeadPosition Object Reference"))
  (for _array_element (`self.GetChildrenComponents` false)
    (bind _asbpc_vrvehicle_head_position (cast `/Game/VRGK/Blueprints/Systems/VehicleMounting/BPC_VRVehicleHeadPosition` _array_element))
    (return _asbpc_vrvehicle_head_position)))

(fn `GetPrimitiveParent`
  (returns (`Parent Primitive` :type "PrimitiveComponent Object Reference") (`Bone Name` :type Name))
  (bind _asprimitive_component (cast `PrimitiveComponent` (`|GetArrayItem` (`self.GetParentComponents`))))
  (return _asprimitive_component (`self.GetAttachSocketName`)))

(fn `GetTargetHeadHeight`
  (returns (`Relative Location Z` :type "Float (double-precision)"))
  (bind _headpositioner (`self.HeadPositioner`)
    (:`then`
      (bind (_relativelocation_x _relativelocation_y _relativelocation_z) (`KismetMathLibrary.BreakVector` (`SceneComponent.RelativeLocation` _headpositioner)))
      (return _relativelocation_z))
    (:`else`
      (return 999.0))))

(fn `SetNewPawnAttached`
  (params (`New Game Pawn` :type "/Game/VRGK/Blueprints/Player/PlayerCore/BP_VRGamePawn Object Reference"))
  (`/Engine/EditorBlueprintResources/StandardMacros.IsValid` `New Game Pawn`
    (:`Is Valid`
      (`/Engine/EditorBlueprintResources/StandardMacros.IsValid` (`self.AttachedGamePawn`)
        (:`Is Not Valid`
          (`|ExecutionSequence`
            (:`then_0`
              (bind _asbpc_vrvehicle_head_position (`self.Cast Get Head Positioner`))
              (set `self.HeadPositioner` _asbpc_vrvehicle_head_position))
            (:`then_1`
              (bind _output_get (set `self.AttachedGamePawn` (`local.New Game Pawn`)))
              (`/Game/VRGK/Blueprints/Player/PlayerCore/BP_VRGamePawn.SetNewVehicleMountingSlot` _output_get self)
              (`self.SetComponentTickEnabled` true)
              (`self.SetLastTickRotation`))))))))

(fn `TryDetachPawn`
  (bind _attachedgamepawn (`self.AttachedGamePawn`)
    (:`then`
      (`/Game/VRGK/Blueprints/Player/PlayerCore/BP_VRGamePawn.DetachFromVehicleMountingSlot` _attachedgamepawn)
      (set `self.AttachedGamePawn` null)
      (`self.SetComponentTickEnabled` false))
    (:`else`)))