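; Player inventory bag actor that mounts itself on the body of its owning BP_VRGamePawn.
; On BeginPlay it attaches to the pawn, then re-parents its UpperBody and Pelvis components to the spine and pelvis sockets of the pawn's mesh with a corrective rotation, so each follows that body part.
; It binds to the pawn's EndPlay event and destroys itself when the pawn leaves play.
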(event `self.ReceiveBeginPlay`
  (bind _upperbody (`self.UpperBody`))
  (bind _pelvis (`self.Pelvis`))
  (bind _asbp_vrgame_pawn (cast `/Game/VRGK/Blueprints/Player/PlayerCore/BP_VRGamePawn` (`self.GetOwner`)))
  (bind _output_get (set `self.VRPawn` _asbp_vrgame_pawn))
  (add `self.OnEndPlay` _output_get (delegate `OnPlayerEndPlay`))
  (`self.K2_AttachToActor` (`self.VRPawn`) "None" "SnapToTarget" "SnapToTarget" "KeepWorld" false)
  (`SceneComponent.K2_AttachToComponent` _upperbody (`Character.Mesh` (`self.VRPawn`)) "spine_03" "SnapToTarget" "SnapToTarget" "KeepWorld" false)
  (`SceneComponent.K2_SetRelativeRotation` _upperbody (struct :`Yaw` 90.0 :`Roll` -90.0) false false)
  (`SceneComponent.K2_AttachToComponent` _pelvis (`Character.Mesh` (`self.VRPawn`)) "pelvis" "SnapToTarget" "SnapToTarget" "KeepWorld" false)
  (`SceneComponent.K2_SetRelativeRotation` _pelvis (struct :`Yaw` 90.0 :`Roll` -90.0) false false))

(event `OnPlayerEndPlay` :!signature `self.OnEndPlay`
  (params (Actor :type "Actor Object Reference") (EndPlayReason :type "EEndPlayReason Enum" :default "Destroyed"))
  (`self.K2_DestroyActor`))

(fn `UserConstructionScript`)