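; Inventory slot component for the VR kit that stores and hands back inventory objects through air release and air grab hand events.
; Releasing a held actor tries to attach it to the slot, while an empty-handed grab releases the stored object straight into that hand.
; It specializes a parent attachment component, accepting only BPC_InventoryObject and adding an exact item-size tag match against allowed sizes to the parent's tag check.
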(event `self.ReceiveBeginPlay`)

(event `/Game/VRGK/Blueprints/Player/Hand/BPI_HandOverlapInteraction.OnVRHandAirRelease`
  (params (`Grabbed Hand` :type "/Game/VRGK/Blueprints/Player/Hand/BP_VRHand Object Reference") (`Last Grabbed Actor` :type "Actor Object Reference"))
  (bind _sucess (`self.TryAttachActor` `Last Grabbed Actor`))
  (`KismetSystemLibrary.PrintString` (`KismetStringLibrary.Concat_StrStr` "Try Air Release - " (`KismetStringLibrary.Conv_BoolToString` _sucess))))

(event `/Game/VRGK/Blueprints/Player/Hand/BPI_HandOverlapInteraction.OnVRHandAirGrab`
  (params (`Grabbed Hand` :type "/Game/VRGK/Blueprints/Player/Hand/BP_VRHand Object Reference"))
  (if (not (`/Game/VRGK/Blueprints/Player/Hand/BP_VRHand.IsGrabbingAnyObject` `Grabbed Hand`))
    (bind (_success _released_object) (`self.TryReleaseCurrentObject`))
    (`/Engine/EditorBlueprintResources/StandardMacros.IsValid` _released_object
      (:`Is Valid`
        (`/Game/VRGK/Blueprints/Player/Hand/BP_VRHand.Try Grabbing Actor Directly` `Grabbed Hand` (`self.GetOwner` _released_object))
        (`KismetSystemLibrary.PrintString` "Grab Air")))))

(fn `CheckIfAttachedTagsAreValid`
  (params (`Attachable Object Ref` :type "/Game/VRGK/Blueprints/Systems/AttachmentSlots/BPC_AttachableObject Object Reference"))
  (returns (Valid :type Boolean))
  (return (and (`parent.CheckIfAttachedTagsAreValid` `Attachable Object Ref`) (`BlueprintGameplayTagLibrary.MatchesAnyTags` (`/Game/VRGK/Blueprints/Systems/Inventory/BPC_InventoryObject.Item Size` (cast `/Game/VRGK/Blueprints/Systems/Inventory/BPC_InventoryObject` `Attachable Object Ref` :!pure true)) (`self.Allowed Item Sizes`) true))))

(fn `GetValidAttachmentObjectClass`
  (returns (`Attachable Object Class` :type "/Game/VRGK/Blueprints/Systems/AttachmentSlots/BPC_AttachableObject Class Reference"))
  (return "/Game/VRGK/Blueprints/Systems/Inventory/BPC_InventoryObject.BPC_InventoryObject_C"))