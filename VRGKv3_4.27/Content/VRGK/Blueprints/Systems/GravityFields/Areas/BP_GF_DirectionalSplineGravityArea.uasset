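; Directional gravity area that follows a spline, pulling along the inverse of the nearest spline up vector with a set strength and priority.
; The construction script sizes the box collision, applies point type and loop settings, and builds roll-matched spline meshes scaled to gravity radius and height.
; Range checks test a thin oriented box above the closest spline point, which the direction query can also draw for debugging.
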(fn `GetGravityAreaDirection`
  (params (AtLocation :type "Vector Structure"))
  (returns (ToRotation :type "Rotator Structure") (Priority :type Integer) (Strength :type "Float (double-precision)"))
  (bind _returnvalue (/ (`self.GravityHeight`) 2.0))
  (bind _rotation (.rotation (`SplineComponent.FindTransformClosestToWorldLocation` (`self.Spline`) AtLocation "World" false)))
  (if (`self.DrawDebug`)
    (`KismetSystemLibrary.DrawDebugBox` (+ (.location (`SplineComponent.FindTransformClosestToWorldLocation` (`self.Spline`) AtLocation "World" false)) (* (`KismetMathLibrary.GetUpVector` _rotation) _returnvalue)) (`KismetMathLibrary.MakeVector` 20.0 (`self.GravityRadius`) _returnvalue) (struct :`R` 1.0 :`G` 1.0 :`B` 1.0 :`A` 1.0) _rotation 0.0 10.0))
  (return (`KismetMathLibrary.FindLookAtRotation` (0.0 0.0 0.0) (`KismetMathLibrary.NegateVector` (`SplineComponent.FindUpVectorClosestToWorldLocation` (`self.Spline`) AtLocation "World"))) (`self.Priority`) (`self.GravityStrength`)))

(fn `IsInRange`
  (params (AtLocation :type "Vector Structure"))
  (returns (InRange :type Boolean))
  (bind _returnvalue (/ (`self.GravityHeight`) 2.0))
  (bind _rotation (.rotation (`SplineComponent.FindTransformClosestToWorldLocation` (`self.Spline`) AtLocation "World" false)))
  (return (`KismetMathLibrary.IsPointInBoxWithTransform` AtLocation (`KismetMathLibrary.MakeTransform` (+ (.location (`SplineComponent.FindTransformClosestToWorldLocation` (`self.Spline`) AtLocation "World" false)) (* (`KismetMathLibrary.GetUpVector` _rotation) _returnvalue)) _rotation) (`KismetMathLibrary.MakeVector` 20.0 (`self.GravityRadius`) _returnvalue))))

(fn `UserConstructionScript`
  (bind _spline (`self.Spline`))
  (bind _spline_2 (`self.Spline`))
  (bind _spline_3 (`self.Spline`))
  (bind _returnvalue (`KismetMathLibrary.MakeVector2D` (/ (`self.GravityRadius`) 50.0) (/ (`self.GravityHeight`) 100.0)))
  (`parent.UserConstructionScript`)
  (`BoxComponent.SetBoxExtent` (`self.BoxCollision`) (`self.BoxExtent`) true)
  (`|ExecutionSequence`
    (:`then_0`
      (`|ExecutionSequence`
        (:`then_0`
          (for _index (range (`SplineComponent.GetNumberOfSplinePoints` (`self.Spline`)))
            (`SplineComponent.SetSplinePointType` (`self.Spline`) _index (`self.SplineType`) false)
            (`SplineComponent.SetUpVectorAtSplinePoint` _spline_3 _index (`SplineComponent.GetUpVectorAtSplinePoint` _spline_3 _index "World") "World" false))
          (`SplineComponent.UpdateSpline` (`self.Spline`)))
        (:`then_1`
          (`SplineComponent.SetClosedLoop` (`self.Spline`) (`self.ClosedLoop`) true))))
    (:`then_1`
      (for _index_2 (range (+ (- (`SplineComponent.GetNumberOfSplinePoints` (`self.Spline`)) 2) 1))
        (bind _returnvalue_2 (`AddComponent|NODE_AddSplineMeshComponent-2`))
        (bind (_location _tangent) (`SplineComponent.GetLocationAndTangentAtSplinePoint` _spline _index_2 "Local"))
        (bind _returnvalue_3 (+ _index_2 1))
        (bind (_location_2 _tangent_2) (`SplineComponent.GetLocationAndTangentAtSplinePoint` _spline _returnvalue_3 "Local"))
        (`SplineMeshComponent.SetStartAndEnd` _returnvalue_2 _location _tangent _location_2 _tangent_2 true)
        (`SplineMeshComponent.SetStartScale` _returnvalue_2 _returnvalue true)
        (`SplineMeshComponent.SetEndScale` _returnvalue_2 _returnvalue true)
        (`SplineMeshComponent.SetStartRoll` _returnvalue_2 (`KismetMathLibrary.DegreesToRadians` (`SplineComponent.GetRollAtSplinePoint` _spline_2 _index_2 "Local")) true)
        (`SplineMeshComponent.SetEndRoll` _returnvalue_2 (`KismetMathLibrary.DegreesToRadians` (`SplineComponent.GetRollAtSplinePoint` _spline_2 _returnvalue_3 "Local")) true)))))