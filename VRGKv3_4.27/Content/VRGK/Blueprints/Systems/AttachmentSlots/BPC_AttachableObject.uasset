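; Actor component that lets its VR-grabbable owner attach to and release from attachment slots.
; It attaches by the slot's method: component attachment, welding to a parent primitive, or a physics constraint, adjusting physics and collision to match.
; Grab updater events trigger release on grab or hard pull, while timing checks and override interfaces gate attachment.
; Hands briefly let go during transitions, with physics fixes and regrabs deferred a tick.
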(event `self.ReceiveEndPlay`
  (params (EndPlayReason :type "EEndPlayReason Enum" :default "Destroyed"))
  ;[0.3135 0.1115 0.1296] End Play
  (`self.TryReleaseFromSlot`))

(event `self.ReceiveBeginPlay`
  ;[1 0.5288 0.3698 1 32] SETUP
  ; Bind "OnAnyGrab" from Owner Actor.
  (bind _output_get (set `self.HandGrabCollisionUpdater` (`Actor.GetComponentByClass` (`self.GetOwner`) "/Game/VRGK/Blueprints/Components/GrabCollisionUpdater/BPC_HandGrabUpdater.BPC_HandGrabUpdater_C")))
  (`/Engine/EditorBlueprintResources/StandardMacros.IsValid` _output_get
    (:`Is Valid`
      (add `/Game/VRGK/Blueprints/Components/GrabCollisionUpdater/BPC_HandGrabUpdater.OnAnyGrab` (`self.HandGrabCollisionUpdater`) (delegate `OnOwnerAnyGrab`))
      (add `/Game/VRGK/Blueprints/Components/GrabCollisionUpdater/BPC_HandGrabUpdater.OnGrabbingStrengthUpdate` (`self.HandGrabCollisionUpdater`) (delegate `OnGrabbingStrengthUpdate`)))))

(event `OnOwnerAnyGrab`
  (params (`Updater Component` :type "/Game/VRGK/Blueprints/Components/GrabCollisionUpdater/BPC_HandGrabUpdater Object Reference"))
  ;[1 0.4024 0.6866] Event if Owner is Grabbed. Allows for Objects to be released by Grabbing it.
  (if (`self.DetachOnGrab`)
    (bind _attachedslot (`self.AttachedSlot`)
      (:`then`
        (`/Game/VRGK/Blueprints/Systems/AttachmentSlots/BPC_AttachmentSlot.TryReleaseCurrentObject` _attachedslot))
      (:`else`))))

(event `OnGrabbingStrengthUpdate`
  (params (Strength :type "Float (double-precision)"))
  ;[1 0.575 0.9573] Check for hold Hands Grabbing Strength Update. Allows for Releasing this Object by Pulling it out.
  (if (`self.DetachOnPull`)
    (bind _attachedslot (`self.AttachedSlot`)
      (:`then`
        (if (and (> Strength (`self.PullDetachThreshold`)) (> (- (`Actor.GetGameTimeSinceCreation` (`self.GetOwner`)) (`self.AttachGameTime`)) (`self.PullDetachMinimumTime`)))
          (`/Game/VRGK/Blueprints/Systems/AttachmentSlots/BPC_AttachmentSlot.TryReleaseCurrentObject` _attachedslot)))
      (:`else`))))

(event `TryDetachAllHands`
  ;[0.2264 0.4015 1] Detach / Reattach Hands from Attachment State Changes
  (bind _handgrabcollisionupdater (`self.HandGrabCollisionUpdater`)
    (:`then`
      (set `self.TempReleasedHands` (`/Game/VRGK/Blueprints/Components/GrabCollisionUpdater/BPC_HandGrabUpdater.GetAttachedHands` _handgrabcollisionupdater))
      (`/Game/VRGK/Blueprints/Components/GrabCollisionUpdater/BPC_HandGrabUpdater.TryReleaseAllGrabbedHands` (`self.HandGrabCollisionUpdater`)))
    (:`else`)))

(event `TryReattachAllHands`
  ;[0.2264 0.4015 1] Detach / Reattach Hands from Attachment State Changes
  (for _array_element (`self.TempReleasedHands`)
    (`/Game/VRGK/Blueprints/Player/Hand/BP_VRHand.Try Grabbing Actor Directly` _array_element (`self.GetOwner`)))
  (`KismetArrayLibrary.Array_Clear` (`self.TempReleasedHands`)))

(event `DoDelayedAttachEvents`
  (bind (_returnvalue_location _returnvalue_rotation) (`KismetMathLibrary.BreakTransform` (`SceneComponent.K2_GetComponentToWorld` (`self.AttachedSlot`))))
  ;[0.02322 1 0.5195] Delayed and Final Attachment Events
  ; This is needed, because some functionality needs to wait a tick to be working correctly. (Physics/Collision)
  (`KismetSystemLibrary.Delay` 0.0) ; Some physics/collision functionality does not work correctly in the same tick, \nso we offset those events to the following tick.
  (`|ExecutionSequence`
    (:`then_0`
      (switch `/Game/VRGK/Blueprints/Systems/AttachmentSlots/Enum_SlotAttachmentType` (`/Game/VRGK/Blueprints/Systems/AttachmentSlots/BPC_AttachmentSlot.Attachment Method` (`self.AttachedSlot`))
        (:`NewEnumerator1`
          (`Actor.K2_SetActorLocationAndRotation` (`self.GetOwner`) _returnvalue_location _returnvalue_rotation false true)
          (bind _asprimitive_component (`self.Get Owner Root Primitive Component`))
          (bind (_hasphysicsroot _physics_root) (`/Game/VRGK/Blueprints/BPFL_PhysicsObjects.GetPhysicsRoot` _asprimitive_component))
          (if _hasphysicsroot
            (`/Game/VRGK/Blueprints/BPFL_PhysicsObjects.TryResetPhysicsSimulation` _physics_root)))))
    (:`then_1`
      (if (not (`self.ReleaseHandsAfterAttaching`))
        (`self.TryReattachAllHands`)))
    (:`then_2`
      (set `self.AllowDetach` true))))

(event `DoDelayedReleaseEvents`
  ;[1 0.4278 0] Delayed and Final Release Events
  ; This is needed, because some functionality needs to wait a tick to be working correctly. (Physics/Collision)
  (`KismetSystemLibrary.Delay` 0.0)
  (`|ExecutionSequence`
    (:`then_0`
      (`self.TryReattachAllHands`))
    (:`then_1`
      (set `self.DetachGameTime` (`Actor.GetGameTimeSinceCreation` (`self.GetOwner`))))))

(fn `CanAttach`
  (params (NeedsGrab :type Boolean))
  (returns (True :type Boolean))
  (if (`self.IsAttachedToSlot`)
    (return false)
    (elif (> (- (`Actor.GetGameTimeSinceCreation` (`self.GetOwner`)) (`self.DetachGameTime`)) (`self.ReattachMinimumTime`))
      (`|ExecutionSequence`
        (:`then_0`
          (for _array_element (`Actor.K2_GetComponentsByClass` (`self.GetOwner`) "/Script/Engine.ActorComponent")
            (if (`KismetSystemLibrary.DoesImplementInterface` _array_element "/Game/VRGK/Blueprints/Systems/AttachmentSlots/BPI_AttachmentOverride.BPI_AttachmentOverride_C")
              (bind _disable_attachments (message `/Game/VRGK/Blueprints/Systems/AttachmentSlots/BPI_AttachmentOverride.GetShouldDisableAnyAttachments` _array_element))
              (if _disable_attachments
                (return false)))))
        (:`then_1`
          (if (or (`local.NeedsGrab`) (`self.OnlyAttachWhileGrabbed`))
            (return (`/Game/VRGK/Blueprints/Components/GrabCollisionUpdater/BPC_HandGrabUpdater.HasHandGrabbing` (`self.HandGrabCollisionUpdater`)))
            (else
              (return true)))))
      (else
        (return false)))))

(fn `CanRelease`
  (returns (True :type Boolean))
  (return (`self.AllowDetach`)))

(fn `DoAttachmentToSlot`
  (bind _returnvalue (`self.GetOwner`))
  (`self.TryDetachAllHands`)
  (`|ExecutionSequence`
    (:`then_0`
      (switch `/Game/VRGK/Blueprints/Systems/AttachmentSlots/Enum_SlotAttachmentType` (`/Game/VRGK/Blueprints/Systems/AttachmentSlots/BPC_AttachmentSlot.Attachment Method` (`self.AttachedSlot`))
        (:`NewEnumerator0`
          (`|ExecutionSequence`
            (:`then_0`
              ;[1 1 1] Try to Update Simulate Physics State
              (if (`self.Should Update Simulate Physics of Root Component`)
                (bind _asprimitive_component (cast `PrimitiveComponent` (`Actor.RootComponent` (`self.GetOwner`))))
                (`PrimitiveComponent.SetSimulatePhysics` _asprimitive_component false)))
            (:`then_1`
              (if (`self.Should Update Collision Enabled of Actor`)
                (`Actor.SetActorEnableCollision` (`self.GetOwner`) false)))))))
    (:`then_1`
      (switch `/Game/VRGK/Blueprints/Systems/AttachmentSlots/Enum_SlotAttachmentType` (`/Game/VRGK/Blueprints/Systems/AttachmentSlots/BPC_AttachmentSlot.Attachment Method` (`self.AttachedSlot`))
        (:`NewEnumerator0`
          ;[0.5178 1 0.7132] Default / Attach To Slot Component
          (`Actor.K2_AttachToComponent` _returnvalue (`self.AttachedSlot`) "None" "SnapToTarget" "SnapToTarget" "KeepWorld" false)
          (`Actor.K2_SetActorRelativeRotation` _returnvalue (`self.Rotation in Slot`) false false)
          (`Actor.K2_SetActorRelativeLocation` _returnvalue (`self.Location in Slot`) false false))
        (:`NewEnumerator1`
          ;[0.9221 1 0.3705] Weld to Primitive Parent
          (bind (_asprimitive_component_2 _socket_name) (`/Game/VRGK/Blueprints/Systems/AttachmentSlots/BPC_AttachmentSlot.GetParentPrimitiveComponentOfSlot` (`self.AttachedSlot`)))
          (`SceneComponent.K2_AttachToComponent` (`Actor.RootComponent` (`self.GetOwner`)) _asprimitive_component_2 _socket_name "KeepWorld" "KeepWorld" "KeepWorld" true))
        (:`NewEnumerator2`
          ;[1 0.3259 0.7991] Physics Constraint Attachment
          (bind _physics_constraint_comp (`/Game/VRGK/Blueprints/Systems/AttachmentSlots/BPC_AttachmentSlot.GetParentPhysicsConstraint` (`self.AttachedSlot`)))
          (bind _asprimitive_component_3 (cast `PrimitiveComponent` (`SceneComponent.GetAttachParent` _physics_constraint_comp))
            (:`then`
              (bind _asprimitive_component_4 (`self.Get Owner Root Primitive Component`))
              (`|ExecutionSequence`
                (:`then_0`
                  (`PhysicsConstraintComponent.SetConstrainedComponents` _physics_constraint_comp _asprimitive_component_4 "None" _asprimitive_component_3 "None")
                  (`PhysicsConstraintComponent.SetConstraintReferenceFrame` _physics_constraint_comp "Frame1" (`KismetMathLibrary.MakeTransform` (0.0 0.0 0.0))) ; Child / Frame 1
                  (bind (_returnvalue_location _returnvalue_rotation) (`KismetMathLibrary.BreakTransform` (`SceneComponent.GetRelativeTransform` _physics_constraint_comp)))
                  (`PhysicsConstraintComponent.SetConstraintReferenceFrame` _physics_constraint_comp "Frame2" (`KismetMathLibrary.MakeTransform` _returnvalue_location _returnvalue_rotation)) ; Parent / Frame 2
                )
                (:`then_1`
                  ;;[1 1 1] Reset Physics, to correctly update the "Disable Collision" of the Constraint.
                  (`/Game/VRGK/Blueprints/BPFL_PhysicsObjects.TryResetPhysicsSimulation` _asprimitive_component_4))))
            (:`CastFailed`
              (`KismetSystemLibrary.PrintString` (`KismetStringLibrary.Concat_StrStr` (`KismetSystemLibrary.GetDisplayName` (`self.AttachedSlot`)) " - Physics Constraint has no Primitive Parent.") true true (struct :`R` 1.0 :`B` 0.032956 :`A` 1.0)))))))
    (:`then_2`
      ;[0.0647 0.4427 0.2048] Finalize Attachment
      (`KismetArrayLibrary.Array_AddUnique` (`Actor.Tags` (`self.GetOwner`)) (`/Game/VRGK/Blueprints/Core/BPFL_GlobalVariables.GetTagAttachedActor`))
      (`self.OnDidAttach`)
      (set `self.AttachGameTime` (`Actor.GetGameTimeSinceCreation` (`self.GetOwner`)))
      (`self.DoDelayedAttachEvents`))))

(fn `DoReleaseAttachment`
  (`self.TryDetachAllHands`)
  (`|ExecutionSequence`
    (:`then_0`
      (switch `/Game/VRGK/Blueprints/Systems/AttachmentSlots/Enum_SlotAttachmentType` (`/Game/VRGK/Blueprints/Systems/AttachmentSlots/BPC_AttachmentSlot.Attachment Method` (`self.AttachedSlot`))
        (:`NewEnumerator0`
          ;[1 1 1] Default Attached to Socket
          (`Actor.K2_DetachFromActor` (`self.GetOwner`) "KeepWorld" "KeepWorld" "KeepWorld" :!label _label)
          (bind _asprimitive_component (`self.Get Owner Root Primitive Component`))
          (`PrimitiveComponent.SetSimulatePhysics` _asprimitive_component true))
        (:`NewEnumerator1`
          (goto _label))
        (:`NewEnumerator2`
          ;[1 1 1] Physics Constraint Attachment
          (bind _physics_constraint_comp (`/Game/VRGK/Blueprints/Systems/AttachmentSlots/BPC_AttachmentSlot.GetParentPhysicsConstraint` (`self.AttachedSlot`)))
          (`PhysicsConstraintComponent.BreakConstraint` _physics_constraint_comp))))
    (:`then_1`
      (switch `/Game/VRGK/Blueprints/Systems/AttachmentSlots/Enum_SlotAttachmentType` (`/Game/VRGK/Blueprints/Systems/AttachmentSlots/BPC_AttachmentSlot.Attachment Method` (`self.AttachedSlot`))
        (:`NewEnumerator0`
          (`|ExecutionSequence`
            (:`then_0`
              (if (`self.Should Update Collision Enabled of Actor`)
                (`Actor.SetActorEnableCollision` (`self.GetOwner`) true)))
            (:`then_1`
              ;[1 0.5971 0.9232] Try to Update Simulate Physics State
              (if (`self.Should Update Simulate Physics of Root Component`)
                (bind _asprimitive_component_2 (cast `PrimitiveComponent` (`Actor.RootComponent` (`self.GetOwner`))))
                (`PrimitiveComponent.SetSimulatePhysics` _asprimitive_component_2 true)))))
        (:`NewEnumerator1`
          (bind (_asprimitive_component_3 _socket_name) (`/Game/VRGK/Blueprints/Systems/AttachmentSlots/BPC_AttachmentSlot.GetParentPrimitiveComponentOfSlot` (`self.AttachedSlot`)))
          (`/Game/VRGK/Blueprints/BPFL_PhysicsObjects.TryResetPhysicsSimulation` _asprimitive_component_3 _socket_name)
          (bind (_hasphysicsroot _physics_root _physics_root_bone_name) (`/Game/VRGK/Blueprints/BPFL_PhysicsObjects.GetPhysicsRoot` _asprimitive_component_3 _socket_name))
          (if _hasphysicsroot
            (`/Game/VRGK/Blueprints/BPFL_PhysicsObjects.TryResetPhysicsSimulation` _physics_root _physics_root_bone_name)))))
    (:`then_2`
      ;[0.1692 0.4094 0.1365] Finalize Detachment
      (`KismetArrayLibrary.Array_RemoveItem` (`Actor.Tags` (`self.GetOwner`)) (`/Game/VRGK/Blueprints/Core/BPFL_GlobalVariables.GetTagAttachedActor`))
      (set `self.AttachedSlot` null)
      (`self.OnDidRelease`)
      (`self.DoDelayedReleaseEvents`))))

(fn `Get Owner Root Primitive Component`
  (returns (`AsPrimitive Component` :type "PrimitiveComponent Object Reference"))
  (bind _asprimitive_component (cast `PrimitiveComponent` (`Actor.RootComponent` (`self.GetOwner`)))
    (:`then`
      (return _asprimitive_component))
    (:`CastFailed`
      (`KismetSystemLibrary.PrintString` (`KismetStringLibrary.Concat_StrStr` (`KismetSystemLibrary.GetDisplayName` self) " - Could not find Root Primitive Component.") true true (struct :`R` 1.0 :`B` 0.032956 :`A` 1.0)))))

(fn `GetAttachedSlotActor`
  (returns (ReturnValue :type "Actor Object Reference"))
  (return (`self.GetOwner` (`self.AttachedSlot`))))

(fn `GetShouldDisableAnyAttachments`
  (returns (`Disable Attachments` :type Boolean))
  (return (`self.IsAttachedToSlot`)))

(fn `IsAttachedToSlot`
  (returns (True :type Boolean))
  (return (`KismetSystemLibrary.IsValid` (`self.AttachedSlot`))))

(fn `PrepareNewAttachment`
  (params (`New Slot` :type "/Game/VRGK/Blueprints/Systems/AttachmentSlots/BPC_AttachmentSlot Object Reference"))
  (set `self.AttachedSlot` `New Slot`)
  (set `self.AllowDetach` false)
  (`self.OnPrepareAttach`))

(fn `PrepareRelease`
  (`self.OnPrepareRelease`)
  ;[0.9607 1 0.3609] Add custom Local Actor Offset after Release, to not have the Object be stuck in the Slot.
  (if (!= (`self.ActorOffsetOnRelease`) (0.0 0.0 0.0) :`ErrorTolerance` 0.1)
    (`Actor.K2_AddActorLocalOffset` (`self.GetOwner`) (`self.ActorOffsetOnRelease`) false true)))

(fn `TryReleaseFromSlot`
  (returns (Success :type Boolean))
  (bind _attachedslot (`self.AttachedSlot`)
    (:`then`
      (bind _success (`/Game/VRGK/Blueprints/Systems/AttachmentSlots/BPC_AttachmentSlot.TryReleaseCurrentObject` _attachedslot))
      (return _success))
    (:`else`
      (return false))))