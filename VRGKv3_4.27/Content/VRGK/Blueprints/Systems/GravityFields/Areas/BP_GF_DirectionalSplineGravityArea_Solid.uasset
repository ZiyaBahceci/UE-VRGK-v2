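; Solid variant of a directional spline gravity area, with a visible mesh built along its spline; no gravity logic is defined here.
; The construction script adds a spline mesh per segment, matching point positions, tangents and roll, and applies a shared scale and material.
; With DrawDebug on, BeginPlay enables Tick, which sweeps along the spline drawing coordinate axes to show its orientation.
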(event `self.ReceiveBeginPlay`
  (`parent.ReceiveBeginPlay`)
  (if (`self.DrawDebug`)
    (`self.SetActorTickEnabled` true)))

(event `self.ReceiveTick`
  (params (DeltaSeconds :type "Float (single-precision)"))
  (bind _spline (`self.Spline`))
  (bind (_returnvalue_location _returnvalue_rotation) (`KismetMathLibrary.BreakTransform` (`SplineComponent.GetTransformAtDistanceAlongSpline` _spline (`self.CurDist`) "World" true)))
  ;[1 1 1] Event Tick will only be enableed when "Draw Debug" is True!
  (`parent.ReceiveTick` DeltaSeconds)
  (if (`self.DrawDebug`)
    (set `self.CurDist` (mod (+ (`self.CurDist`) (* DeltaSeconds 10000.0)) (`SplineComponent.GetSplineLength` _spline)))
    (`KismetSystemLibrary.DrawDebugCoordinateSystem` _returnvalue_location _returnvalue_rotation 600.0 20.0 10.0)))

(fn `UserConstructionScript`
  (bind _spline (`self.Spline`))
  (bind _meshscale (`self.MeshScale`))
  (`parent.UserConstructionScript`)
  (for _index (range (+ (- (`SplineComponent.GetNumberOfSplinePoints` (`self.Spline`)) 2) 1))
    (bind _returnvalue (`AddComponent|NODE_AddSplineMeshComponent-1`))
    (bind (_location _tangent) (`SplineComponent.GetLocationAndTangentAtSplinePoint` _spline _index "Local"))
    (bind _returnvalue_2 (+ _index 1))
    (bind (_location_2 _tangent_2) (`SplineComponent.GetLocationAndTangentAtSplinePoint` _spline _returnvalue_2 "Local"))
    (`SplineMeshComponent.SetStartAndEnd` _returnvalue _location _tangent _location_2 _tangent_2 true)
    (`SplineMeshComponent.SetStartRoll` _returnvalue (`KismetMathLibrary.DegreesToRadians` (`SplineComponent.GetRollAtSplinePoint` _spline _index "Local")) true)
    (`SplineMeshComponent.SetEndRoll` _returnvalue (`KismetMathLibrary.DegreesToRadians` (`SplineComponent.GetRollAtSplinePoint` _spline _returnvalue_2 "Local")) true)
    (`SplineMeshComponent.SetStartScale` _returnvalue _meshscale true)
    (`SplineMeshComponent.SetEndScale` _returnvalue _meshscale true)
    (`PrimitiveComponent.SetMaterial` _returnvalue 0 (`self.Material`))))