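; Spline gravity area variant that, going by its name, adds a solid visible body along a gravity field's spline.
; The construction script runs the parent's setup, then adds a spline mesh component for each segment between consecutive spline points.
; Each segment follows the local point locations and tangents, with a shared MeshScale at both ends and the Material applied.
; The event graph holds only disabled stubs, so no runtime logic is added here.
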(fn `UserConstructionScript`
  (bind _spline (`self.Spline`))
  (bind _meshscale (`self.MeshScale`))
  (`parent.UserConstructionScript`)
  (for _index (range (+ (- (`SplineComponent.GetNumberOfSplinePoints` (`self.Spline`)) 2) 1))
    (bind _returnvalue (`AddComponent|NODE_AddSplineMeshComponent-1`))
    (bind (_location _tangent) (`SplineComponent.GetLocationAndTangentAtSplinePoint` _spline _index "Local"))
    (bind (_location_2 _tangent_2) (`SplineComponent.GetLocationAndTangentAtSplinePoint` _spline (+ _index 1) "Local"))
    (`SplineMeshComponent.SetStartAndEnd` _returnvalue _location _tangent _location_2 _tangent_2 true)
    (`SplineMeshComponent.SetStartScale` _returnvalue _meshscale true)
    (`SplineMeshComponent.SetEndScale` _returnvalue _meshscale true)
    (`PrimitiveComponent.SetMaterial` _returnvalue 0 (`self.Material`))))