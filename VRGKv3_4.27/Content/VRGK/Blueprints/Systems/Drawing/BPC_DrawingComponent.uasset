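; Drawing component that turns trace hits into brush strokes, stamped textures and erasing on a runtime canvas render target.
; On BeginPlay it creates the target, binds it to a dynamic display material, fires OnDrawingSetup and draws any default texture.
; Hit collision UVs map to canvas pixels, where a mask material stamps tinted textures.
; Lines interpolate stamp position and size between two hits, while erasing draws black lines.
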(event `self.ReceiveBeginPlay`
  (bind _screensize (`self.ScreenSize`))
  (bind _returnvalue (`KismetMathLibrary.Conv_IntToDouble` (`self.ScreenSize`)))
  (bind _returnvalue_2 (`KismetMaterialLibrary.CreateDynamicMaterialInstance` (`self.DrawingDefaultMaterial`) "Drawing Component"))
  (set `self.DrawingMaterial` _returnvalue_2)
  (bind _returnvalue_3 (`CanvasRenderTarget2D.CreateCanvasRenderTarget2D` "/Game/VRGK/Blueprints/Systems/Drawing/BP_DrawingCanvasRT.BP_DrawingCanvasRT_C" _screensize _screensize))
  (set `self.CanvasRT` _returnvalue_3)
  (`KismetRenderingLibrary.ClearRenderTarget2D` (`self.CanvasRT`))
  (`MaterialInstanceDynamic.SetTextureParameterValue` (`self.DrawingMaterial`) "DrawingTexture" (`self.CanvasRT`))
  (`self.OnDrawingSetup`)
  (bind _returnvalue_4 (`KismetMaterialLibrary.CreateDynamicMaterialInstance` "/Game/VRGK/Demo/Materials/DrawingBoard/M_DrawMaskMaterial.M_DrawMaskMaterial" "Drawing Component Mask"))
  (bind _output_get (set `self.DrawMask` _returnvalue_4))
  (`MaterialInstanceDynamic.SetTextureParameterValue` _output_get "Base" (`self.CanvasRT`))
  (bind _defaulttexture (`self.DefaultTexture`)
    (:`then`
      (`self.DrawTexture` (0.0 0.0) (`KismetMathLibrary.MakeVector2D` _returnvalue _returnvalue) _defaulttexture (struct :`R` 1.0 :`G` 1.0 :`B` 1.0 :`A` 1.0)))
    (:`else`)))

(fn `DrawTexture`
  (params (ScreenPosition :type "Vector2D Structure") (ScreenSize :type "Vector2D Structure") (Texture :type "Texture Object Reference") (Color :type "LinearColor Structure"))
  (`self.SetDrawMaskData` Texture Color)
  (bind (_canvas _size _context) (`KismetRenderingLibrary.BeginDrawCanvasToRenderTarget` (`self.CanvasRT`)))
  (`Canvas.K2_DrawMaterial` _canvas (`self.DrawMask`) ScreenPosition ScreenSize (0.0 0.0) (1.0 1.0) 0.0 (0.5 0.5))
  (`KismetRenderingLibrary.EndDrawCanvasToRenderTarget` _context))

(fn `Get Draw Location`
  (params (Hit :type "HitResult Structure (by ref)") (UVChannel :type Integer) (Size :type "Float (double-precision)"))
  (returns (Valid :type Boolean) (`Raw Screen Position` :type "Vector2D Structure") (`Screen Position` :type "Vector2D Structure") (`Screen Size` :type "Vector2D Structure"))
  (bind (_uv _returnvalue) (`GameplayStatics.FindCollisionUV` Hit UVChannel))
  (bind _returnvalue_2 (* _uv (`KismetMathLibrary.Conv_IntToDouble` (`self.ScreenSize`))))
  (return _returnvalue _returnvalue_2 (- _returnvalue_2 (/ Size 2.0)) (`KismetMathLibrary.MakeVector2D` Size Size)))

(fn `SetDrawMaskData`
  (params (`Mask Texture` :type "Texture Object Reference") (`Mask Color` :type "LinearColor Structure"))
  (bind _drawmask (`self.DrawMask`))
  (`MaterialInstanceDynamic.SetTextureParameterValue` _drawmask "Mask" `Mask Texture`)
  (`MaterialInstanceDynamic.SetVectorParameterValue` _drawmask "Color" `Mask Color`))

(fn `TryDrawTextureBrushLineWithHits`
  (params (`Hit A` :type "HitResult Structure") (`Hit B` :type "HitResult Structure") (`Size A` :type "Float (double-precision)") (`Size B` :type "Float (double-precision)") (RenderTexture :type "Texture Object Reference") (RenderColor :type "LinearColor Structure"))
  (locals (PosA :type "Vector2D Structure") (PosB :type "Vector2D Structure") (Length :type "Float (double-precision)" :default 0.0))
  (bind (_posa_x _posa_y) (`KismetMathLibrary.BreakVector2D` (`local.PosA`)))
  (bind (_posb_x _posb_y) (`KismetMathLibrary.BreakVector2D` (`local.PosB`)))
  (bind (_rendercolor_r _rendercolor_g _rendercolor_b) (break `LinearColor` (`local.RenderColor`)))
  (bind (_valid _raw_screen_position) (`self.Get Draw Location` (`local.Hit B`) (`self.UVChannel`) 2.0))
  (bind (_valid_2 _raw_screen_position_2) (`self.Get Draw Location` (`local.Hit A`) (`self.UVChannel`) 2.0))
  (if (and _valid_2 _valid)
    (set `local.PosA` _raw_screen_position_2)
    (set `local.PosB` _raw_screen_position)
    (`self.SetDrawMaskData` (`local.RenderTexture`) (`KismetMathLibrary.MakeColor` _rendercolor_r _rendercolor_g _rendercolor_b 0.0))
    (bind (_canvas _size _context) (`KismetRenderingLibrary.BeginDrawCanvasToRenderTarget` (`self.CanvasRT`)))
    (bind _output_get (set `local.Length` (`KismetMathLibrary.FMax` 1.0 (/ (`KismetMathLibrary.Distance2D` (`local.PosA`) (`local.PosB`)) (/ (`KismetMathLibrary.FMin` (`local.Size A`) (`local.Size B`)) 2.0)))))
    (for _index (range (+ (`KismetMathLibrary.FCeil` _output_get) 1))
      (bind _returnvalue (/ (`KismetMathLibrary.Conv_IntToDouble` _index) (`local.Length`)))
      (bind _returnvalue_2 (`KismetMathLibrary.Lerp` (`local.Size A`) (`local.Size B`) _returnvalue))
      (`Canvas.K2_DrawMaterial` _canvas (`self.DrawMask`) (- (`KismetMathLibrary.Conv_VectorToVector2D` (`KismetMathLibrary.VLerp` (`KismetMathLibrary.MakeVector` _posa_x _posa_y) (`KismetMathLibrary.MakeVector` _posb_x _posb_y) _returnvalue)) (/ _returnvalue_2 2.0)) (`KismetMathLibrary.MakeVector2D` _returnvalue_2 _returnvalue_2) (0.0 0.0) (1.0 1.0) 0.0 (0.5 0.5)))
    (`KismetRenderingLibrary.EndDrawCanvasToRenderTarget` _context)))

(fn `TryDrawTextureBrushWithHit`
  (params (Hit :type "HitResult Structure") (Size :type "Float (double-precision)") (RenderTexture :type "Texture Object Reference") (RenderColor :type "LinearColor Structure"))
  (bind (_rendercolor_r _rendercolor_g _rendercolor_b) (break `LinearColor` (`local.RenderColor`)))
  (bind (_valid _raw_screen_position _screen_position _screen_size) (`self.Get Draw Location` Hit (`self.UVChannel`) Size))
  (if _valid
    (`self.DrawTexture` _screen_position _screen_size (`local.RenderTexture`) (make `LinearColor` _rendercolor_r _rendercolor_g _rendercolor_b))))

(fn `TryErase`
  (params (`Hit A` :type "HitResult Structure") (`Hit B` :type "HitResult Structure") (Size :type "Float (double-precision)"))
  (bind (_valid _raw_screen_position _screen_position) (`self.Get Draw Location` (`local.Hit A`) (`self.UVChannel`) (`local.Size`)))
  (if _valid
    (bind (_canvas _size _context) (`KismetRenderingLibrary.BeginDrawCanvasToRenderTarget` (`self.CanvasRT`)))
    (`Canvas.K2_DrawLine` _canvas _screen_position (`.Raw Screen Position` (`self.Get Draw Location` (`local.Hit B`) (`self.UVChannel`) (`local.Size`))) (`local.Size`) (struct :`A` 1.0))
    (`KismetRenderingLibrary.EndDrawCanvasToRenderTarget` _context)))