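; VR physical input component for a slider that moves a child primitive along one local axis.
; AdjustWeldedLever projects the supplied world location onto the selected axis in component space, caps it within ValueRange and locks the child to the component's rotation.
; It then refreshes the first tracked hand's grab constraint frames and recalculates input values.
; GetRawValue returns the child's local offset along that axis.
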(event `self.AdjustWeldedLever`
  (params (FromWorldLocation :type "Vector Structure"))
  (bind _trackedhandarray (`self.TrackedHandArray`))
  (bind _valuerange (`self.ValueRange`))
  (`|ExecutionSequence`
    (:`then_0`
      (`self.K2_SetWorldLocationAndRotation` (`self.ChildPrimitiveComponent`) (`KismetMathLibrary.TransformLocation` (`self.K2_GetComponentToWorld`) (`KismetMathLibrary.ClampVectorSize` (* (`KismetMathLibrary.InverseTransformLocation` (`self.K2_GetComponentToWorld`) FromWorldLocation) (select `/Game/VRGK/Blueprints/Systems/PhysicalInputs/Enum_PhysicalInputDirection` (`self.Direction`) :`NewEnumerator0` (1.0 0.0 0.0) :`NewEnumerator1` (0.0 1.0 0.0) :`NewEnumerator2` (0.0 0.0 1.0) :!type "Vector Structure")) (* _valuerange -1.0) _valuerange)) (`self.K2_GetComponentRotation`) false false)
      (if (`KismetArrayLibrary.Array_IsValidIndex` _trackedhandarray)
        (`/Game/VRGK/Blueprints/Player/Hand/BP_VRHand.Update Grab Constraint Frames from Grab` _trackedhandarray)))
    (:`then_1`
      (`self.CalculateCurrentInputValues`))))

(fn `Get Raw Value`
  (returns (Value :type "Float (double-precision)"))
  (return (select `/Game/VRGK/Blueprints/Systems/PhysicalInputs/Enum_PhysicalInputDirection` (`self.Direction`) :`NewEnumerator0` (.x (`KismetMathLibrary.InverseTransformLocation` (`self.K2_GetComponentToWorld`) (`self.K2_GetComponentLocation` (`self.ChildPrimitiveComponent`)))) :`NewEnumerator1` (.y (`KismetMathLibrary.InverseTransformLocation` (`self.K2_GetComponentToWorld`) (`self.K2_GetComponentLocation` (`self.ChildPrimitiveComponent`)))) :`NewEnumerator2` (.z (`KismetMathLibrary.InverseTransformLocation` (`self.K2_GetComponentToWorld`) (`self.K2_GetComponentLocation` (`self.ChildPrimitiveComponent`)))))))