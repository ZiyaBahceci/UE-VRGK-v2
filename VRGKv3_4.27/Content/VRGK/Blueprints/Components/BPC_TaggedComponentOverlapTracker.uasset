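; Actor component that tracks whether registered primitive components overlap any component carrying a configured tag.
; Primitives register singly or in batches, binding their begin and end overlap events to handlers that filter by tag and maintain one shared unique list.
; Additions and successful removals fire a tracker update event with a bool indicating whether any tagged component remains in the list.
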(event `Batch Register Primitive Components`
  (params (Primitive :type "Array of PrimitiveComponent Object Reference"))
  (for _array_element Primitive
    (`self.Register Primitive Component For Overlaps` _array_element)))

(event `Register Primitive Component For Overlaps`
  (params (Primitive :type "PrimitiveComponent Object Reference"))
  (`|ExecutionSequence`
    (:`then_0`
      (add `PrimitiveComponent.OnComponentBeginOverlap` Primitive (delegate `OnBegintOverlap`)))
    (:`then_1`
      (add `PrimitiveComponent.OnComponentEndOverlap` Primitive (delegate `OnEndOverlap`)))))

(event `OnBegintOverlap`
  (params (OverlappedComponent :type "PrimitiveComponent Object Reference") (OtherActor :type "Actor Object Reference") (OtherComp :type "PrimitiveComponent Object Reference") (OtherBodyIndex :type Integer) (bFromSweep :type Boolean) (SweepResult :type "HitResult Structure (by ref)"))
  (if (`self.ComponentHasTag` OtherComp (`self.Component Tag to Track`))
    (`KismetArrayLibrary.Array_AddUnique` (`self.OverlappingComponents`) OtherComp)
    (`self.UpdateTrackerState`)))

(event `OnEndOverlap`
  (params (OverlappedComponent :type "PrimitiveComponent Object Reference") (OtherActor :type "Actor Object Reference") (OtherComp :type "PrimitiveComponent Object Reference") (OtherBodyIndex :type Integer))
  (if (`self.ComponentHasTag` OtherComp (`self.Component Tag to Track`))
    (bind _returnvalue (`KismetArrayLibrary.Array_RemoveItem` (`self.OverlappingComponents`) OtherComp))
    (if _returnvalue
      (`self.UpdateTrackerState`))))

(event `UpdateTrackerState`
  (`self.OnTrackerStateUpdate` (`self.IsCurrentlyOverlappingTaggedComponents`)))

(fn `IsCurrentlyOverlappingTaggedComponents`
  (returns (ReturnValue :type Boolean))
  (return (> (`KismetArrayLibrary.Array_Length` (`self.OverlappingComponents`)) 0)))