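; Desktop input handler that drives the VR game pawn with mouse and keyboard, standing in for VR controls.
; On BeginPlay it shows an overlay and warning, disables pawn input, forces standing mode and detaches both hands.
; Tick applies mouse look and pins mirrored hands to the camera at a wheel-adjusted distance.
; Keys forward movement, sprint, crouch, jump, teleport and grabs to the pawn, and the handler destroys itself when the pawn ends play.
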(event `self.ReceiveBeginPlay`
  (`|ExecutionSequence`
    (:`then_0`
      (bind _returnvalue (`|CreateWidget` "/Game/VRGK/Blueprints/Player/PlayerCore/NonVR/BPW_NonVRHandlerOverlay.BPW_NonVRHandlerOverlay_C"))
      (`UserWidget.AddToViewport` _returnvalue 0))
    (:`then_1`
      (`KismetSystemLibrary.PrintString` "WARNING: NonVR Input Handler is active!" true true (struct :`R` 1.0 :`G` 0.010869 :`A` 1.0) 5.0)
      (`self.EnableInput` (`GameplayStatics.GetPlayerController` 0))
      (add `self.OnEndPlay` (`self.VRGamePawn`) (delegate `OnPawnEndPlay`))
      (bind _settings (`/Game/VRGK/Blueprints/BPFL_GlobalFunctions.Get BPO Game Settings`))
      (`/Game/VRGK/Blueprints/Core/BPO_Settings.SetSeatedPlayModeEnabled` _settings false)
      (`/Game/VRGK/Blueprints/Core/BPO_Settings.SetStandingPlayerHeight` _settings (`/Game/VRGK/Blueprints/Player/PlayerCore/BP_VRGamePawn.DefaultPlayerHeight` (`self.VRGamePawn`)))
      (`self.AddTickPrerequisiteActor` self (`/Game/VRGK/Blueprints/Player/PlayerCore/BP_VRGamePawn.LeftHand` (`self.VRGamePawn`)))
      (`self.AddTickPrerequisiteActor` self (`self.VRGamePawn`))
      (`self.DisableInput` (`self.VRGamePawn`) (`GameplayStatics.GetPlayerController` 0))
      (`SceneComponent.K2_SetRelativeLocationAndRotation` :`self` (`/Game/VRGK/Blueprints/Player/Hand/BP_VRHand.HandSocket` (`/Game/VRGK/Blueprints/Player/PlayerCore/BP_VRGamePawn.LeftHand` (`self.VRGamePawn`))))
      (`SceneComponent.K2_SetRelativeLocationAndRotation` :`self` (`/Game/VRGK/Blueprints/Player/Hand/BP_VRHand.HandSocket` (`/Game/VRGK/Blueprints/Player/PlayerCore/BP_VRGamePawn.RightHand` (`self.VRGamePawn`))))
      (`self.K2_DetachFromActor` (`/Game/VRGK/Blueprints/Player/PlayerCore/BP_VRGamePawn.LeftHand` (`self.VRGamePawn`)) "KeepWorld" "KeepWorld" "KeepWorld")
      (`self.K2_DetachFromActor` (`/Game/VRGK/Blueprints/Player/PlayerCore/BP_VRGamePawn.RightHand` (`self.VRGamePawn`)) "KeepWorld" "KeepWorld" "KeepWorld"))))

(event `OnPawnEndPlay` :!signature `self.OnEndPlay`
  (params (Actor :type "Actor Object Reference") (EndPlayReason :type "EEndPlayReason Enum" :default "Destroyed"))
  (`self.K2_DestroyActor`))

(event `self.ReceiveTick`
  (params (DeltaSeconds :type "Float (single-precision)"))
  (bind (_nextcameravector_x _nextcameravector_y) (`KismetMathLibrary.BreakVector2D` (`self.NextCameraVector`)))
  (bind _camera (`/Game/VRGK/Blueprints/Player/PlayerCore/BP_VRBasePawn.Camera` (`self.VRGamePawn`)))
  (bind (_relativerotation_roll _relativerotation_pitch _relativerotation_yaw) (`KismetMathLibrary.BreakRotator` (`SceneComponent.RelativeRotation` _camera)))
  (set `self.CurDeltaSeconds` DeltaSeconds)
  (`|ExecutionSequence`
    (:`then_0`
      (`SceneComponent.K2_SetRelativeRotation` _camera (`KismetMathLibrary.RInterpTo` (`SceneComponent.RelativeRotation` _camera) (`KismetMathLibrary.MakeRotator` 0.0 (`KismetMathLibrary.FClamp` (- _relativerotation_pitch _nextcameravector_y) -89.0 89.0) (+ _relativerotation_yaw _nextcameravector_x)) (`self.CurDeltaSeconds`) 180.0) false false))
    (:`then_1`
      (`self.UpdateMotionControllerLocation` "NewEnumerator0")
      (`self.UpdateMotionControllerLocation` "NewEnumerator1"))))

(event `UpdateMotionControllerLocation`
  (params (`Hand Type` :type "/Game/VRGK/Blueprints/Player/Hand/Enum_HandType Enum" :default "NewEnumerator0"))
  (bind _vrgamepawn (`self.VRGamePawn`))
  (bind _returnvalue (`KismetMathLibrary.MakeTransform` (`KismetMathLibrary.MakeVector` (+ 20.0 (`self.HandDistance`)) -20.0 -10.0) (struct :`Pitch` 20.0)))
  (bind _returnvalue_2 (`SceneComponent.K2_GetComponentToWorld` (`/Game/VRGK/Blueprints/Player/PlayerCore/BP_VRBasePawn.Camera` (`self.VRGamePawn`))))
  (bind (_returnvalue_location _returnvalue_rotation) (`KismetMathLibrary.BreakTransform` (select `/Game/VRGK/Blueprints/Player/Hand/Enum_HandType` `Hand Type` :`NewEnumerator0` (`/Game/VRGK/Blueprints/BPFL_GlobalFunctions.MirrorTransformByAxis` "NewEnumerator2" _returnvalue) :`NewEnumerator1` _returnvalue)))
  ;[1 1 1] Update Hand Location
  (`self.K2_SetActorLocationAndRotation` (select `/Game/VRGK/Blueprints/Player/Hand/Enum_HandType` `Hand Type` :`NewEnumerator0` (`/Game/VRGK/Blueprints/Player/PlayerCore/BP_VRGamePawn.RightHand` _vrgamepawn) :`NewEnumerator1` (`/Game/VRGK/Blueprints/Player/PlayerCore/BP_VRGamePawn.LeftHand` _vrgamepawn)) (`KismetMathLibrary.TransformLocation` _returnvalue_2 _returnvalue_location) (`KismetMathLibrary.TransformRotation` _returnvalue_2 _returnvalue_rotation) false false))

(event `Key|T`
  (params (Key :type "Key Structure"))
  (bind _vrgamepawn (`self.VRGamePawn`))
  ;[1 1 1] Teleport
  (:`Pressed`
    (`/Game/VRGK/Blueprints/Player/PlayerCore/BP_VRGamePawn.ActivateTeleporter` _vrgamepawn "NewEnumerator0"))
  (:`Released`
    (`/Game/VRGK/Blueprints/Player/PlayerCore/BP_VRGamePawn.TryTeleporter` _vrgamepawn "NewEnumerator0")))

(event `Key|W`
  (params (Key :type "Key Structure"))
  (bind _vrgamepawn (`self.VRGamePawn`))
  ;[1 1 1] WASD Movement / Left Thumbstick
  (:`Pressed`
    (`/Game/VRGK/Blueprints/BPML_ActorInputHelpers.AdvancedInputTrigger` 0.0 :!label _label
      (:`Triggered`
        (`/Game/VRGK/Blueprints/Player/PlayerCore/BP_VRGamePawn.DoPlayerMovementY` _vrgamepawn 1.0))
      (:`Completed`
        (`/Game/VRGK/Blueprints/Player/PlayerCore/BP_VRGamePawn.DoPlayerMovementY` _vrgamepawn 0.0))))
  (:`Released`
    (goto _label :!via `Released`)))

(event `Key|Q`
  (params (Key :type "Key Structure"))
  ;[1 1 1] Sprinting
  (:`Pressed`
    (set `/Game/VRGK/Blueprints/Player/PlayerCore/BP_VRGamePawn.CurrentlySprinting` true (`self.VRGamePawn`))))

(event `Key|S`
  (params (Key :type "Key Structure"))
  (bind _vrgamepawn (`self.VRGamePawn`))
  ;[1 1 1] WASD Movement / Left Thumbstick
  (:`Pressed`
    (`/Game/VRGK/Blueprints/BPML_ActorInputHelpers.AdvancedInputTrigger` 0.0 :!label _label_2
      (:`Triggered`
        (`/Game/VRGK/Blueprints/Player/PlayerCore/BP_VRGamePawn.DoPlayerMovementY` _vrgamepawn -1.0))
      (:`Completed`
        (`/Game/VRGK/Blueprints/Player/PlayerCore/BP_VRGamePawn.DoPlayerMovementY` _vrgamepawn 0.0))))
  (:`Released`
    (goto _label_2 :!via `Released`)))

(event `Key|D`
  (params (Key :type "Key Structure"))
  (bind _vrgamepawn (`self.VRGamePawn`))
  ;[1 1 1] WASD Movement / Left Thumbstick
  (:`Pressed`
    (`/Game/VRGK/Blueprints/BPML_ActorInputHelpers.AdvancedInputTrigger` 0.0 :!label _label_3
      (:`Triggered`
        (`/Game/VRGK/Blueprints/Player/PlayerCore/BP_VRGamePawn.DoPlayerMovementX` _vrgamepawn 1.0))
      (:`Completed`
        (`/Game/VRGK/Blueprints/Player/PlayerCore/BP_VRGamePawn.DoPlayerMovementX` _vrgamepawn 0.0))))
  (:`Released`
    (goto _label_3 :!via `Released`)))

(event `InputVectorAxis|Mouse2D`
  (params (AxisValue :type "Vector Structure"))
  ;[1 1 1] Camera / Looking Direction
  (set `self.NextCameraVector` (`KismetMathLibrary.MakeVector2D` (* AxisValue_X (`self.CurDeltaSeconds`) 90.0) (* AxisValue_Y -1.0 (`self.CurDeltaSeconds`) 90.0))))

(event `Key|A`
  (params (Key :type "Key Structure"))
  (bind _vrgamepawn (`self.VRGamePawn`))
  ;[1 1 1] WASD Movement / Left Thumbstick
  (:`Pressed`
    (`/Game/VRGK/Blueprints/BPML_ActorInputHelpers.AdvancedInputTrigger` 0.0 :!label _label_4
      (:`Triggered`
        (`/Game/VRGK/Blueprints/Player/PlayerCore/BP_VRGamePawn.DoPlayerMovementX` _vrgamepawn -1.0))
      (:`Completed`
        (`/Game/VRGK/Blueprints/Player/PlayerCore/BP_VRGamePawn.DoPlayerMovementX` _vrgamepawn 0.0))))
  (:`Released`
    (goto _label_4 :!via `Released`)))

(event `InputAxisKey|MouseWheelAxis`
  (params (AxisValue :type "Float (single-precision)"))
  ;[1 1 1] Hand Distance
  (set `self.HandDistance` (`KismetMathLibrary.FClamp` (+ (`self.HandDistance`) (* AxisValue (`self.CurDeltaSeconds`) 500.0)) 0.0 100.0)))

(event `Key|LeftMouseButton`
  (params (Key :type "Key Structure"))
  (bind _vrgamepawn (`self.VRGamePawn`))
  (bind _lefthand (`/Game/VRGK/Blueprints/Player/PlayerCore/BP_VRGamePawn.LeftHand` _vrgamepawn))
  ;[1 1 1] Hand Grabbing
  (:`Pressed`
    (`/Game/VRGK/Blueprints/Player/PlayerCore/BP_VRGamePawn.DoPlayerGrabLeftPressed` _vrgamepawn)
    (`/Game/VRGK/Blueprints/Player/Hand/BP_VRHand.SetFingerGrabPress` _lefthand 1.0))
  (:`Released`
    (`/Game/VRGK/Blueprints/Player/PlayerCore/BP_VRGamePawn.DoPlayerGrabLeftReleased` _vrgamepawn)
    (`/Game/VRGK/Blueprints/Player/Hand/BP_VRHand.SetFingerGrabPress` _lefthand 0.0)))

(event `Key|LeftShift`
  (params (Key :type "Key Structure"))
  (bind _vrgamepawn (`self.VRGamePawn`))
  ;[1 1 1] Virtual Crouching
  (:`Pressed`
    (`/Game/VRGK/Blueprints/BPML_ActorInputHelpers.AdvancedInputTrigger` 0.0 :!label _label_5
      (:`Triggered`
        (`/Game/VRGK/Blueprints/Player/PlayerCore/BP_VRGamePawn.DoPlayerCrouchY` _vrgamepawn 1.0))
      (:`Completed`
        (`/Game/VRGK/Blueprints/Player/PlayerCore/BP_VRGamePawn.DoPlayerCrouchY` _vrgamepawn 0.0))))
  (:`Released`
    (goto _label_5 :!via `Released`)))

(event `Key|RightMouseButton`
  (params (Key :type "Key Structure"))
  (bind _vrgamepawn (`self.VRGamePawn`))
  (bind _righthand (`/Game/VRGK/Blueprints/Player/PlayerCore/BP_VRGamePawn.RightHand` _vrgamepawn))
  ;[1 1 1] Hand Grabbing
  (:`Pressed`
    (`/Game/VRGK/Blueprints/Player/PlayerCore/BP_VRGamePawn.DoPlayerGrabRightPressed` _vrgamepawn)
    (`/Game/VRGK/Blueprints/Player/Hand/BP_VRHand.SetFingerGrabPress` _righthand 1.0))
  (:`Released`
    (`/Game/VRGK/Blueprints/Player/PlayerCore/BP_VRGamePawn.DoPlayerGrabRightReleased` _vrgamepawn)
    (`/Game/VRGK/Blueprints/Player/Hand/BP_VRHand.SetFingerGrabPress` _righthand 0.0)))

(event `Key|LeftControl`
  (params (Key :type "Key Structure"))
  (bind _vrgamepawn (`self.VRGamePawn`))
  ;[1 1 1] Virtual Crouching
  (:`Pressed`
    (`/Game/VRGK/Blueprints/BPML_ActorInputHelpers.AdvancedInputTrigger` 0.0 :!label _label_6
      (:`Triggered`
        (`/Game/VRGK/Blueprints/Player/PlayerCore/BP_VRGamePawn.DoPlayerCrouchY` _vrgamepawn -1.0))
      (:`Completed`
        (`/Game/VRGK/Blueprints/Player/PlayerCore/BP_VRGamePawn.DoPlayerCrouchY` _vrgamepawn 0.0))))
  (:`Released`
    (goto _label_6 :!via `Released`)))

(event `Key|SpaceBar`
  (params (Key :type "Key Structure"))
  (bind _vrgamepawn (`self.VRGamePawn`))
  ;[1 1 1] Jumping
  (:`Pressed`
    (`/Game/VRGK/Blueprints/Player/PlayerCore/BP_VRGamePawn.DoPlayerJumpPressed` _vrgamepawn))
  (:`Released`
    (`/Game/VRGK/Blueprints/Player/PlayerCore/BP_VRGamePawn.DoPlayerJumpReleased` _vrgamepawn)))

(fn `UserConstructionScript`)