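; VR physical joystick input component that turns the tilt of a child primitive into a 2D axis value.
; Each physical input tick converts the child's up vector into the component's local space, projects it onto the plane of the component's up axis and keeps X and Y.
; The result is cached for GetJoystickValue and broadcast through OnJoystickValueChange every tick, with no change check.
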(event `self.ReceiveBeginPlay`
  (`parent.ReceiveBeginPlay`))

(event `self.Physical Input Tick`
  (params (`Delta Seconds` :type "Float (single-precision)"))
  (bind _output_get (set `self.CurValue` (`self.GetRawJoystickValue`)))
  (`self.OnJoystickValueChange` self _output_get))

(fn `GetJoystickValue`
  (returns (CurValue :type "Vector2D Structure"))
  (return (`self.CurValue`)))

(fn `GetRawJoystickValue`
  (returns (Value :type "Vector2D Structure"))
  (bind _returnvalue (`self.K2_GetComponentToWorld`))
  (bind _returnvalue_2 (`KismetMathLibrary.InverseTransformDirection` _returnvalue (`self.GetUpVector`)))
  (bind (_returnvalue_x _returnvalue_y) (`KismetMathLibrary.BreakVector` (`KismetMathLibrary.ProjectPointOnToPlane` (`KismetMathLibrary.InverseTransformDirection` _returnvalue (`self.GetUpVector` (`self.ChildPrimitiveComponent`))) (`KismetMathLibrary.MakeVector` 0.0 0.0 (.z _returnvalue_2)) _returnvalue_2)))
  (return (`KismetMathLibrary.MakeVector2D` _returnvalue_x _returnvalue_y)))