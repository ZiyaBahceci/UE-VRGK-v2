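; VR physical input component for a hand-grabbed lever that reports a rotation value about a chosen axis, clamped to a symmetric range.
; In constraint mode it only reads the physics-driven child's rotation each tick.
; In welded mode it rotates the child toward the hand using atan2 (X axis only; Y/Z yield zero) and updates grab constraint frames.
; The optionally inverted value is broadcast and also available normalized.
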(event `self.ReceiveBeginPlay`
  (`parent.ReceiveBeginPlay`)
  (`self.SetDefaultValues`))

(event `self.Physical Input Tick`
  (params (`Delta Seconds` :type "Float (single-precision)"))
  (bind _trackedhandarray (`self.TrackedHandArray`))
  (bind _returnvalue_location (`KismetMathLibrary.BreakTransform` (`/Game/VRGK/Blueprints/Player/Hand/BP_VRHand.GetSocketRelativeGrabRootTransform` (`|GetArrayItem` _trackedhandarray))))
  (switch `/Game/VRGK/Blueprints/Systems/PhysicalInputs/Enum_PhysicalInputInteractionmode` (`self.Interaction Mode`)
    (:`NewEnumerator0`
      (`self.CalculateCurrentInputValues`))
    (:`NewEnumerator1`
      (if (`KismetArrayLibrary.Array_IsValidIndex` _trackedhandarray)
        (`self.AdjustWeldedLever` _returnvalue_location)))))

(event `self.CalculateCurrentInputValues`
  (bind _valuerange (`self.ValueRange`))
  (bind _output_get (set `self.CurrentInputValue` (`KismetMathLibrary.FClamp` (`self.Get Raw Value`) (* _valuerange -1.0) _valuerange)))
  (`self.OnInputValueChange` self _output_get))

(event `AdjustWeldedLever`
  (params (FromWorldLocation :type "Vector Structure"))
  (bind _trackedhandarray (`self.TrackedHandArray`))
  (bind _valuerange (`self.ValueRange`))
  (`|ExecutionSequence`
    (:`then_0`
      (`self.K2_SetWorldLocationAndRotation` (`self.ChildPrimitiveComponent`) (`self.K2_GetComponentLocation`) (`KismetMathLibrary.TransformRotation` (`self.K2_GetComponentToWorld`) (select `/Game/VRGK/Blueprints/Systems/PhysicalInputs/Enum_PhysicalInputDirection` (`self.Direction`) :`NewEnumerator0` (`KismetMathLibrary.MakeRotator` (`KismetMathLibrary.FClamp` (`KismetMathLibrary.DegAtan2` (.y (`KismetMathLibrary.InverseTransformLocation` (`self.K2_GetComponentToWorld`) FromWorldLocation)) (.z (`KismetMathLibrary.InverseTransformLocation` (`self.K2_GetComponentToWorld`) FromWorldLocation))) (* _valuerange -1.0) _valuerange)) :`NewEnumerator1` (`KismetMathLibrary.MakeRotator` 0.0) :`NewEnumerator2` (`KismetMathLibrary.MakeRotator` 0.0) :!type "Rotator Structure")) false false)
      (if (`KismetArrayLibrary.Array_IsValidIndex` _trackedhandarray)
        (`/Game/VRGK/Blueprints/Player/Hand/BP_VRHand.Update Grab Constraint Frames from Grab` _trackedhandarray)))
    (:`then_1`
      (`self.CalculateCurrentInputValues`))))

(event `SetWeldedLeverValue`
  (params (`New Value` :type "Float (double-precision)"))
  (`self.AdjustWeldedLever` (`KismetMathLibrary.TransformLocation` (`self.K2_GetComponentToWorld`) (`KismetMathLibrary.Conv_DoubleToVector` `New Value`))))

(event `SetDefaultValues`
  (switch `/Game/VRGK/Blueprints/Systems/PhysicalInputs/Enum_PhysicalInputInteractionmode` (`self.Interaction Mode`)
    (:`NewEnumerator1`
      (`self.SetWeldedLeverValue` (`self.DefaultValue`)))))

(fn `Get Current Value`
  (returns (Value :type "Float (double-precision)"))
  (return (`self.CurrentInputValue`)))

(fn `Get Normalized Current Value`
  (params (`Use 0 to 1` :type Boolean))
  (returns (Normalized :type "Float (double-precision)"))
  (bind _valuerange (`self.ValueRange`))
  (return (`KismetMathLibrary.MapRangeClamped` (`self.CurrentInputValue`) (* _valuerange -1.0) _valuerange (`KismetMathLibrary.SelectFloat` 0.0 -1.0 `Use 0 to 1`) 1.0)))

(fn `Get Raw Value`
  (returns (Value :type "Float (double-precision)"))
  (bind _returnvalue (select `/Game/VRGK/Blueprints/Systems/PhysicalInputs/Enum_PhysicalInputDirection` (`self.Direction`) :`NewEnumerator0` (.roll (`KismetMathLibrary.InverseTransformRotation` (`self.K2_GetComponentToWorld`) (`self.K2_GetComponentRotation` (`self.ChildPrimitiveComponent`)))) :`NewEnumerator1` (.pitch (`KismetMathLibrary.InverseTransformRotation` (`self.K2_GetComponentToWorld`) (`self.K2_GetComponentRotation` (`self.ChildPrimitiveComponent`)))) :`NewEnumerator2` (.yaw (`KismetMathLibrary.InverseTransformRotation` (`self.K2_GetComponentToWorld`) (`self.K2_GetComponentRotation` (`self.ChildPrimitiveComponent`))))))
  (return (`KismetMathLibrary.SelectFloat` (* _returnvalue -1.0) _returnvalue (`self.InvertValue`))))