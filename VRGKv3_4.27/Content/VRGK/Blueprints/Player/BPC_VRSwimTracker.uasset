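; VR player component that turns hand motion into a swim velocity for the owning BP_VRGamePawn.
; Each tick it sums both hands' physics velocities at their tracker points, scaled by an eased speed ramp and by hand separation, so slow or close-together motion is damped.
; It broadcasts the result, with optional debug arrows.
; Enabling or disabling tracking toggles component tick and broadcasts the new state.
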(event `self.ReceiveBeginPlay`
  (bind _asbp_vrgame_pawn (cast `/Game/VRGK/Blueprints/Player/PlayerCore/BP_VRGamePawn` (`self.GetOwner`)))
  (set `self.GamePawn` _asbp_vrgame_pawn))

(event `SetSwimTrackerEnabled`
  (params (Enabled :type Boolean))
  (`self.SetComponentTickEnabled` Enabled)
  (`self.OnSwimmingEnabled` (`self.IsSwimmingEnabled`)))

(event `self.ReceiveTick`
  (params (DeltaSeconds :type "Float (single-precision)"))
  (bind _gamepawn (`self.GamePawn`))
  (bind _gamepawn_2 (`self.GamePawn`))
  (bind _righthand (`/Game/VRGK/Blueprints/Player/PlayerCore/BP_VRGamePawn.RightHand` _gamepawn_2))
  (bind _lefthand (`/Game/VRGK/Blueprints/Player/PlayerCore/BP_VRGamePawn.LeftHand` _gamepawn_2))
  (bind _returnvalue (`SceneComponent.K2_GetComponentLocation` (`/Game/VRGK/Blueprints/Player/Hand/BP_VRHand.VelocityTrackerLocation` _righthand)))
  (bind _returnvalue_2 (`SceneComponent.K2_GetComponentLocation` (`/Game/VRGK/Blueprints/Player/Hand/BP_VRHand.VelocityTrackerLocation` _lefthand)))
  (bind _returnvalue_3 (`PrimitiveComponent.GetPhysicsLinearVelocityAtPoint` (`/Game/VRGK/Blueprints/Player/Hand/BP_VRHand.HandBaseCollision` _lefthand) _returnvalue_2 "None"))
  (bind _returnvalue_4 (`PrimitiveComponent.GetPhysicsLinearVelocityAtPoint` (`/Game/VRGK/Blueprints/Player/Hand/BP_VRHand.HandBaseCollision` _righthand) _returnvalue "None"))
  (bind _returnvalue_5 (+ _returnvalue_3 _returnvalue_4))
  (bind _output_get (set `self.CurSwimVelocity` (* _returnvalue_5 (* (`KismetMathLibrary.FInterpEaseInOut` 0.0 1.0 (`KismetMathLibrary.MapRangeClamped` (`KismetMathLibrary.VSize` _returnvalue_5) 50.0 100.0 0.0 1.0) 1.5) (`KismetMathLibrary.MapRangeClamped` (`KismetMathLibrary.Vector_Distance` _returnvalue_2 _returnvalue) 20.0 100.0 0.0 1.0)))))
  (`self.OnSwimmingMotion` _output_get)
  ;[1 1 1] Debug Drawing
  (if (`self.DrawDebug`)
    (for _array_element (`|MakeArray` (`/Game/VRGK/Blueprints/Player/PlayerCore/BP_VRGamePawn.LeftHand` _gamepawn) (`/Game/VRGK/Blueprints/Player/PlayerCore/BP_VRGamePawn.RightHand` _gamepawn))
      (bind _returnvalue_6 (`Actor.K2_GetActorLocation` _array_element))
      (`KismetSystemLibrary.DrawDebugArrow` _returnvalue_6 (+ _returnvalue_6 (`self.CurSwimVelocity`)) 2.0 (struct :`R` 1.0 :`G` 0.75 :`A` 1.0) 0.0 0.5))))

(fn `GetCurrentSwimVelocity`
  (returns (CurSwimVelocity :type "Vector Structure"))
  (return (`self.CurSwimVelocity`)))

(fn `IsSwimmingEnabled`
  (returns (True :type Boolean))
  (return (`self.IsComponentTickEnabled`)))