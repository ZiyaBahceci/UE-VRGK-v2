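; Actor component that plays impact sounds when its owning actor hits another actor.
; It picks a sound by the hit physical material's surface type from a data asset, with default fallbacks.
; Impulse magnitude, mapped through that sound's threshold range, sets the volume of a sound spawned attached at the impact point.
; A DoOnce gate and last-hit timestamp debounce repeated hits, so sustained contact does not retrigger sounds.
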(event `self.ReceiveBeginPlay`
  (bind _returnvalue (`self.GetOwner`))
  (add `Actor.OnActorHit` _returnvalue (delegate `OnActorHit`))
  (bind _asprimitive_component (cast `PrimitiveComponent` (`Actor.RootComponent` _returnvalue)))
  (set `self.RootPrimitive` _asprimitive_component))

(event `OnActorHit`
  (params (SelfActor :type "Actor Object Reference") (OtherActor :type "Actor Object Reference") (NormalImpulse :type "Vector Structure") (Hit :type "HitResult Structure (by ref)"))
  (if (!= SelfActor OtherActor)
    (set `self.CurNormalImpulse` NormalImpulse)
    (set `self.CurHit` Hit)
    (`|ExecutionSequence`
      (:`then_0`
        (if (> (- (`Actor.GetGameTimeSinceCreation` (`self.GetOwner`)) (`self.LastHitTime`)) 0.02)
          (`self.ResetActorHit`)))
      (:`then_1`
        (`/Engine/EditorBlueprintResources/StandardMacros.DoOnce` false :!label _label
          (:`Completed`
            (`/Engine/EditorBlueprintResources/StandardMacros.IsValid` (`.HitComponent` (`GameplayStatics.BreakHitResult` (`self.LastHitResult`)))
              (:`Is Valid`
                (if (> (- (`Actor.GetGameTimeSinceCreation` (`self.GetOwner`)) (`self.LastHitTime`)) 0.1)
                  (set `self.LastHitResult` (struct))
                  (else
                    (`self.ResetActorHit`)
                    (if (not (!= (`.HitActor` (`GameplayStatics.BreakHitResult` (`self.LastHitResult`))) (`.HitActor` (`GameplayStatics.BreakHitResult` (`self.CurHit`)))))
                      (`self.UpdateLastHitTime`)))))
              (:`Is Not Valid`
                (`self.DoCollisionSoundEvents`)))))))))

(event `ResetActorHit`
  (goto _label :!via `Reset`))

(event `SetLastHitResultActive`
  (set `self.LastHitResult` (`self.CurHit`))
  (`self.UpdateLastHitTime`))

(event `UpdateLastHitTime`
  (set `self.LastHitTime` (`Actor.GetGameTimeSinceCreation` (`self.GetOwner`))))

(event `DoCollisionSoundEvents`
  (bind _sound_da (`self.GetSoundDataAsset`))
  (bind _cursounddata_soundtoplay (break `/Game/VRGK/Blueprints/Data/Struct_CollisionSoundData` (`self.CurSoundData`)))
  (bind _cursounddata_soundtoplay_2 (break `/Game/VRGK/Blueprints/Data/Struct_CollisionSoundData` (`self.CurSoundData`)))
  (bind _cursounddata (`self.CurSoundData`))
  (bind _defaultsound (`/Game/VRGK/Blueprints/Data/BP_CollisionSoundDataAsset.DefaultSound` _sound_da))
  (bind (_value _returnvalue) (`BlueprintMapLibrary.Map_Find` (`/Game/VRGK/Blueprints/Data/BP_CollisionSoundDataAsset.SurfaceSounds` _sound_da) (`PhysicalMaterial.SurfaceType` (`.PhysMat` (`GameplayStatics.BreakHitResult` (`self.CurHit`))))))
  (`|ExecutionSequence`
    (:`then_0`
      (`/Engine/EditorBlueprintResources/StandardMacros.IsValid` (`.PhysMat` (`GameplayStatics.BreakHitResult` (`self.CurHit`)))
        (:`Is Valid`
          (set `self.CurSoundData` (select `bool` _returnvalue :`false` _defaultsound :`true` _value)))
        (:`Is Not Valid`
          (set `self.CurSoundData` _defaultsound))))
    (:`then_1`
      (`/Engine/EditorBlueprintResources/StandardMacros.IsValid` _cursounddata_soundtoplay
        (:`Is Valid`
          (`|ExecutionSequence`
            (:`then_0`
              (set `self.TempVolume` 1.0)
              (if (> (`self.TempVolume`) 0.0)
                (bind _output_get (set `self.TempVolume` (* (`KismetMathLibrary.MapRangeClamped` (`KismetMathLibrary.VSize` (`self.CurNormalImpulse`)) (break `InputRange` (`.HitThresholdRange_8_C877EF4448F516C8B4F4BC8FF11C1A91` (break `/Game/VRGK/Blueprints/Data/Struct_CollisionSoundData` _cursounddata))) (`.Max` (break `InputRange` (`.HitThresholdRange_8_C877EF4448F516C8B4F4BC8FF11C1A91` (break `/Game/VRGK/Blueprints/Data/Struct_CollisionSoundData` _cursounddata)))) 0.0 1.0) (`self.TempVolume`))))
                (if (> _output_get 0.0)
                  (`|ExecutionSequence`
                    (:`then_0`
                      (`GameplayStatics.SpawnSoundAttached` _cursounddata_soundtoplay_2 (`Actor.RootComponent` (`self.GetOwner`)) "None" (`.ImpactPoint` (`GameplayStatics.BreakHitResult` (`self.CurHit`))) (struct) "KeepWorldPosition" false (`self.TempVolume`) 1.0 0.0 null null))
                    (:`then_2`
                      (`self.SetLastHitResultActive`)
                      (`self.ResetActorHit`)))
                  (else
                    (`self.SetLastHitResultActive`)
                    (`self.ResetActorHit`)))
                (else
                  (`self.ResetActorHit`))))))
        (:`Is Not Valid`
          (`self.ResetActorHit`))))))

(fn `GetSoundDataAsset`
  (returns (`Sound DA` :type "/Game/VRGK/Blueprints/Data/BP_CollisionSoundDataAsset Object Reference"))
  (bind _collision_sound_data (`self.Collision Sound Data`))
  (return (select `bool` (`KismetSystemLibrary.IsValid` _collision_sound_data) :`false` (`self.Default Sound Data Asset`) :`true` _collision_sound_data)))