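; Finger-tip variant of the VR interaction laser pointer that simulates physically pressing widgets with a finger.
; Each tick it presses the widget when the widget interaction hit is very close, and releases it otherwise.
; A looping timer sphere-traces around the WidgetOverlapper while the laser is enabled.
; That trace, plus interaction-change events, updates the overlapping-widgets flag and fires the overlap range dispatcher.
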(event `self.ReceiveBeginPlay`
  (`parent.ReceiveBeginPlay`)
  (add `self.OnInteractionChange` (delegate `OnInteractionChange_Event_0`))
  (`KismetSystemLibrary.K2_SetTimerDelegate` (delegate `UpdateWidgetOverlap`) 0.2 true 0.2))

(event `OnInteractionChange_Event_0` :!signature `self.OnInteractionChange`
  (params (`Has Widget` :type Boolean))
  (if `Has Widget`
    (bind _output_get (set `self.IsOverlappingWidgets` true))
    (`self.OnOverlapRange` _output_get)))

(event `UpdateWidgetOverlap`
  (bind _widgetoverlapper (`self.WidgetOverlapper`))
  (bind _returnvalue (`SceneComponent.K2_GetComponentLocation` _widgetoverlapper))
  (if (`self.IsLaserPointerEnabled`)
    ;[1 1 1] Try to trace if a Widget is in Finger Reach
    (bind (_outhit _returnvalue_2) (`KismetSystemLibrary.SphereTraceSingle` _returnvalue _returnvalue (`SphereComponent.SphereRadius` _widgetoverlapper) "TraceTypeQuery5"))
    (bind _output_get (set `self.IsOverlappingWidgets` (or _returnvalue_2 (`self.HasValidWidgetToInteract`))))
    (`self.OnOverlapRange` _output_get)
    (else
      (set `self.IsOverlappingWidgets` false))))

(event `self.ReceiveTick`
  (params (DeltaSeconds :type "Float (single-precision)"))
  (bind (_returnvalue_bblockinghit _returnvalue_binitialoverlap _returnvalue_time _returnvalue_distance) (`GameplayStatics.BreakHitResult` (`WidgetInteractionComponent.GetLastHitResult` (`self.WidgetInteraction`))))
  (`parent.ReceiveTick` DeltaSeconds)
  ;[1 1 1] Simulate Physical FInger Press on the Widget
  (if (and _returnvalue_bblockinghit (< _returnvalue_distance 3.0))
    (`self.TryWidgetPress`)
    (else
      (`self.TryWidgetRelease`))))

(fn `UserConstructionScript`
  (`parent.UserConstructionScript`))